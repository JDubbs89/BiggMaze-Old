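; BP_UserDataAccessLayer is a database access layer that reads the list of user accounts as SUserData structs.
; Startup has QueryManager load its prepared statements, which GetQuery looks up by name with a validity check.
; GetUserAccountList executes the named select and passes the result to a converter.
; The converter maps fields by column index and builds banner color via TryFillColor, falling back to a default color.
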(event `self.Startup`
  (params (DatabaseFilePath :type String) (Config :type "GameDbConfig Structure (by ref)"))
  (`PreparedStatementManager.LoadStatements` (`self.QueryManager`)))

(fn `Get Query`
  (params (`Statement Name` :type String))
  (returns (Statement :type "DbStatement Object Reference") (`Is Valid` :type Boolean))
  (bind _returnvalue (`PreparedStatementManager.FindStatement` (`self.QueryManager`) `Statement Name`))
  (return _returnvalue (`KismetSystemLibrary.IsValid` _returnvalue)))

(fn `Get User Account List`
  (returns (Data :type "Array of /Game/DataBase/Structs/S_UserData Structure"))
  (locals (`Prepared Statement` :type "DbStatement Object Reference") (`Result Data` :type "QueryResult Structure"))
  (bind (_statement _is_valid) (`self.Get Query` "GetUserAccountsList"))
  (if _is_valid
    (set `local.Prepared Statement` _statement)
    (bind _returnvalue (`DbStatement.ExecuteSelect` (`local.Prepared Statement`)))
    (bind _output_get (set `local.Result Data` _returnvalue))
    (bind _result_array (`self.Query Result to Simple Array` _output_get))
    (return _result_array)))

(fn `Query Result to Simple Array`
  (params (`Query Result` :type "QueryResult Structure"))
  (returns (`Result Array` :type "Array of /Game/DataBase/Structs/S_UserData Structure"))
  (locals (`TMP Color` :type "LinearColor Structure") (`Result Item` :type "/Game/DataBase/Structs/S_UserData Structure") (`Results Array` :type "Array of /Game/DataBase/Structs/S_UserData Structure"))
  (for _array_element (`.Rows` (break `QueryResult` `Query Result`))
    (bind (_color _returnvalue) (`GameDatabaseStatics.TryFillColor` _array_element))
    (if _returnvalue
      (set `local.TMP Color` _color)
      (else
        (set `local.TMP Color` (make `LinearColor` 0.0))))
    (bind _fields (break `QueryResultRow` _array_element))
    (bind _output_get (set `local.Result Item` (make `/Game/DataBase/Structs/S_UserData` (`KismetMathLibrary.Conv_Int64ToInt` (`.IntVal` (break `QueryResultField` (`|GetArrayItem` _fields)))) (`.StrVal` (break `QueryResultField` (`|GetArrayItem` _fields 1))) (`KismetMathLibrary.Conv_Int64ToInt` (`.IntVal` (break `QueryResultField` (`|GetArrayItem` _fields 2)))) (`.DblVal` (break `QueryResultField` (`|GetArrayItem` _fields 3))) (`.StrVal` (break `QueryResultField` (`|GetArrayItem` _fields 4))) (`local.TMP Color`))))
    (`KismetArrayLibrary.Array_Add` (`local.Results Array`) _output_get))
  (return (`local.Results Array`)))