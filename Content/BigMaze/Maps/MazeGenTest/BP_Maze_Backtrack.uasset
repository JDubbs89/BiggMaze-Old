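; Test maze generator Blueprint, named for backtracking, that so far builds a square grid border and seeds a path start in the Construction Script.
; PopulateBorder stores edge tiles as flat indices, though its west-edge loop is unconnected and never runs.
; SpawnInstances converts indices to local grid positions for instanced static mesh walls when ShowBorder is on.
; SetInitialTile records the first inner tile in PathTiles; no carving or backtracking exists yet.
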(fn `Populate Border`
  (params (Size :type Integer) (BorderArray :type "Array of Integer"))
  (locals (L_Size :type Integer))
  (bind _l_size (`local.L_Size`))
  (bind _l_size_2 (`local.L_Size`))
  (set `local.L_Size` Size)
  ;[1 1 1] NorthBorder
  (for _index (range (`local.L_Size`))
    (`KismetArrayLibrary.Array_Add` BorderArray _index))
  ;[1 1 1] EastBorder
  (for _index_2 (range 1 (+ (- (`local.L_Size`) 2) 1))
    (`KismetArrayLibrary.Array_Add` BorderArray (+ (* _index_2 _l_size) (- _l_size 1))))
  ;[1 1 1] SouthBorder
  (for _index_3 (range 1 (+ (`local.L_Size`) 1))
    (`KismetArrayLibrary.Array_Add` BorderArray (+ (- _index_3 1) (* _l_size_2 (- _l_size_2 1))))))

(fn `SetInitialTile`
  (bind _output_get (set `self.CurrentTile` (+ (`self.Size`) 1)))
  (`KismetArrayLibrary.Array_Add` (`self.PathTiles`) _output_get))

(fn `UserConstructionScript`
  (`self.Populate Border` (`self.Size`) (`self.Border Tiles`))
  (if (`self.ShowBorder?`)
    (`self.SpawnInstances` (`self.Border Tiles`) (`self.Size`) (`self.Tile Size`) (8.0 8.0 16.0) (`self.InstancedStaticMeshWall`)
      (:`Completed`
        (if (`self.ShowMaze?`)
          (`self.SetInitialTile` :!label _label))))
    (else
      (goto _label))))