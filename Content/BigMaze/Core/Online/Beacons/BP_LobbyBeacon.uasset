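; Online lobby beacon that tracks party members and the host for a multiplayer lobby, naming itself from the local player's Steam persona.
; The host registers itself at start, then connecting beacons are added up to a party size check or disconnected.
; Departures remove the member and attempt host reassignment when the host leaves.
; Multicast-style MC events relay join, leave and host changes through Call events, with debug prints throughout.
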(event `Server Add Self to Party List`
  (params (`Is Host?` :type Boolean))
  ;[1 1 1] When initialized, the beacon will set itself as the designated host.
  (if `Is Host?`
    (`KismetArrayLibrary.Array_Set` (`self.Party Member Beacons`) 0 self true)
    (set `self.Host Beacon` self)))

(event `self.ReceiveBeginPlay`
  ;[1 1 1] When initialized, the beacon will set itself as the designated host.
  (`parent.ReceiveBeginPlay`)
  (bind _returnvalue (`AdvancedSteamFriendsLibrary.GetSteamPersonaName` (`AdvancedSessionsLibrary.GetUniqueNetID` (`GameplayStatics.GetPlayerController` 0))))
  (set `self.Beacon Name` _returnvalue)
  (`self.Server Add Self to Party List` (`self.Is Host?`)))

(event `self.OnClientConnected`
  (params (Client :type "OnlineBeaconBlueprint Object Reference"))
  ;[1 1 1] When a new client connects, add it to the party members list.
  (`parent.OnClientConnected` Client)
  (bind _asbp_lobby_beacon (cast `/Game/BigMaze/Core/Online/Beacons/BP_LobbyBeacon` Client)
    (:`then`
      (if (<= (`KismetArrayLibrary.Array_Length` (`self.Party Member Beacons`)) (`self.Max Party Size`))
        (bind _returnvalue (`KismetArrayLibrary.Array_Add` (`self.Party Member Beacons`) _asbp_lobby_beacon))
        (set `/Game/BigMaze/Core/Online/Beacons/BP_LobbyBeacon.Party Member Index` _returnvalue _asbp_lobby_beacon)
        (set `/Game/BigMaze/Core/Online/Beacons/BP_LobbyBeacon.Is Host?` false _asbp_lobby_beacon)
        (`self.MC Client Joined` _asbp_lobby_beacon)
        (`KismetSystemLibrary.PrintString` (`KismetStringLibrary.Concat_StrStr` (`/Game/BigMaze/Core/Online/Beacons/BP_LobbyBeacon.Beacon Name` _asbp_lobby_beacon) " Joined the Lobby."))
        (else
          (`self.DisconnectClient` Client :!label _label))))
    (:`CastFailed`
      (goto _label))))

(event `MC Client Joined`
  (params (`New Client` :type "/Game/BigMaze/Core/Online/Beacons/BP_LobbyBeacon Object Reference"))
  ;[1 1 1] When a new client connects, add it to the party members list.
  (`self.Client Join` `New Client`))

(event `self.OnClientDisconnected`
  (params (Client :type "OnlineBeaconBlueprint Object Reference"))
  (bind _party_member_beacons (`self.Party Member Beacons`))
  (bind _host_beacon (`self.Host Beacon`))
  ;[1 1 1] When a client leaves, if that client is the host,appoint a new host.
  (`parent.OnClientDisconnected` Client)
  (bind _asbp_lobby_beacon (cast `/Game/BigMaze/Core/Online/Beacons/BP_LobbyBeacon` Client))
  (if (`/Game/BigMaze/Core/Online/Beacons/BP_LobbyBeacon.Is Host?` _asbp_lobby_beacon)
    (bind _party_member_index (`/Game/BigMaze/Core/Online/Beacons/BP_LobbyBeacon.Party Member Index` _asbp_lobby_beacon))
    (`KismetArrayLibrary.Array_Remove` _party_member_beacons _party_member_index)
    (for (_array_element _array_index) _party_member_beacons
      (bind _output_get (set `/Game/BigMaze/Core/Online/Beacons/BP_LobbyBeacon.Is Host?` (== _array_index _party_member_index) _array_element))
      (if _output_get
        (`self.MC Host Disconnect` _host_beacon (`/Game/BigMaze/Core/Online/Beacons/BP_LobbyBeacon.Host Beacon` _array_element))
        (`KismetSystemLibrary.PrintString` (`KismetStringLibrary.Concat_StrStr` (`/Game/BigMaze/Core/Online/Beacons/BP_LobbyBeacon.Beacon Name` _host_beacon) ", the host, has disconnected. Relocating remaining lobby members."))))
    (else
      (`KismetArrayLibrary.Array_Remove` (`self.Party Member Beacons`) _party_member_index)
      (`self.MC Client Disconnect` _asbp_lobby_beacon)
      (`KismetSystemLibrary.PrintString` (`KismetStringLibrary.Concat_StrStr` (`/Game/BigMaze/Core/Online/Beacons/BP_LobbyBeacon.Beacon Name` _asbp_lobby_beacon) " Left the Lobby.")))))

(event `MC Client Disconnect`
  (params (`Disconnected Client` :type "/Game/BigMaze/Core/Online/Beacons/BP_LobbyBeacon Object Reference"))
  ;[1 1 1] When a client leaves, if that client is the host,appoint a new host.
  (`self.Client Disconnect` `Disconnected Client`))

(event `MC Host Disconnect`
  (params (`Old Host Beacon` :type "/Game/BigMaze/Core/Online/Beacons/BP_LobbyBeacon Object Reference") (`New Host Beacon` :type "/Game/BigMaze/Core/Online/Beacons/BP_LobbyBeacon Object Reference"))
  ;[1 1 1] When a client leaves, if that client is the host,appoint a new host.
  (`self.Host Disconnect` `Old Host Beacon` `New Host Beacon`))

(event `self.OnNetworkFailure`
  (params (FailureType :type "ENetworkFailure Enum" :default "NetDriverAlreadyExists"))
  (`KismetSystemLibrary.PrintString` (`|GetEnumeratorNameAsString` FailureType)))

(event `self.OnConnectionFailureBlueprint`
  (`KismetSystemLibrary.PrintString` "AAAAAAAAAAAAAA"))

(fn `UserConstructionScript`)