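; Session beacon that accepts join-beacon client connections to deliver friend session invites and join requests to players in the current game.
; On connect, it matches the client's target ID against PlayerArray, looks up the sender's friend session, then calls the target controller's invite or join-request UI message.
; Separate receive events forward invites and requests to the GameInstance as non-local.
; Plain messages are unhandled; CLRecieveMessage and OnRep_Players are empty.
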(event `CL Recieve Message`)

(event `CL Recieve Invite`
  (params (`Friend Session` :type "/Game/BigMaze/Core/Engine/S_FriendSession Structure"))
  (message `/Game/BigMaze/Core/Characters/PlayerCharacter/Interfaces/BPI_GM.GI Receive Invite` (`GameplayStatics.GetGameInstance`) `Friend Session` false))

(event `CL Recieve Join Req`
  (params (`Friend Session` :type "/Game/BigMaze/Core/Engine/S_FriendSession Structure"))
  (message `/Game/BigMaze/Core/Characters/PlayerCharacter/Interfaces/BPI_GM.GI Receive Request to Join` (`GameplayStatics.GetGameInstance`) `Friend Session` false))

(event `self.OnClientConnected`
  (params (Client :type "OnlineBeaconBlueprint Object Reference"))
  (bind _asbp_session_join_beacon (cast `/Game/BigMaze/Core/Online/Beacons/BP_SessionJoinBeacon` Client))
  (for _array_element (`GameStateBase.PlayerArray` (`GameplayStatics.GetGameState`))
    (if (== (`AdvancedSessionsLibrary.GetUniqueNetIDFromPlayerState` _array_element) (`/Game/BigMaze/Core/Online/Beacons/BP_SessionJoinBeacon.Target Player` _asbp_session_join_beacon))
      (if (not (`/Game/BigMaze/Core/Online/Beacons/BP_SessionJoinBeacon.Is Message?` _asbp_session_join_beacon))
        (bind _returnvalue (`PlayerState.GetPlayerController` _array_element))
        (bind _owning_player (`/Game/BigMaze/Core/Online/Beacons/BP_SessionJoinBeacon.Owning Player` _asbp_session_join_beacon))
        (bind _sessioninfo (`FindFriendSessionCallbackProxy.FindFriendSession` _returnvalue _owning_player)
          (:`OnSuccess`
            (bind _friend (`AdvancedFriendsLibrary.GetFriend` _returnvalue _owning_player))
            (if (`/Game/BigMaze/Core/Online/Beacons/BP_SessionJoinBeacon.Invite?` _asbp_session_join_beacon)
              (bind _array (`|MakeArray` (make `/Game/BigMaze/Core/Engine/S_FriendSession` _friend (`|GetArrayItem` _sessioninfo))))
              (message `/Game/BigMaze/Core/Characters/PlayerCharacter/Interfaces/BPI_UI.UI Invite Recieved` _returnvalue _array)
              (break)
              (else
                (message `/Game/BigMaze/Core/Characters/PlayerCharacter/Interfaces/BPI_UI.UI Join Req Recieved` _returnvalue _array)
                (break))))
          (:`OnFailure`
            (break)))))))

(fn `OnRep_Players`)

(fn `UserConstructionScript`)