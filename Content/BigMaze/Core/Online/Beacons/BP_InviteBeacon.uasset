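; Online beacon that delivers a session invite from one player to another.
; On connection, it passes its session and friend to SRInviteRecieved, which fires the invite-received call and disconnects the client.
; A handler bound at BeginPlay packs both into a friend-session struct with a zero join code and hands it to the GameInstance as a non-local invite.
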(event `self.ReceiveBeginPlay`
  (add `self.Invite Recieved` (delegate `Event Invite Recieved`)))

(event `Event Invite Recieved` :!signature `self.Invite Recieved`
  (params (Session :type "BlueprintSessionResult Structure") (Friend :type "BPFriendInfo Structure"))
  (message `/Game/BigMaze/Core/Characters/PlayerCharacter/Interfaces/BPI_GM.GI Receive Invite` (`GameplayStatics.GetGameInstance`) (make `/Game/BigMaze/Core/Engine/S_FriendSession` Friend Session) false)
  (`KismetSystemLibrary.PrintString` "Invite recieved"))

(event `self.OnConnectedBlueprint`
  (`self.SRInviteRecieved` self (`self.Session`) (`self.Friend`)))

(event `SRInviteRecieved`
  (params (Client :type "/Game/BigMaze/Core/Online/Beacons/BP_InviteBeacon Object Reference") (`Client Session` :type "BlueprintSessionResult Structure") (Friend :type "BPFriendInfo Structure"))
  (`self.Invite Recieved` `Client Session` Friend)
  (`self.DisconnectClient` Client))

(fn `UserConstructionScript`)