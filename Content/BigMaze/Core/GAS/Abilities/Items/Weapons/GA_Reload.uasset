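; Gameplay ability for reloading a weapon in the BigMaze item system.
; On activation it reads two attributes from the owner's Ability System Component and proceeds only if both exist and the first is lower than the second.
; It then starts the reload montage and, without waiting for completion, applies GE_ReloadCost to self, commits and ends.
; A failed check ends the ability immediately.
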(event `self.K2_ActivateAbility`
  (bind (_bsuccessfullyfoundattribute _returnvalue) (`AbilitySystemBlueprintLibrary.GetFloatAttributeFromAbilitySystemComponent` null (struct :`AttributeName` "MaxMagCount" :`Attribute` "/Script/BigMaze_Alpha_0.AS_EquippedItem:MaxMagCount" :`AttributeOwner` "/Script/CoreUObject.Class'/Script/BigMaze_Alpha_0.AS_EquippedItem'")))
  (bind _returnvalue_2 (`self.GetAbilitySystemComponentFromActorInfo`))
  (bind (_bsuccessfullyfoundattribute_2 _returnvalue_3) (`AbilitySystemBlueprintLibrary.GetFloatAttributeFromAbilitySystemComponent` _returnvalue_2 (struct :`AttributeName` "MagCount" :`Attribute` "/Script/BigMaze_Alpha_0.AS_EquippedItem:MagCount" :`AttributeOwner` "/Script/CoreUObject.Class'/Script/BigMaze_Alpha_0.AS_EquippedItem'")))
  (if (and _bsuccessfullyfoundattribute_2 _bsuccessfullyfoundattribute (< _returnvalue_3 _returnvalue))
    (`AbilityTask_PlayMontageAndWait.CreatePlayMontageAndWaitProxy` "Reload" (`self.Montage to Play`) (`self.Play Rate`)
      (:`then`
        (`AbilitySystemComponent.BP_ApplyGameplayEffectToSelf` :`self` _returnvalue_2 :`GameplayEffectClass` "/Game/BigMaze/Core/GAS/GameplayEffects/Items/AmmoTypes/GE_ReloadCost.GE_ReloadCost_C" :`Level` 1.0)
        (`self.K2_CommitAbility`)
        (`self.K2_EndAbility`)))
    (else
      (`self.K2_EndAbility`))))