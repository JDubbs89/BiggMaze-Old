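; Gameplay ability for the AK47's action 0, firing a single hitscan shot per activation.
; After committing, it decrements the equipped item's ammo stat and refreshes the owner's hotbar.
; A camera-forward line trace takes its range and channel from item stats, with debug drawing on.
; A hit actor receives GE_Damage with set-by-caller magnitude from the damage stat, then the ability ends.
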(event `self.K2_ActivateAbility`
  (`self.Set References`)
  (bind _returnvalue (`self.K2_CommitAbility`))
  (if _returnvalue
    (`self.Fire`)
    (else
      (`self.K2_CancelAbility`))))

(event `self.K2_OnEndAbility`
  (params (bWasCancelled :type Boolean)))

(event `CL Update Slot`
  (`/Game/BigMaze/Core/ItemSystem2/Components/AC_InventoryComponent.Inventory Changed` (`/Game/BigMaze/Core/Characters/Character/BP_BiggMazeCharacter.HotbarComponent` (`self.Char`))))

(event `Fire`
  (bind _item__ref_ (`self.Get Equipped Item`))
  (bind (_out_item _out_stat) (`/Game/BigMaze/Core/ItemSystem2/Libraries/BFL_ItemSystem.Get Float Stat by ID` (`self.Get Equipped Item`) 10))
  (bind _camera (`/Game/BigMaze/Core/Characters/Character/BP_BiggMazeCharacter.Camera` (`self.Char`)))
  (bind _returnvalue (`SceneComponent.K2_GetComponentLocation` _camera))
  (`/Game/BigMaze/Core/ItemSystem2/Libraries/BFL_ItemSystem.Decrement Int Stat By ID` (`self.Get Equipped Item`) 5)
  (bind _outhit (`KismetSystemLibrary.LineTraceSingle` :`Start` _returnvalue :`End` (+ _returnvalue (* (`SceneComponent.GetForwardVector` _camera) (`.Out Stat` (`/Game/BigMaze/Core/ItemSystem2/Libraries/BFL_ItemSystem.Get Float Stat by ID` _item__ref_ 4)))) :`TraceChannel` (select `int` (`.Out Stat` (`/Game/BigMaze/Core/ItemSystem2/Libraries/BFL_ItemSystem.Get Int Stat by ID` _item__ref_ 11)) :`0` "TraceTypeQuery3" :`1` "TraceTypeQuery4" :`2` "TraceTypeQuery5" :!type "ETraceTypeQuery Enum") :`DrawDebugType` "ForDuration"))
  (`self.CL Update Slot`)
  (bind (_bblockinghit _binitialoverlap _time _distance _location _impactpoint _normal _impactnormal _physmat _hitactor) (`GameplayStatics.BreakHitResult` _outhit))
  (`/Engine/EditorBlueprintResources/StandardMacros.IsValid` _hitactor
    (:`Is Valid`
      (bind _returnvalue_2 (`AbilitySystemBlueprintLibrary.AssignTagSetByCallerMagnitude` (`self.MakeOutgoingGameplayEffectSpec` "/Game/BigMaze/Core/GAS/GameplayEffects/GE_Damage.GE_Damage_C" (`KismetMathLibrary.Conv_IntToDouble` (`self.GetAbilityLevel`))) (struct :`TagName` "DataTags.OutGoingDamage") _out_stat))
      (`self.K2_ApplyGameplayEffectSpecToTarget` _returnvalue_2 (`AbilitySystemBlueprintLibrary.AbilityTargetDataFromActor` _hitactor))
      (`KismetSystemLibrary.PrintString` (`KismetStringLibrary.Concat_StrStr` (`KismetStringLibrary.Conv_DoubleToString` _out_stat))))
    (:`Is Not Valid`
      _))
  (`self.K2_EndAbility`))