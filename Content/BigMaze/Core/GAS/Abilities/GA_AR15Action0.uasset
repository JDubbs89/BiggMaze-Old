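; GA_AR15Action0 is a gameplay ability for the AR15's action 0, currently a stub with no firing logic.
; On activation it reaches the BP_BiggMazeCharacter pawn through the owning PlayerState and prints the equipped hotbar item's name.
; It then applies GE_Damage to the owner itself rather than to a target.
; It never commits or ends the ability, and the "Shoot!!!!" print is disconnected.
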(event `self.K2_ActivateAbility`
  (bind _asplayer_state (cast `PlayerState` (`self.GetOwningActorFromActorInfo`)))
  (bind _asbp_bigg_maze_character (cast `/Game/BigMaze/Core/Characters/Character/BP_BiggMazeCharacter` (`PlayerState.GetPawn` _asplayer_state)))
  (bind _output_get (set `self.Source Item` (`|GetArrayItem` (`/Game/BigMaze/Core/ItemSystem2/Components/AC_InventoryComponent.Items` (`/Game/BigMaze/Core/Characters/Character/BP_BiggMazeCharacter.HotbarComponent` _asbp_bigg_maze_character)) (`/Game/BigMaze/Core/Characters/Character/BP_BiggMazeCharacter.Equipped Index` _asbp_bigg_maze_character))))
  (`KismetSystemLibrary.PrintString` (`.Name` (break `Item` _output_get)))
  (`self.BP_ApplyGameplayEffectToOwner` "/Game/BigMaze/Core/GAS/GameplayEffects/GE_Damage.GE_Damage_C"))