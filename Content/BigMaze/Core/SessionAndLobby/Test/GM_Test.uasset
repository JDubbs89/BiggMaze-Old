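; Test game mode for Steam friend-session discovery and lobby requests over online beacons.
; BeginPlay creates an advanced session, hosts a BP_LobbyTransactionBeacon, then repeatedly refreshes friend sessions until one is found or attempts run out.
; It sends the first friend a transaction through a spawned beacon, tracked by recipient ID until a reply disconnects it.
; Incoming requests get random accept/decline answers, and progress is reported through debug prints.
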(event `Update Friend Session List`
  (bind _returnvalue (`GameplayStatics.GetPlayerController` 0))
  (bind _results (`GetFriendsCallbackProxy.GetAndStoreFriendsList` _returnvalue)
    (:`then`
      (`KismetSystemLibrary.PrintString` "Attempting to Retrieve Friends List" true true (struct :`R` 1.0 :`G` 1.0 :`A` 1.0) 5.0))
    (:`OnSuccess`
      (for _array_element _results
        (bind ((`UniqueNetId` _uniquenetid) (`PresenceInfo` _presenceinfo)) (break `BPFriendInfo` _array_element))
        (if (`.bIsPlaying` (break `BPFriendPresenceInfo` _presenceinfo))
          (bind _sessioninfo (`FindFriendSessionCallbackProxy.FindFriendSession` _returnvalue _uniquenetid)
            (:`then`
              (`KismetSystemLibrary.PrintString` "Attempting to Find Friend Session" true true (struct :`R` 1.0 :`G` 0.5 :`A` 1.0) 5.0))
            (:`OnSuccess`
              (`KismetArrayLibrary.Array_Add` (`self.Found Friend Sessions`) (make `/Game/BigMaze/Core/Engine/S_FriendSession` _array_element (`|GetArrayItem` _sessioninfo)))
              (`KismetSystemLibrary.PrintString` "Friend Session Found!" true true (struct :`G` 1.0 :`A` 1.0) 10.0))
            (:`OnFailure`
              (`KismetSystemLibrary.PrintString` "Session Not Found" true true (struct :`R` 1.0 :`A` 1.0))))
          (else
            (`KismetSystemLibrary.PrintString` "Friend Not Playing" true true (struct :`R` 1.0 :`B` 0.25 :`A` 1.0)))))
      (`KismetSystemLibrary.PrintString` "Friend List Entries Updated" true true (struct :`G` 1.0 :`A` 1.0) 5.0))
    (:`OnFailure`
      (`KismetSystemLibrary.PrintString` "Failed to Retrieve Friends List" true true (struct :`R` 1.0 :`A` 1.0) 15.0))))

(event `self.ReceiveBeginPlay`
  (bind _found_friend_sessions (`self.Found Friend Sessions`))
  (bind (_output_friendid _output_session) (break `/Game/BigMaze/Core/Engine/S_FriendSession` (`|GetArrayItem` _found_friend_sessions)))
  ; Begin Play, Start Session, Send Requests
  (if (`AdvancedSessionsLibrary.HasOnlineSubsystem` "STEAM")
    (`CreateSessionCallbackProxyAdvanced.CreateAdvancedSession` (`|MakeArray` (`AdvancedSessionsLibrary.MakeLiteralSessionPropertyString` "name" "sessiontest") (`AdvancedSessionsLibrary.MakeLiteralSessionPropertyString` "status" "ballin")) (`GameplayStatics.GetPlayerController` 0) 100 0 false true false true true false true true true true
      (:`OnSuccess`
        (`self.Bind Request Notifies`)
        (`KismetSystemLibrary.PrintString` "Success!")
        (`self.Refresh Friend List` 30
          (:`Success`
            (if (`KismetArrayLibrary.Array_IsNotEmpty` _found_friend_sessions)
              (`self.Send Request` _output_session (`AdvancedSessionsLibrary.Conv_BPUniqueIDToUniqueNetIDRepl` (`.UniqueNetId` (break `BPFriendInfo` _output_friendid))))
              (`KismetSystemLibrary.PrintString` "Sending Request" true true (struct :`R` 1.0 :`G` 1.0 :`A` 1.0) 10.0)
              (else
                (`KismetSystemLibrary.PrintString` "Friends List Empty"))))
          (:`Failed`
            (`KismetSystemLibrary.PrintString` "Friend Sessions Failed to Update." true true (struct :`R` 1.0 :`A` 1.0) 15.0))))
      (:`OnFailure`
        (`KismetSystemLibrary.PrintString` "Failed")))
    (else
      (`KismetSystemLibrary.PrintString` "No Steam"))))

(event `Bind Request Notifies`
  (bind _returnvalue (subsystem `OnlineBeaconSubsystem`))
  ; Starts Hosting a Beacon if Not Already, Binds Event to On Request Received
  (if (not (`OnlineBeaconSubsystem.IsHostingBeacon` _returnvalue "/Game/BigMaze/Core/SessionAndLobby/Beacons/BP_LobbyTransactionBeacon.BP_LobbyTransactionBeacon_C"))
    (`OnlineBeaconSubsystem.StartHostingBeacon` _returnvalue "/Game/BigMaze/Core/SessionAndLobby/Beacons/BP_LobbyTransactionBeacon.BP_LobbyTransactionBeacon_C"))
  (add `/Game/BigMaze/Core/SessionAndLobby/Beacons/BP_LobbyTransactionBeacon.On Request Received` (`OnlineBeaconSubsystem.GetHostingBeacon` _returnvalue "/Game/BigMaze/Core/SessionAndLobby/Beacons/BP_LobbyTransactionBeacon.BP_LobbyTransactionBeacon_C") (`|CreateDelegate` :!event `Request Received`)))

(event `Send Request`
  (params (`Host Session` :type "BlueprintSessionResult Structure") (`Host UID` :type "UniqueNetIdRepl Structure") (`Transaction Type` :type "/Game/BigMaze/Core/SessionAndLobby/Beacons/Data/E_LobbyTransactionType Enum" :default "NewEnumerator0"))
  (bind _returnvalue (`GameplayStatics.GetPlayerController` 0))
  (bind _uniquenetid (`AdvancedSessionsLibrary.GetUniqueNetID` _returnvalue))
  ; Creates a Beacon to Connect to the Desired Session, then Sends a Request
  (bind _info (`self.Get Session Info` `Host Session`)
    (:`then`
      _)
    (:`Not Found`
      _)
    (:`Wrong Type`
      _))
  (bind _sessioninfo (`FindFriendSessionCallbackProxy.FindFriendSession` _returnvalue _uniquenetid)
    (:`OnSuccess`
      (bind _output (`|GetArrayItem` _sessioninfo))
      (bind _info_2 (`self.Get Session Info` _output)
        (:`then`
          _)
        (:`Not Found`
          _)
        (:`Wrong Type`
          _))
      (bind _returnvalue_2 (`|SpawnActorFromClass` "/Game/BigMaze/Core/SessionAndLobby/Beacons/BP_LobbyTransactionBeacon.BP_LobbyTransactionBeacon_C" (`KismetMathLibrary.MakeTransform` (0.0 0.0 -5000.0)) "Undefined" "MultiplyWithRoot" null (make `/Game/BigMaze/Core/SessionAndLobby/Beacons/Data/S_LobbyTransaction` 0 _output `Host Session` _info_2 _info (`AdvancedSessionsLibrary.Conv_BPUniqueIDToUniqueNetIDRepl` _uniquenetid) `Host UID` `Transaction Type`) (`GameplayStatics.GetPlayerController` 0) null))
      (`BlueprintMapLibrary.Map_Add` (`self.OutGoing Requests`) `Host UID` _returnvalue_2)
      (add `/Game/BigMaze/Core/SessionAndLobby/Beacons/BP_LobbyTransactionBeacon.On Request Reply` _returnvalue_2 (`|CreateDelegate` :!event `Reply Received`))
      (`OnlineBeaconConnectProxy.ConnectBySessionAsync` _returnvalue_2 (`.SenderSession_21_EDA07FD44F0970F112BBE7AB3F04F2DA` (break `/Game/BigMaze/Core/SessionAndLobby/Beacons/Data/S_LobbyTransaction` (`/Game/BigMaze/Core/SessionAndLobby/Beacons/BP_LobbyTransactionBeacon.Transaction` _returnvalue_2)))
        (:`then`
          (`KismetSystemLibrary.PrintString` "Sending Request" true true (struct :`R` 1.0 :`G` 1.0 :`A` 1.0)))
        (:`OnSuccess`
          (`KismetSystemLibrary.PrintString` "Successfully Sent Request" true true (struct :`G` 1.0 :`A` 1.0)))
        (:`OnFailure`
          (`KismetSystemLibrary.PrintString` "Request Failed to Send" true true (struct :`R` 1.0 :`A` 1.0)))))
    (:`OnFailure`
      (`KismetSystemLibrary.PrintString` "Session Find Failure" true true (struct :`R` 1.0 :`G` 0.044643 :`A` 1.0) 10.0))))

(event `Reply Received`
  (params (Transaction :type "/Game/BigMaze/Core/SessionAndLobby/Beacons/Data/S_LobbyTransaction Structure") (`Accepted?` :type Boolean))
  (bind ((`RecipientID_31_04890D824A78F5B300FDECA2C84CA640` _recipientid)) (break `/Game/BigMaze/Core/SessionAndLobby/Beacons/Data/S_LobbyTransaction` Transaction))
  (bind _outgoing_requests (`self.OutGoing Requests`))
  ; Receiving and Resolving Requests
  (`OnlineBeaconBlueprint.Disconnect` (`BlueprintMapLibrary.Map_Find` _outgoing_requests _recipientid))
  (`BlueprintMapLibrary.Map_Remove` _outgoing_requests _recipientid)
  (if `Accepted?`
    (`KismetSystemLibrary.PrintString` "Accepted!")
    (else
      (`KismetSystemLibrary.PrintString` "Not Accepted!"))))

(event `Request Received`
  (params (Transaction :type "/Game/BigMaze/Core/SessionAndLobby/Beacons/Data/S_LobbyTransaction Structure"))
  (bind _returnvalue (`KismetMathLibrary.RandomBool`))
  ; Receiving and Resolving Requests
  (`KismetSystemLibrary.PrintString` "Request Received!")
  (`/Game/BigMaze/Core/SessionAndLobby/Beacons/BP_LobbyTransactionBeacon.Resolve Transaction` (`OnlineBeaconSubsystem.GetHostingBeacon` (subsystem `OnlineBeaconSubsystem`) "/Game/BigMaze/Core/SessionAndLobby/Beacons/BP_LobbyTransactionBeacon.BP_LobbyTransactionBeacon_C") Transaction _returnvalue)
  (if _returnvalue
    (`KismetSystemLibrary.PrintString` "Accepting Request!")
    (else
      (`KismetSystemLibrary.PrintString` "Declining Request!"))))

(fn `UserConstructionScript`)