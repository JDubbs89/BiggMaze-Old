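; BP_MessageTransactionBeacon is a session and lobby beacon for message transactions, currently mostly scaffolding.
; Host notifications for received messages and whispers are empty stubs marked TODO, and client connection only casts the client to this beacon class.
; Disconnect, connection failure and network failure events print debug strings tagged with the transaction type, adding the reason or failure type where available.
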(event `Notify Host of Received Message`
  ; TODO: Provisions for Host Recieve Message and Whisper
)

(event `Notify Host of Received Whisper`
  ; TODO: Provisions for Host Recieve Message and Whisper
)

(event `self.OnClientConnected`
  (params (Client :type "OnlineBeaconBlueprint Object Reference"))
  (bind _asbp_message_transaction_beacon (cast `/Game/BigMaze/Core/SessionAndLobby/Beacons/BP_MessageTransactionBeacon` Client)))

(event `self.OnDisconnected`
  (params (Reason :type "EBeaconDisconnectReason Enum" :default "BDR_Client"))
  ; Connection Error/Termination Debug
  (`KismetSystemLibrary.PrintString` (`KismetStringLibrary.Concat_StrStr` (`|GetEnumeratorNameAsString` (`.TransactionType_21_656C26A947A81EF0378E2A84D0AC10CD` (break `/Game/BigMaze/Core/SessionAndLobby/Beacons/Data/S_MessageTransaction` (`self.Transaction`)))) " Transaction Beacon Disconnected. Reason: " (`|GetEnumeratorNameAsString` Reason)) true true (struct :`R` 1.0 :`G` 0.433233 :`A` 1.0) 5.0))

(event `self.OnConnectionFailureBlueprint`
  ; Connection Error/Termination Debug
  (`KismetSystemLibrary.PrintString` (`KismetStringLibrary.Concat_StrStr` (`|GetEnumeratorNameAsString` (`.TransactionType_21_656C26A947A81EF0378E2A84D0AC10CD` (break `/Game/BigMaze/Core/SessionAndLobby/Beacons/Data/S_MessageTransaction` (`self.Transaction`)))) " Transaction Beacon Connection Failure. ") true true (struct :`R` 1.0 :`A` 1.0) 5.0))

(event `self.OnNetworkFailure`
  (params (FailureType :type "ENetworkFailure Enum" :default "NetDriverAlreadyExists"))
  ; Connection Error/Termination Debug
  (`KismetSystemLibrary.PrintString` (`KismetStringLibrary.Concat_StrStr` (`|GetEnumeratorNameAsString` (`.TransactionType_21_656C26A947A81EF0378E2A84D0AC10CD` (break `/Game/BigMaze/Core/SessionAndLobby/Beacons/Data/S_MessageTransaction` (`self.Transaction`)))) " Transaction Beacon Network Failure. Failure Type: " (`|GetEnumeratorNameAsString` FailureType)) true true (struct :`R` 1.0 :`G` 1.0 :`A` 1.0) 5.0))

(fn `UserConstructionScript`)