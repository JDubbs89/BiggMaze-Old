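; BP_LobbyTransactionBeacon is a network beacon for lobby session invites and join requests.
; On client connection, it reads the client beacon's transaction type and routes to a matching notify event, disconnecting the client after invites and join requests.
; Accepted requests call ExtendInvitetoRequestee without a disconnect; all three handler events are still empty stubs.
; Disconnects, connection failures and network failures only print debug strings tagged with the transaction type.
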(event `Notify Host of Join Request`
  (params (Transaction :type "/Game/BigMaze/Core/SessionAndLobby/Beacons/Data/S_LobbyTransaction Structure"))
  ;[0.15 0.1325 0 0.5] TODO: Provisions for Invite/Join Request Notifies
)

(event `Notify Host of Session Invite`
  (params (Transaction :type "/Game/BigMaze/Core/SessionAndLobby/Beacons/Data/S_LobbyTransaction Structure"))
  ;[0.15 0.1325 0 0.5] TODO: Provisions for Invite/Join Request Notifies
)

(event `Extend Invite to Requestee`
  (params (Transaction :type "/Game/BigMaze/Core/SessionAndLobby/Beacons/Data/S_LobbyTransaction Structure"))
  ;[0.15 0.1325 0 0.5] TODO: Provisions for Invite/Join Request Notifies
)

(event `self.OnClientConnected`
  (params (Client :type "OnlineBeaconBlueprint Object Reference"))
  ; Determine which type of transaction is being handled, then notify the sender/recipient
  (bind _asbp_lobby_transaction_beacon (cast `/Game/BigMaze/Core/SessionAndLobby/Beacons/BP_LobbyTransactionBeacon` Client))
  (bind _transaction (`/Game/BigMaze/Core/SessionAndLobby/Beacons/BP_LobbyTransactionBeacon.Transaction` _asbp_lobby_transaction_beacon))
  (switch `/Game/BigMaze/Core/SessionAndLobby/Beacons/Data/E_LobbyTransactionType` (`.TransactionType_13_6F1E133B40E9C6B8CD10FF8C06517624` (break `/Game/BigMaze/Core/SessionAndLobby/Beacons/Data/S_LobbyTransaction` _transaction))
    (:`NewEnumerator0`
      (`self.Notify Host of Session Invite` _transaction)
      (`self.DisconnectClient` Client :!label _label))
    (:`NewEnumerator1`
      (`self.Notify Host of Join Request` _transaction)
      (goto _label))
    (:`NewEnumerator3`
      (`self.Extend Invite to Requestee` (struct)))))

(event `self.OnDisconnected`
  (params (Reason :type "EBeaconDisconnectReason Enum" :default "BDR_Client"))
  ; Connection Failure/Termination Debug
  (`KismetSystemLibrary.PrintString` (`KismetStringLibrary.Concat_StrStr` (`|GetEnumeratorNameAsString` (`.TransactionType_13_6F1E133B40E9C6B8CD10FF8C06517624` (break `/Game/BigMaze/Core/SessionAndLobby/Beacons/Data/S_LobbyTransaction` (`self.Transaction`)))) " Transaction Beacon Disconnected. Reason: " (`|GetEnumeratorNameAsString` Reason)) true true (struct :`R` 1.0 :`G` 0.433233 :`A` 1.0) 5.0))

(event `self.OnConnectionFailureBlueprint`
  ; Connection Failure/Termination Debug
  (`KismetSystemLibrary.PrintString` (`KismetStringLibrary.Concat_StrStr` (`|GetEnumeratorNameAsString` (`.TransactionType_13_6F1E133B40E9C6B8CD10FF8C06517624` (break `/Game/BigMaze/Core/SessionAndLobby/Beacons/Data/S_LobbyTransaction` (`self.Transaction`)))) " Transaction Beacon Connection Failure. ") true true (struct :`R` 1.0 :`A` 1.0) 5.0))

(event `self.OnNetworkFailure`
  (params (FailureType :type "ENetworkFailure Enum" :default "NetDriverAlreadyExists"))
  ; Connection Failure/Termination Debug
  (`KismetSystemLibrary.PrintString` (`KismetStringLibrary.Concat_StrStr` (`|GetEnumeratorNameAsString` (`.TransactionType_13_6F1E133B40E9C6B8CD10FF8C06517624` (break `/Game/BigMaze/Core/SessionAndLobby/Beacons/Data/S_LobbyTransaction` (`self.Transaction`)))) " Transaction Beacon Network Failure. Failure Type: " (`|GetEnumeratorNameAsString` FailureType)) true true (struct :`R` 1.0 :`G` 1.0 :`A` 1.0) 5.0))

(fn `UserConstructionScript`)