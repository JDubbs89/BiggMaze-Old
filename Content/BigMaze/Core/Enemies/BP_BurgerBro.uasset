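; BP_BurgerBro is a melee-style enemy pawn that chases seen pawns and attacks the player.
; PawnSensing turns it toward loud noises and drives AIMoveTo toward seen pawns, arming a two-second attack timer on arrival.
; The attack is a debug-drawn forward sphere trace that ignores "ai" actors and damages "Player"-tagged hits.
; Damage from non-AI instigators lowers Health and turns it toward the causer; no death logic exists, and GetHealth returns zeros.
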(event `self.PawnSensing.OnHearNoise`
  (params (Instigator :type "Pawn Object Reference") (Location :type "Vector Structure (by ref)") (Volume :type "Float (single-precision)"))
  (if (>= Volume 0.6)
    (`self.K2_SetActorRotation` (`KismetMathLibrary.FindLookAtRotation` (`self.K2_GetActorLocation`) Location))))

(event `self.ReceiveAnyDamage`
  (params (Damage :type "Float (single-precision)") (DamageType :type "DamageType Object Reference") (InstigatedBy :type "Controller Object Reference") (DamageCauser :type "Actor Object Reference"))
  (if (not (`self.ActorHasTag` InstigatedBy "ai"))
    (set `self.Health` (- (`self.Health`) Damage))
    (`self.K2_SetActorRotation` (`KismetMathLibrary.FindLookAtRotation` (`self.K2_GetActorLocation`) (`self.K2_GetActorLocation` DamageCauser)))))

(event `self.PawnSensing.OnSeePawn`
  (params (Pawn :type "Pawn Object Reference"))
  (`|AIMoveTo` self (`self.K2_GetActorLocation` Pawn) null 200.0
    (:`OnSuccess`
      (if (not (`KismetSystemLibrary.K2_IsTimerActiveHandle` (`self.Charge`)))
        (bind _returnvalue (`KismetSystemLibrary.K2_SetTimerDelegate` (delegate `SR Damage`) 2.0))
        (set `self.Charge` _returnvalue)))))

(event `SR Damage`
  (bind _returnvalue (`self.K2_GetActorLocation`))
  (bind _outactors (`GameplayStatics.GetAllActorsWithTag` "ai"))
  (bind (_outhit _returnvalue_2) (`KismetSystemLibrary.SphereTraceSingle` _returnvalue (+ _returnvalue (* (`self.GetActorForwardVector`) 500.0)) 150.0 "TraceTypeQuery3" false _outactors "ForOneFrame"))
  (if _returnvalue_2
    (bind (_bblockinghit _binitialoverlap _time _distance _location _impactpoint _normal _impactnormal _physmat _hitactor) (`GameplayStatics.BreakHitResult` _outhit))
    (if (`self.ActorHasTag` _hitactor "Player")
      (`GameplayStatics.ApplyDamage` _hitactor (`self.Attack damage`) (`AIBlueprintHelperLibrary.GetAIController` self) self "/Game/BigMaze/Core/DamageTypes/Standard.Standard_C")
      (else
        (`KismetSystemLibrary.PrintString` (`KismetSystemLibrary.GetClassDisplayName` (`GameplayStatics.GetObjectClass` _hitactor)))))))

(fn `D Retrieve Score`
  (returns (Score :type "/Game/BigMaze/Core/GameModes/Extraction/Structs/S_PlayerScore Structure") (`Equipped Weapon` :type "/Game/BigMaze/Core/ItemAssets/Common/Structs/S_ItemStruct Structure"))
  (return (`self.Score`) (`self.Equipped Weapon`)))

(fn `Get Health`
  (returns (Health :type "Float (double-precision)") (Shields :type "Float (double-precision)") (MaxHealth :type "Float (double-precision)") (Maxshields :type "Float (double-precision)"))
  (return 0.0 0.0 0.0 0.0))

(fn `OnRep_Health`)

(fn `UserConstructionScript`)