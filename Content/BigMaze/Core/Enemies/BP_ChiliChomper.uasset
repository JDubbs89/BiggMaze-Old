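; BP_ChiliChomper is an enemy pawn that roams around its spawn location until PawnSensing spots a pawn.
; Sighting permanently ends roaming: it faces and moves toward the pawn, jumping on arrival.
; An overlap collider drives a DoOnce-gated chomp loop, damaging Player-tagged targets at a randomized interval.
; Damage from non-"ai" instigators lowers Health, whose RepNotify destroys the actor at zero.
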(event `self.ReceiveTick`
  (params (DeltaSeconds :type "Float (single-precision)")))

(event `self.ReceiveBeginPlay`
  (`self.Roam`)
  (set `self.ChompTimer` (`KismetMathLibrary.RandomFloatInRange` 0.3 0.7)))

(event `Roam`
  (bind _wanderrange (`self.WanderRange`))
  (bind (_initlocation_x _initlocation_y _initlocation_z) (`KismetMathLibrary.BreakVector` (`self.InitLocation`)))
  (set `self.InitLocation` (`self.K2_GetActorLocation`))
  (if (not (`self.iSeeYou`)) :!label _label
    (`|AIMoveTo` self (`KismetMathLibrary.MakeVector` (+ _initlocation_x (* _wanderrange (`KismetMathLibrary.RandomIntegerInRange` -1 1))) (+ _initlocation_y (* _wanderrange (`KismetMathLibrary.RandomIntegerInRange` -1 1))) _initlocation_z) null 50.0
      (:`OnSuccess`
        _)
      (:`OnFail`
        _))
    (`KismetSystemLibrary.Delay` 0.01)
    (goto _label)))

(event `self.ReceiveAnyDamage`
  (params (Damage :type "Float (single-precision)") (DamageType :type "DamageType Object Reference") (InstigatedBy :type "Controller Object Reference") (DamageCauser :type "Actor Object Reference"))
  (if (not (`self.ActorHasTag` InstigatedBy "ai"))
    (set `self.Health` (- (`self.Health`) Damage))))

(event `self.PawnSensing.OnSeePawn`
  (params (Pawn :type "Pawn Object Reference"))
  (bind _returnvalue (`self.K2_GetActorLocation` Pawn))
  (set `self.iSeeYou` true)
  (`|ExecutionSequence`
    (:`then_0`
      (`|AIMoveTo` self _returnvalue null 150.0
        (:`OnSuccess`
          (`self.Jump`))))
    (:`then_1`
      (`self.K2_SetActorRotation` (`KismetMathLibrary.FindLookAtRotation` (`self.K2_GetActorLocation`) _returnvalue)))))

(event `self.CHOMP_cOLLISION.OnComponentBeginOverlap`
  (params (OverlappedComponent :type "PrimitiveComponent Object Reference") (OtherActor :type "Actor Object Reference") (OtherComp :type "PrimitiveComponent Object Reference") (OtherBodyIndex :type Integer) (bFromSweep :type Boolean) (SweepResult :type "HitResult Structure (by ref)"))
  (set `self.Target` OtherActor)
  (set `self.isChomping` true)
  (`self.CHOMP`))

(event `CHOMP`
  (bind _target (`self.Target`))
  (if (`self.ActorHasTag` _target "Player") :!label _label_2
    (`/Engine/EditorBlueprintResources/StandardMacros.DoOnce` false :!label _label_3
      (:`Completed`
        (`GameplayStatics.ApplyDamage` _target (`self.Damage`) null self)
        (`GameplayStatics.PlaySoundAtLocation` "/Game/BigMaze/Core/Enemies/chomp.chomp" (`self.K2_GetActorLocation`) (struct) 1.0 1.0 0.34 "/Game/MilitaryWeapDark/Sound/Attenuation/WeaponHandling_att.WeaponHandling_att" null null null)
        (`KismetSystemLibrary.Delay` (`self.ChompTimer`))
        (`|ExecutionSequence`
          (:`then_0`
            (goto _label_3 :!via `Reset`))
          (:`then_1`
            (if (`self.isChomping`)
              (goto _label_2))))))))

(event `self.CHOMP_cOLLISION.OnComponentEndOverlap`
  (params (OverlappedComponent :type "PrimitiveComponent Object Reference") (OtherActor :type "Actor Object Reference") (OtherComp :type "PrimitiveComponent Object Reference") (OtherBodyIndex :type Integer))
  (set `self.isChomping` false))

(fn `OnRep_Health`
  (if (<= (`self.Health`) 0.0)
    (`self.K2_DestroyActor`)))

(fn `UserConstructionScript`)