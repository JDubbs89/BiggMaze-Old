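; BP_Squashbuckler is a BigMaze enemy that wanders near its location and pursues what it sees.
; Patrol loops random navmesh moves with pauses; PawnSensing sightings set ISeeYou, move it toward the pawn and turn it to face.
; An Attack event, uncalled here, sphere-traces forward to damage Player-tagged actors.
; Incoming standard damage must meet HealthComp's penetration level; health depletion triggers physics ragdoll, then destruction.
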(event `self.ReceiveBeginPlay`
  ;[0 0.3203 1] BeginPlay
  (`self.Patrol`))

(event `self.ReceiveAnyDamage`
  (params (Damage :type "Float (single-precision)") (DamageType :type "DamageType Object Reference") (InstigatedBy :type "Controller Object Reference") (DamageCauser :type "Actor Object Reference"))
  (bind _healthcomp (`self.HealthComp`))
  ;[0.6641 1 0] Damage and Death
  (bind _asbp_standard_damage (cast `/Game/BigMaze/Core/DamageTypes/BP_StandardDamage` DamageType))
  (if (>= (`/Game/BigMaze/Core/DamageTypes/BP_StandardDamage.HealthPenLevel` _asbp_standard_damage) (`/Game/BigMaze/Core/Characters/PlayerCharacter/Components/BP_SimpleHealthComp.PenLevel` _healthcomp))
    (`/Game/BigMaze/Core/Characters/PlayerCharacter/Components/BP_SimpleHealthComp.SR Update Health` _healthcomp Damage)))

(event `Patrol`
  ;[0 1 0.5547] Patrols for Character
  (set `self.InitLocation` (`self.K2_GetActorLocation`))
  (if (not (`self.iSeeYou`))
    (`/Engine/EditorBlueprintResources/StandardMacros.DoOnce` false :!label _label
      (:`Completed`
        (bind _randomlocation (`NavigationSystemV1.K2_GetRandomLocationInNavigableRadius` (`self.InitLocation`) 500.0 null null))
        (`|AIMoveTo` self _randomlocation null 50.0
          (:`OnSuccess`
            _)
          (:`OnFail`
            _))
        (`KismetSystemLibrary.Delay` 3.0)
        (`|ExecutionSequence`
          (:`then_0`
            (goto _label :!via `Reset`))
          (:`then_1`
            (`self.Patrol`)))))
    (else
      (`KismetSystemLibrary.RetriggerableDelay` 3.0)
      (if (not (`self.iSeeYou`))
        (`self.Patrol`)))))

(event `self.HealthComp.Health Depleted`
  (params (`Overflow Damage` :type "Float (double-precision)"))
  ;[0.6641 1 0] Damage and Death
  (`PrimitiveComponent.SetSimulatePhysics` (`self.Mesh`) true)
  (`ActorComponent.Deactivate` (`self.CharacterMovement`))
  (`KismetSystemLibrary.Delay` 3.0)
  (`self.K2_DestroyActor`))

(event `Attack`
  (bind _returnvalue (`self.K2_GetActorLocation`))
  ;[1 0.2812 0] Attack
  (bind _outactors (`GameplayStatics.GetAllActorsWithTag` "ai"))
  (bind _outhit (`KismetSystemLibrary.SphereTraceSingle` _returnvalue (+ _returnvalue (* (`self.GetActorForwardVector`) 500.0)) 100.0 "TraceTypeQuery3" false _outactors "ForOneFrame"))
  (bind (_bblockinghit _binitialoverlap _time _distance _location _impactpoint _normal _impactnormal _physmat _hitactor) (`GameplayStatics.BreakHitResult` _outhit))
  (if (and (`self.ActorHasTag` _hitactor "Player") _bblockinghit)
    (`GameplayStatics.ApplyDamage` _hitactor (`self.Damage`) (`AIBlueprintHelperLibrary.GetAIController` self) self "/Game/BigMaze/Core/DamageTypes/Standard.Standard_C")))

(event `self.PawnSensing.OnSeePawn`
  (params (Pawn :type "Pawn Object Reference"))
  ;[1 0 0.04687] Executes on Enemy Seeing Player
  (`/Engine/EditorBlueprintResources/StandardMacros.IsValid` Pawn
    (:`Is Valid`
      (set `self.iSeeYou` true)
      (`|ExecutionSequence`
        (:`then_0`
          (set `self.Target Loc` (`self.K2_GetActorLocation` Pawn))
          (`|AIMoveTo` self (`self.Target Loc`) null 150.0))
        (:`then_1`
          (`self.K2_SetActorRotation` (`KismetMathLibrary.FindLookAtRotation` (`self.K2_GetActorLocation`) (`self.Target Loc`))))))
    (:`Is Not Valid`
      (set `self.iSeeYou` false)
      (`self.Patrol`))))

(fn `D Retrieve Score`
  (returns (Score :type "/Game/BigMaze/Core/GameModes/Extraction/Structs/S_PlayerScore Structure") (`Equipped Weapon` :type "/Game/BigMaze/Core/ItemAssets/Common/Structs/S_ItemStruct Structure"))
  (return (`self.Score Data`) (`self.Equipped Weapon`)))

(fn `Get Health`
  (returns (Health :type "Float (double-precision)") (Shields :type "Float (double-precision)") (MaxHealth :type "Float (double-precision)") (Maxshields :type "Float (double-precision)"))
  (return 0.0 0.0 0.0 0.0))

(fn `UserConstructionScript`)