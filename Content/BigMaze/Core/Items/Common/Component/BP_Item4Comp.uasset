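; BP_Item4Comp is an item component for BigMaze that declares inventory and weapon operations alongside typed attribute readers.
; The Get Attr functions look up a key in a map, convert the string value to float, int, string or bool, and also return whether it was found.
; Item, inventory, reload, equip and use functions are stubs returning failure or default values, with no logic in this file.
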(fn `Add Item`
  (params (Item :type "/Game/BigMaze/Core/Items/Common/Structs/S_Item3 Structure") (`Inventory?` :type Boolean) (`Ammo?` :type Boolean))
  (returns (`Success?` :type Boolean))
  (return false))

(fn `Drop Item`
  (params (Item :type "/Game/BigMaze/Core/Items/Common/Structs/S_Item3 Structure") (Amount :type Integer) (Index :type Integer) (Inventory :type Boolean) (Ammo :type Boolean))
  (returns (Success :type Boolean))
  (return false))

(fn `Get Bool Attr`
  (params (Map :type "Map of String to String") (Key :type String))
  (returns (Out :type Boolean) (ReturnValue :type Boolean))
  (bind (_value _returnvalue) (`BlueprintMapLibrary.Map_Find` Map Key))
  (return (== _value "true") _returnvalue))

(fn `Get Float Attr`
  (params (Map :type "Map of String to String") (Key :type String))
  (returns (Out :type "Float (double-precision)") (ReturnValue :type Boolean))
  (bind (_value _returnvalue) (`BlueprintMapLibrary.Map_Find` Map Key))
  (return (`KismetStringLibrary.Conv_StringToDouble` _value) _returnvalue))

(fn `Get Int Attr`
  (params (Map :type "Map of String to String") (Key :type String))
  (returns (Out :type Integer) (ReturnValue :type Boolean))
  (bind (_value _returnvalue) (`BlueprintMapLibrary.Map_Find` Map Key))
  (return (`KismetStringLibrary.Conv_StringToInt` _value) _returnvalue))

(fn `Get Item`
  (params (Inventory :type Boolean) (`Uses Space` :type Boolean) (`Item Name` :type String))
  (returns (Item :type "/Game/BigMaze/Core/Items/Common/Structs/S_Item3 Structure") (Found :type Boolean))
  (return (struct) false))

(fn `Get String Attr`
  (params (Map :type "Map of String to String") (Key :type String))
  (returns (Out :type String) (ReturnValue :type Boolean))
  (bind (_value _returnvalue) (`BlueprintMapLibrary.Map_Find` Map Key))
  (return _value _returnvalue))

(fn `Reload Weapon`
  (params (Weapon :type "/Game/BigMaze/Core/Items/Common/Structs/S_Item3 Structure"))
  (returns (Success :type Boolean))
  (return false))

(fn `Remove Item`
  (params (Item :type "/Game/BigMaze/Core/Items/Common/Structs/S_Item3 Structure") (Amount :type Integer) (Index :type Integer) (`Use Index` :type Boolean) (Inventory :type Boolean))
  (returns (Excess :type "/Game/BigMaze/Core/Items/Common/Structs/S_Item3 Structure") (Success :type Boolean))
  (return (struct) false))

(fn `Retrieve Component Ref`
  (returns (Component :type "/Game/BigMaze/Core/Characters/PlayerCharacter/Components/AC_Inventory Object Reference"))
  (return null))

(fn `Secondary Use Item`
  (params (Type :type "/Game/BigMaze/Core/Items/Common/Structs/S_Item3 Structure") (`Hotbar Index` :type Integer) (Press :type Boolean))
  (returns (Success :type Boolean))
  (return false))

(fn `Update Equipped Weapon`
  (params (`Equip Index` :type Integer))
  (returns (`Out Item` :type "/Game/BigMaze/Core/Items/Common/Structs/S_Item3 Structure") (`Out Index` :type Integer))
  (return (struct) 0))

(fn `Use Item`
  (params (Type :type "/Game/BigMaze/Core/Items/Common/Structs/S_Item3 Structure") (`Hotbar Index` :type Integer) (Press :type Boolean))
  (returns (Success :type Boolean))
  (return false))