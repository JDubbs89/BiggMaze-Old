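; AC_PlayerStatComponent is a player stat component that feeds a current and maximum stat value to the HUD through a view model.
; On BeginPlay it updates the existing view model, or constructs a BP_StatViewModel seeded with both values if none is valid.
; The StatonRepOverride event, named as a replication callback, pushes both values to the view model again.
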(event `self.ReceiveBeginPlay`
  ; Initialize View Model for HUD Updates
  (bind _view_model (`self.View Model`)
    (:`then`
      (`/Game/BigMaze/Core/UI/ViewModels/BP_StatViewModel.SetCurrentStat` _view_model (`self.Stat`))
      (`/Game/BigMaze/Core/UI/ViewModels/BP_StatViewModel.SetMaxStat` _view_model (`self.MaxStat`)))
    (:`else`
      (bind _returnvalue (`|GenericCreateObject` "/Game/BigMaze/Core/UI/ViewModels/BP_StatViewModel.BP_StatViewModel_C" (`self.Stat`) (`self.MaxStat`)))
      (set `self.View Model` _returnvalue))))

(event `self.Stat OnRep Override`
  (bind _view_model (`self.View Model`))
  (`/Game/BigMaze/Core/UI/ViewModels/BP_StatViewModel.SetCurrentStat` _view_model (`self.Stat`))
  (`/Game/BigMaze/Core/UI/ViewModels/BP_StatViewModel.SetMaxStat` _view_model (`self.MaxStat`)))