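; Generic replicated stat component that holds a clamped value, such as health or stamina, and broadcasts increase, decrease and depletion events.
; SRUpdateStat applies additive changes, fires the matching event and prints the new value.
; When regeneration is enabled, decreases stop the regen timer, then restart it after a retriggerable delay, looping until the stat is full.
; OnRep_Stat calls an overridable hook and reports depletion with optional overflow, governed by flags.
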(event `Stat OnRep Override`)

(event `SR Update Stat`
  (params (Additive :type "Float (double-precision)"))
  (bind _stat (`self.Stat`))
  (set `self.Last Stat Change` Additive)
  (set `self.Stat On Last Update` (`self.Stat`))
  (bind _output_get (set `self.Stat` (`KismetMathLibrary.FClamp` (+ Additive (`self.Stat`)) 0.0 (`self.MaxStat`))))
  (`KismetSystemLibrary.PrintString` (`KismetStringLibrary.Conv_DoubleToString` _output_get))
  (if (>= _output_get (`self.Stat On Last Update`))
    (`self.Stat Increased` _stat)
    (else
      (`self.Stat Decreased` _stat)
      (if (`self.Regenerate Stat`)
        (`KismetSystemLibrary.K2_ClearAndInvalidateTimerHandle` (`self.RegenTimer`))
        (`KismetSystemLibrary.RetriggerableDelay` (`self.Recharge Delay`))
        (bind _returnvalue (`KismetSystemLibrary.K2_SetTimerDelegate` (`|CreateDelegate` :!event `Regenerate`) (`self.Recharge Interval`) true))
        (set `self.RegenTimer` _returnvalue)))))

(event `Regenerate`
  (`self.SR Update Stat` (`self.Regeneration Additive`))
  (if (== (`self.Stat`) (`self.MaxStat`))
    (`KismetSystemLibrary.K2_ClearAndInvalidateTimerHandle` (`self.RegenTimer`))))

(fn `OnRep_Stat`
  (`self.Stat OnRep Override`)
  (if (`/Game/UlimateBlueprintPack/System/Blueprints/UBPP_FunctionLibrary.Smaller Than or Zero (Float)` (`self.Stat`))
    (`self.Stat Depleted` (`KismetMathLibrary.SelectFloat` 0.0 (`KismetMathLibrary.SelectFloat` (+ (`self.Stat On Last Update`) (`self.Last Stat Change`)) 0.0 (`self.Pass Overflow Decrease When Depleted?`)) (or (not (`self.Deny Overflow Depletion on Full`)) (== (`self.Stat On Last Update`) (`self.MaxStat`)))))))