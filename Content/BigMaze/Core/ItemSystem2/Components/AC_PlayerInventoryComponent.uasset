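; Player inventory component for the maze character that mirrors item slots to the HUD and grants gameplay abilities from equipped items.
; BeginPlay caches the owning character, creates an inventory view model if missing and fills the HUD slots.
; Equip, unequip and inventory-change events extend parent logic with slot update messages.
; SR-prefixed events clear and grant GAS abilities by item level, tracking spec handles for removal.
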(event `self.ReceiveBeginPlay`
  (`parent.ReceiveBeginPlay`)
  (bind _asbp_bigg_maze_character (cast `/Game/BigMaze/Core/Characters/Character/BP_BiggMazeCharacter` (`self.GetOwner`)))
  (set `self.Owning Character` _asbp_bigg_maze_character)
  (`self.View Model`
    (:`then`
      _)
    (:`else`
      (bind _returnvalue (`|GenericCreateObject` "/Game/BigMaze/Core/UI/ViewModels/BP_InventoryViewModel.BP_InventoryViewModel_C" (`self.Items`)))
      (set `self.View Model` _returnvalue)))
  (for (_array_element _array_index) (`self.Items`)
    (message `/Game/BigMaze/Core/ItemSystem2/Interfaces/BPI_InventoryInteraction.Update Slot` (`PlayerController.GetHUD` (`Pawn.GetLocalViewingPlayerController` (`self.Owning Character`))) (make `/Game/BigMaze/Core/ItemSystem2/Misc/S_ItemSlotUpdate` _array_element _array_index (== _array_index 0)))))

(event `self.Equip Item`
  (params (Index :type Integer))
  ;[0.5234 1 0] Equip and Unequip
  (`parent.Equip Item` Index)
  (message `/Game/BigMaze/Core/ItemSystem2/Interfaces/BPI_InventoryInteraction.Update Slot` (`PlayerController.GetHUD` (`Pawn.GetLocalViewingPlayerController` (`self.Owning Character`))) (make `/Game/BigMaze/Core/ItemSystem2/Misc/S_ItemSlotUpdate` (`|GetArrayItem` (`self.Items`) Index) Index true)))

(event `self.Unequip Item`
  (params (Index :type Integer))
  ;[0.5234 1 0] Equip and Unequip
  (`parent.Unequip Item` Index)
  (message `/Game/BigMaze/Core/ItemSystem2/Interfaces/BPI_InventoryInteraction.Update Slot` (`PlayerController.GetHUD` (`Pawn.GetLocalViewingPlayerController` (`self.Owning Character`))) (make `/Game/BigMaze/Core/ItemSystem2/Misc/S_ItemSlotUpdate` (`|GetArrayItem` (`self.Items`) Index) Index)))

(event `SR Equip Item`
  (params (Index :type Integer) (Component :type "/Game/BigMaze/Core/ItemSystem2/Components/AC_PlayerInventoryComponent Object Reference"))
  (bind _equipped_item_abilities (`/Game/BigMaze/Core/ItemSystem2/Components/AC_PlayerInventoryComponent.Equipped Item Abilities` Component))
  (bind ((`Level` _level) (`GameplayAbilities` _gameplayabilities)) (break `Item` (`|GetArrayItem` (`/Game/BigMaze/Core/ItemSystem2/Components/AC_InventoryComponent.Items` Component) Index)))
  ;[0.5234 1 0] Equip and Unequip
  (for _array_element _equipped_item_abilities
    (`AbilitySystemComponent.ClearAbility` (`AbilitySystemBlueprintLibrary.GetAbilitySystemComponent` (`self.GetOwner` Component)) _array_element))
  (for _array_element_2 _gameplayabilities
    (bind _returnvalue (`AbilitySystemComponent.K2_GiveAbility` (`AbilitySystemBlueprintLibrary.GetAbilitySystemComponent` (`self.GetOwner` Component)) _array_element_2 _level -1))
    (`KismetArrayLibrary.Array_Add` _equipped_item_abilities _returnvalue)))

(event `SR Unequip Item`
  (params (Index :type Integer) (Component :type "/Game/BigMaze/Core/ItemSystem2/Components/AC_PlayerInventoryComponent Object Reference"))
  (bind _equipped_item_abilities (`/Game/BigMaze/Core/ItemSystem2/Components/AC_PlayerInventoryComponent.Equipped Item Abilities` Component))
  (bind _returnvalue (`AbilitySystemBlueprintLibrary.GetAbilitySystemComponent` (`self.GetOwner` Component)))
  ;[0.5234 1 0] Equip and Unequip
  (for (_array_element _array_index) _equipped_item_abilities
    (bind (_bisinstance _returnvalue_2) (`AbilitySystemBlueprintLibrary.GetGameplayAbilityFromSpecHandle` _returnvalue _array_element))
    (if (and _bisinstance (`KismetArrayLibrary.Array_Contains` (`.GameplayAbilities` (break `Item` (`|GetArrayItem` (`/Game/BigMaze/Core/ItemSystem2/Components/AC_InventoryComponent.Items` Component) Index))) (`GameplayStatics.GetObjectClass` _returnvalue_2)))
      (`AbilitySystemComponent.ClearAbility` _returnvalue _array_element)
      (`KismetArrayLibrary.Array_Remove` _equipped_item_abilities _array_index))))

(event `self.Inventory Changed`
  (`parent.Inventory Changed`)
  (for (_array_element _array_index) (`self.Items`)
    (message `/Game/BigMaze/Core/ItemSystem2/Interfaces/BPI_InventoryInteraction.Update Slot` (`PlayerController.GetHUD` (`Pawn.GetLocalViewingPlayerController` (`self.Owning Character`))) (make `/Game/BigMaze/Core/ItemSystem2/Misc/S_ItemSlotUpdate` _array_element _array_index (== _array_index (`/Game/BigMaze/Core/Characters/Character/BP_BiggMazeCharacter.Equipped Index` (`self.Owning Character`)))))))