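; Inventory component for BigMaze that stores items in a replicated slot array, prefilled with null items on BeginPlay.
; GiveItem stacks onto a matching slot or fills an empty one within weight and capacity limits, then destroys the pickup actor.
; Equipping grants the item's Gameplay Abilities through the owner's PlayerState ASC, keeping handles to clear on unequip.
; TakeItem is a stub, and an older remainder-splitting add path is disconnected.
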(event Custom|Equip%20Item
  (params (Index :type Integer))
  (bind _items (Variables|Default|GetItems))
  (bind _output (Utilities|Array|Get(acopy) _items Index))
  (bind (_out_item _valid_) (CallFunction|IsItemValid _output))
  (bind (_level _gameplayabilities) (Utilities|Struct|BreakItem _out_item))
  ;[0.3359 1 0] Load An Actor and Mark as Equipped
  (if _valid_
    (for (_array_element _array_index) _gameplayabilities
      (bind _returnvalue (GameplayAbilities|GiveAbility (Utilities|GetASC) _array_element _level _array_index))
      (Utilities|Array|Add (Variables|Default|GetItem%20Equip%20Keys) _returnvalue))
    (Default|CallItemEquipped _out_item Index)))

(event Custom|SR%20Add%20Null%20Items
  (for _index (range 0 (CallFunction|MinusOne(Int) (Variables|Default|GetMax%20Stack%20Capacity)))
    (CallFunction|SetNullItem)
    (Utilities|Array|Add :TargetArray (Variables|Default|GetItems))))

(event Custom|Inventory%20Changed)

(event Custom|Unequip%20Item
  (params (Index :type Integer))
  ;[0.3359 1 0] Load An Actor and Mark as Equipped
  (for (_ _array_index) (Utilities|Struct|BreakItem (Utilities|Array|Get(acopy) (Variables|Default|GetItems) Index))
    (GameplayAbilities|ClearAbility (Utilities|GetASC) (Utilities|Array|Get(acopy) (Variables|Default|GetItem%20Equip%20Keys) _array_index)))
  (Default|CallItemUnequipped Index))

(event EventGiveItem
  (params (Index :type Integer) (Item :type Item%20Structure) (Actor%20to%20Destroy :type A%20Item%20Pickup%20Object%20Reference))
  ;[0.15 0.15 0.15 0.5] Give Item (executed on server)
  (if (.Weight (Utilities|IsNewItemWeightCompliant? Item))
    (bind _out_indexes (CallFunction|FindIndexesCapableOfStacking Item Index))
    (Utilities|IntGreaterThan (Utilities|Array|Length _out_indexes) :!pinned true ; Did we find any stackable indexes?
      (:Greater%20Than
        (bind _out_stacked_item (CallFunction|CombineItems (Utilities|Array|Get(acopy) (Variables|Default|GetItems) (Utilities|Array|Get(acopy) _out_indexes)) Item))
        (Utilities|Array|SetArrayElem (Variables|Default|GetItems) (Utilities|Array|Get(acopy) _out_indexes) _out_stacked_item true) ; Get the first index that is stackable and add onto it.
        (Default|CallItemAdded)
        (Utilities|IsValid Actor%20to%20Destroy
          (:Is%20Valid
            (Actor|DestroyActor Actor%20to%20Destroy) ; Destroy Item Pickup Actor on Successful Add (If Valid)
          )))
      (:Not%20Greater%20Than
        (bind _index (CallFunction|FindFirstEmptyIndex :!pinned true)) ; If no, are there any empty indexes?
        (bind _number_out (Utilities|IntEqualto _index -1)
          (:Equal
            (Development|PrintString "Give Failed (No Empty Indexes)"))
          (:Not%20Equal
            (if (.Stack%20Weight (Utilities|IsNewItemWeightCompliant? Item))
              (Utilities|Array|SetArrayElem (Variables|Default|GetItems) _number_out Item true)
              (Default|CallItemAdded)
              (Utilities|IsValid Actor%20to%20Destroy
                (:Is%20Valid
                  (Actor|DestroyActor Actor%20to%20Destroy) ; Destroy Item Pickup Actor (If Valid)
                ))
              (else
                (Development|PrintString "Give Failed (Stack Exception)")))))))
    (else
      (Development|PrintString "Give Failed (Weight Exception)"))))

(event EventBeginPlay
  (CallFunction|SRAddNullItems))

(fn FindFirstAvailableIndex
  (params (Item :type Item%20Structure%20%28by%20ref%29))
  (bind (_individual_weight _total_weight _stack_weight) (CallFunction|GetItemWeight Item))
  (bind _items (Variables|Default|GetItems))
  (bind _max_stack_capacity (Variables|Default|GetMax%20Stack%20Capacity))
  (bind _max_total_weight (Variables|Default|GetMax%20Total%20Weight))
  (bind (_total_weight_2 _total_stack_weight) (CallFunction|GetItemCombinedWeight _items))
  (if (or (|((x+y)<=z) _total_weight _total_weight_2 _max_total_weight) (== _max_total_weight 0.0))
    (bind (_array_element _array_index) (Utilities|Array|ForEachLoopwithBreak (Variables|Default|GetItems) :!label _label)
      (:LoopBody
        (if (.Valid? (CallFunction|IsItemValid _array_element))
          (if (.Can%20Combine (CallFunction|CanCombineItems? Item _array_element))
            (if (.Has%20Remainder (CallFunction|CanCombineItems? Item _array_element))
              (LocalVariables|SetRemainder%20Item (.Remainder%20Stack (CallFunction|CanCombineItems? Item _array_element)))
              (LocalVariables|SetIndex%20Found%20with%20Remainder true)
              (else
                (LocalVariables|SetFound%20Index _array_index)
                (LocalVariables|SetIndex%20Found? true)
                (goto _label Break))))
          (elif (not (LocalVariables|GetFound%20Empty%20Index))
            (LocalVariables|SetEmpty%20Index _array_index)
            (LocalVariables|SetFound%20Empty%20Index true))))
      (:Completed
        (if (and (or (== _max_stack_capacity 0) (|((x+y)<=z) _stack_weight _total_stack_weight _max_stack_capacity)) (not (select (LocalVariables|GetIndex%20Found?) (LocalVariables|GetIndex%20Found?) (LocalVariables|GetFound%20Empty%20Index))))
          (return (Utilities|Array|Length (Variables|Default|GetItems)) true false 0 "")
          (elif (LocalVariables|GetIndex%20Found%20with%20Remainder)
            (bind (_index _found) (CallFunction|FindFirstAvailableIndex (LocalVariables|GetRemainder%20Item)))
            (return (Math|Integer|SelectInt (Math|Integer|SelectInt (LocalVariables|GetFound%20Index) (LocalVariables|GetEmpty%20Index) (LocalVariables|GetIndex%20Found?)) -1 (select (LocalVariables|GetIndex%20Found?) (LocalVariables|GetIndex%20Found?) (LocalVariables|GetFound%20Empty%20Index))) (select (LocalVariables|GetIndex%20Found?) (LocalVariables|GetIndex%20Found?) (LocalVariables|GetFound%20Empty%20Index)) _found _index (LocalVariables|GetRemainder%20Item))
            (else
              (bind _out_item (CallFunction|SetNullItem))
              (return (Math|Integer|SelectInt (Math|Integer|SelectInt (LocalVariables|GetFound%20Index) (LocalVariables|GetEmpty%20Index) (LocalVariables|GetIndex%20Found?)) -1 (select (LocalVariables|GetIndex%20Found?) (LocalVariables|GetIndex%20Found?) (LocalVariables|GetFound%20Empty%20Index))) (select (LocalVariables|GetIndex%20Found?) (LocalVariables|GetIndex%20Found?) (LocalVariables|GetFound%20Empty%20Index)) false -1 _out_item))))))
    (else
      (return -1 false false 0 ""))))

(fn FindFirstEmptyIndex
  (bind (_array_element _array_index) (Utilities|Array|ForEachLoopwithBreak (Variables|Default|GetItems) :!label _label)
    (:LoopBody
      (if (not (.Valid? (CallFunction|IsItemValid _array_element)))
        (LocalVariables|SetFound%20Index _array_index)
        (goto _label Break)))
    (:Completed
      (return (LocalVariables|GetFound%20Index)))))

(fn FindMatchingItemIndexes
  (params (Item :type Item%20Structure) (Preferred%20Index :type Integer))
  (if (CallFunction|AreItemsEqual? Item (Utilities|Array|Get(acopy) (Variables|Default|GetItems) Preferred%20Index))
    (Utilities|Array|Add (LocalVariables|GetIndexes%20Found) Preferred%20Index))
  (for (_array_element _array_index) (Variables|Default|GetItems)
    (if (CallFunction|AreItemsEqual? Item _array_element)
      (bind _number_out (Utilities|IntEqualto Preferred%20Index _array_index)
        (:Not%20Equal
          (Utilities|Array|Add (LocalVariables|GetIndexes%20Found) _number_out)))))
  (return (LocalVariables|GetIndexes%20Found)))

(fn FindIndexesCapableOfStacking
  (params (In%20Item :type Item%20Structure) (Preferred%20Index :type Integer))
  (bind _indexes (CallFunction|FindMatchingItemIndexes In%20Item Preferred%20Index :!pinned true)) ; Find the indexes that have the same item as is being added
  (for _array_element _indexes
    (if (and (.Weight (Utilities|IsNewItemWeightCompliant? In%20Item)) (Utilities|StackAvailable? In%20Item (Utilities|Array|Get(acopy) (Variables|Default|GetItems) _array_element)))
      (Utilities|Array|Add (LocalVariables|GetIndexes%20Found) _array_element)))
  (return (LocalVariables|GetIndexes%20Found)))

(fn OnRepItems
  (CallFunction|InventoryChanged))

(fn GetFirstAvailableIndex
  (params (Item :type Item%20Structure))
  (bind (_index _found _found_r_index _r_index _r_item) (CallFunction|FindFirstAvailableIndex Item))
  (return _found _index _found_r_index _r_index _r_item))

(fn TakeItem
  (params (Index :type Integer) (Amount :type Integer))
  (return "" false))