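; BP_Extraction_GameState is the Game State for the Extraction mode and maintains a replicated Leaderboard array of player info.
; SRSetPlayers stores a new player by ID and sends the array to that player's controller.
; UpdatePlayerInformation rebuilds entries from each PlayerArray member's info message, pushing the board to its owner inside the same loop.
; The Leaderboard RepNotify is empty, so these events deliver updates explicitly.
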(event `self.ReceiveBeginPlay`)

(event `SR Set Players`
  (params (`New Player` :type "/Game/BigMaze/Core/GameModes/Extraction/Structs/S_PlayerScore Structure") (`New Controller` :type "/Game/BigMaze/Core/Characters/PlayerCharacter/BP_Controller Object Reference"))
  (`KismetArrayLibrary.Array_Set` (`self.Leaderboard`) (`.ID_18_6F442BF5413D1DBC19CA08AB2E8B2C77` (break `/Game/BigMaze/Core/GameModes/Extraction/Structs/S_PlayerScore` `New Player`)) `New Player` true)
  (`/Game/BigMaze/Core/Characters/PlayerCharacter/BP_Controller.Update Leaderboard` `New Controller` (`self.Leaderboard`)))

(event `Update Player Information`
  (for (_array_element _array_index) (`self.PlayerArray`)
    (bind _info (message `/Game/BigMaze/Core/Characters/PlayerCharacter/Interfaces/BPI_Player.Get Player Info` _array_element))
    (`KismetArrayLibrary.Array_Set` (`self.Leaderboard`) _array_index _info true)
    (message `/Game/BigMaze/Core/Characters/PlayerCharacter/Interfaces/BPI_HUD.Update Leaderboard` (`self.GetOwner` _array_element) (`self.Leaderboard`))))

(fn `OnRep_Leaderboard`)

(fn `UserConstructionScript`)