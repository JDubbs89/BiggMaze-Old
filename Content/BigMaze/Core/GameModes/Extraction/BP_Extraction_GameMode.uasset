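; Game mode for the Extraction mode that registers joining players, scores combat and respawns players after death.
; New controllers get an index-based name and ID, and a looping timer caches the game state once available.
; PlayerDeath updates death, kill and assist stats using the ScoringRules table, then refreshes the game state's player information.
; It also computes a formula-based death score from character stats before possessing a new character at a random tagged start.
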(event `Player Death`
  (params (Controller :type "/Game/BigMaze/Core/Characters/PlayerCharacter/BP_Controller Object Reference") (Character :type "/Game/BigMaze/Core/Characters/PlayerCharacter/BP_Character Object Reference") (`Kill Credit` :type "/Game/BigMaze/Core/Characters/PlayerCharacter/BP_PlayerState Object Reference") (`Assist Credit` :type "Array of /Game/BigMaze/Core/Characters/PlayerCharacter/BP_PlayerState Object Reference"))
  (bind _player_score (`/Game/BigMaze/Core/Characters/PlayerCharacter/BP_PlayerState.Player Score` `Kill Credit`))
  (bind (_name _id _kills _deaths _assists _score) (break `/Game/BigMaze/Core/GameModes/Extraction/Structs/S_PlayerScore` _player_score))
  (`|ExecutionSequence`
    (:`then_0`
      (bind _ps (`/Game/BigMaze/Core/Characters/PlayerCharacter/BP_Controller.Retrieve Playerstate` Controller))
      (bind (_name_2 _id_2 _kills_2 _deaths_2 _assists_2 _score_2) (break `/Game/BigMaze/Core/GameModes/Extraction/Structs/S_PlayerScore` (`/Game/BigMaze/Core/Characters/PlayerCharacter/BP_PlayerState.Player Score` _ps)))
      (`/Engine/EditorBlueprintResources/StandardMacros.IncrementInt` _deaths_2
        (:`  `
          (bind _returnvalue (`|GetDataTableRow` (`self.Scoring Rules`) "death")
            (:`then`
              (`|VariableSetRef` _score_2 (+ _score_2 (`.Score_5_1670A4A64D8923E134128FABE9F0AFA1` (break `/Game/BigMaze/Core/GameModes/Extraction/Structs/S_ScoreRule` _returnvalue)))))))))
    (:`then_1`
      (`/Engine/EditorBlueprintResources/StandardMacros.IncrementInt` _kills
        (:`  `
          (`KismetArrayLibrary.Array_Set` (`/Game/BigMaze/Core/GameModes/Extraction/BP_Extraction_GameState.Leaderboard` (`self.Extraction Game State`)) _id _player_score)
          (bind _returnvalue_2 (`|GetDataTableRow` (`self.Scoring Rules`) "kill")
            (:`then`
              (`|VariableSetRef` _score (+ _score (`.Score_5_1670A4A64D8923E134128FABE9F0AFA1` (break `/Game/BigMaze/Core/GameModes/Extraction/Structs/S_ScoreRule` _returnvalue_2)))))))))
    (:`then_2`
      (for _array_element `Assist Credit`
        (if (not (== `Kill Credit` _array_element))
          (bind _player_score_2 (`/Game/BigMaze/Core/Characters/PlayerCharacter/BP_PlayerState.Player Score` _array_element))
          (bind (_name_3 _id_3 _kills_3 _deaths_3 _assists_3 _score_3) (break `/Game/BigMaze/Core/GameModes/Extraction/Structs/S_PlayerScore` _player_score_2))
          (`/Engine/EditorBlueprintResources/StandardMacros.IncrementInt` _assists_3
            (:`  `
              (`KismetArrayLibrary.Array_Set` (`/Game/BigMaze/Core/GameModes/Extraction/BP_Extraction_GameState.Leaderboard` (`self.Extraction Game State`)) _id_3 _player_score_2)
              (bind _returnvalue_3 (`|GetDataTableRow` (`self.Scoring Rules`) "assist")
                (:`then`
                  (`|VariableSetRef` _score_3 (+ _score_3 (`.Score_5_1670A4A64D8923E134128FABE9F0AFA1` (break `/Game/BigMaze/Core/GameModes/Extraction/Structs/S_ScoreRule` _returnvalue_3))))))))))
      (`/Game/BigMaze/Core/GameModes/Extraction/BP_Extraction_GameState.Update Player Information` (`self.Extraction Game State`)))
    (:`then_3`
      (`self.DisableInput` Character Controller)
      (`self.Finalize Death Score` Controller Character)
      (`/Game/BigMaze/Core/GameModes/Extraction/BP_Extraction_GameState.Update Player Information` (`self.Extraction Game State`)))))

(event `self.ReceiveBeginPlay`
  (bind _returnvalue (`KismetSystemLibrary.K2_SetTimerDelegate` (delegate `Init GM`) 0.1 true)))

(event `self.K2_OnLogout`
  (params (ExitingController :type "Controller Object Reference"))
  ;[1 1 1] Disconnection
  (bind _asbp_controller (cast `/Game/BigMaze/Core/Characters/PlayerCharacter/BP_Controller` ExitingController))
  (`KismetArrayLibrary.Array_RemoveItem` (`self.Players`) _asbp_controller))

(event `Init GM`
  (bind _asbp_extraction_game_state (cast `/Game/BigMaze/Core/GameModes/Extraction/BP_Extraction_GameState` (`GameplayStatics.GetGameState`)))
  (set `self.Extraction Game State` _asbp_extraction_game_state)
  (`KismetSystemLibrary.K2_ClearAndInvalidateTimerHandle` (stale `self.ReceiveBeginPlay` _returnvalue)))

(event `self.K2_OnSwapPlayerControllers`
  (params (OldPC :type "PlayerController Object Reference") (NewPC :type "PlayerController Object Reference"))
  ;[1 1 1] Connection
  (bind _asbp_controller (cast `/Game/BigMaze/Core/Characters/PlayerCharacter/BP_Controller` NewPC))
  (bind _returnvalue (`KismetArrayLibrary.Array_Add` (`self.Players`) _asbp_controller))
  (bind _s_playerscore (make `/Game/BigMaze/Core/GameModes/Extraction/Structs/S_PlayerScore` (`KismetStringLibrary.Conv_StringToName` (`KismetStringLibrary.Concat_StrStr` "Player" "" (`KismetStringLibrary.Conv_IntToString` _returnvalue))) _returnvalue 0 0 0 0.0 0.0 0.0 true null))
  (message `/Game/BigMaze/Core/Characters/PlayerCharacter/Interfaces/BPI_Player.Set Player Info` (`Controller.PlayerState` NewPC) _s_playerscore)
  (bind _asbp_extraction_game_state (cast `/Game/BigMaze/Core/GameModes/Extraction/BP_Extraction_GameState` (`GameplayStatics.GetGameState`)))
  (`/Game/BigMaze/Core/GameModes/Extraction/BP_Extraction_GameState.SR Set Players` _asbp_extraction_game_state _s_playerscore (`|GetArrayItem` (`self.Players`) _returnvalue)))

(event `self.K2_PostLogin`
  (params (NewPlayer :type "PlayerController Object Reference"))
  ;[1 1 1] Connection
  (bind _asbp_controller (cast `/Game/BigMaze/Core/Characters/PlayerCharacter/BP_Controller` NewPlayer))
  (bind _returnvalue (`KismetArrayLibrary.Array_Add` (`self.Players`) _asbp_controller))
  (message `/Game/BigMaze/Core/Characters/PlayerCharacter/Interfaces/BPI_Player.Set Player Info` (`Controller.PlayerState` NewPlayer) (make `/Game/BigMaze/Core/GameModes/Extraction/Structs/S_PlayerScore` (`KismetStringLibrary.Conv_StringToName` (`KismetStringLibrary.Concat_StrStr` "Player" "" (`KismetStringLibrary.Conv_IntToString` _returnvalue))) _returnvalue 0 0 0 0.0 0.0 0.0 true null))
  (bind _asbp_extraction_game_state (cast `/Game/BigMaze/Core/GameModes/Extraction/BP_Extraction_GameState` (`GameplayStatics.GetGameState`)))
  (`/Game/BigMaze/Core/GameModes/Extraction/BP_Extraction_GameState.Update Player Information` _asbp_extraction_game_state))

(event `Finalize Death Score`
  (params (Controller :type "/Game/BigMaze/Core/Characters/PlayerCharacter/BP_Controller Object Reference") (Character :type "/Game/BigMaze/Core/Characters/PlayerCharacter/BP_Character Object Reference"))
  ;[1 1 1] Calculate Death Score
  (bind _score (`self.Calculate Death Score` Character))
  (set `/Game/BigMaze/Core/Characters/PlayerCharacter/BP_Controller.Death Score` _score Controller)
  (`self.Spawn Player` Controller))

(fn `Calculate Death Score`
  (params (Character :type "/Game/BigMaze/Core/Characters/PlayerCharacter/BP_Character Object Reference"))
  (returns (Score :type "Float (double-precision)"))
  (locals (`Player Death Order` :type Integer) (`Explosive Damage Taken` :type "Float (double-precision)") (`Postmortem Airtime` :type "Float (double-precision)") (`Damage Taken in LTI` :type "Float (double-precision)") (`Enemies in Close Prox` :type Integer) (`Damage Dealt in LTI` :type "Float (double-precision)") (`Postmortem Distance Travelled (m)` :type "Float (double-precision)") (`Death Score` :type "Float (double-precision)"))
  (bind _player_death_order (`local.Player Death Order`))
  (set `local.Player Death Order` (`/Game/BigMaze/Core/Characters/PlayerCharacter/BP_Character.Death Order` Character))
  (set `local.Damage Dealt in LTI` (`/Game/BigMaze/Core/Characters/PlayerCharacter/BP_Character.Damage Dealt in LTI` Character))
  (set `local.Enemies in Close Prox` (`/Game/BigMaze/Core/Characters/PlayerCharacter/BP_Character.Enemies in Close Proximity` Character))
  (set `local.Explosive Damage Taken` (`/Game/BigMaze/Core/Characters/PlayerCharacter/BP_Character.Explosive Damage Taken` Character))
  (set `local.Postmortem Airtime` (`/Game/BigMaze/Core/Characters/PlayerCharacter/BP_Character.PostMortem Airtime` Character))
  (set `local.Postmortem Distance Travelled (m)` (`/Game/BigMaze/Core/Characters/PlayerCharacter/BP_Character.Postmortem Distance Travelled (m)` Character))
  (bind _output_get (set `local.Death Score` (* (/ (+ (`local.Postmortem Airtime`) (/ (`local.Explosive Damage Taken`) 5.0) (/ (`local.Damage Taken in LTI`) 10.0) (`local.Enemies in Close Prox`) (/ (`local.Damage Dealt in LTI`) 10.0) (* (`local.Postmortem Distance Travelled (m)`) 2.0) (/ 10.0 (* 100.0 _player_death_order))) (`KismetMathLibrary.MultiplyMultiply_FloatFloat` (- (* _player_death_order 100) 100.0) 0.002)) 10.0)))
  (return _output_get))

(fn `Find Random Player Start`
  (returns (`Player Start Transform` :type "Transform Structure (by ref)"))
  (bind _outactors (`GameplayStatics.GetAllActorsOfClassWithTag` "/Script/Engine.PlayerStart" "player"))
  (`KismetSystemLibrary.PrintString` (`KismetStringLibrary.Conv_IntToString` (`KismetArrayLibrary.Array_Length` _outactors)))
  (return (`self.GetTransform` (`KismetArrayLibrary.Array_Random` _outactors))))

(fn `Find Random UIPawn Start`
  (returns (`Player Start Transform` :type "Transform Structure (by ref)"))
  (bind _outactors (`GameplayStatics.GetAllActorsOfClassWithTag` "/Script/Engine.PlayerStart" "uipawn"))
  (return (`self.GetTransform` (`|GetArrayItem` _outactors (`KismetMathLibrary.RandomIntegerInRange` 0 (`KismetArrayLibrary.Array_LastIndex` _outactors))))))

(fn `Spawn Player`
  (params (`Player Controller` :type "/Game/BigMaze/Core/Characters/PlayerCharacter/BP_Controller Object Reference"))
  (bind _returnvalue (`Controller.K2_GetPawn` `Player Controller`))
  (bind _player_controller (`local.Player Controller`))
  (`/Engine/EditorBlueprintResources/StandardMacros.IsValid` _returnvalue
    (:`Is Valid`
      (`self.K2_DestroyActor` _returnvalue))
    (:`Is Not Valid`
      _))
  (bind _returnvalue_2 (`|SpawnActorFromClass` "/Game/BigMaze/Core/Characters/PlayerCharacter/BP_Character.BP_Character_C" (`self.Find Random Player Start`) "Undefined" "MultiplyWithRoot" null null))
  (`Controller.Possess` _player_controller _returnvalue_2)
  (`/Engine/EditorBlueprintResources/StandardMacros.IsValid` (`/Game/BigMaze/Core/Characters/PlayerCharacter/BP_Controller.UIPawn` _player_controller)
    (:`Is Valid`
      (`KismetSystemLibrary.PrintString` "UI Pawn Already Valid" true true (struct :`R` 0.185905 :`G` 1.0 :`A` 1.0)))
    (:`Is Not Valid`
      (bind _ps (message `/Game/BigMaze/Core/Characters/PlayerCharacter/Interfaces/BPI_Player.Retrieve Playerstate` _player_controller))
      (set `/Game/BigMaze/Core/Characters/PlayerCharacter/BP_Controller.Player Index` (`.ID_18_6F442BF5413D1DBC19CA08AB2E8B2C77` (break `/Game/BigMaze/Core/GameModes/Extraction/Structs/S_PlayerScore` (`/Game/BigMaze/Core/Characters/PlayerCharacter/BP_PlayerState.Player Score` _ps))) _player_controller))))

(fn `UserConstructionScript`)