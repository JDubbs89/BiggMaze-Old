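; Game mode that manages a party of up to four players, their spawning and death scoring.
; Login and logout update rosters, Steam-named player info and party HUDs, kicking extra joiners.
; Deaths apply data-table score rules for deaths, kills and assists, compute a stat-based death score and broadcast a killfeed.
; Respawns use random tagged PlayerStarts while tokens remain, otherwise the view switches to a living player.
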(event `self.ReceiveBeginPlay`
  (bind _returnvalue (`KismetSystemLibrary.K2_SetTimerDelegate` (delegate `Init GM`) 0.1 true)))

(event `Init GM`
  (bind _asbp_extraction_game_state (cast `/Game/BigMaze/Core/GameModes/Extraction/BP_Extraction_GameState` (`GameplayStatics.GetGameState`)))
  (set `self.Extraction Game State` _asbp_extraction_game_state)
  (`KismetSystemLibrary.K2_ClearAndInvalidateTimerHandle` (stale `self.ReceiveBeginPlay` _returnvalue)))

(event `self.K2_OnLogout`
  (params (ExitingController :type "Controller Object Reference"))
  ;[1 1 1] Disconnection
  (bind _asplayer_controller (cast `PlayerController` ExitingController))
  (`KismetArrayLibrary.Array_RemoveItem` (`self.Party members`) (`AdvancedSessionsLibrary.GetUniqueNetID` _asplayer_controller))
  (bind _asbp_controller (cast `/Game/BigMaze/Core/Characters/PlayerCharacter/BP_Controller` ExitingController))
  (`KismetArrayLibrary.Array_RemoveItem` (`self.Players`) _asbp_controller)
  (`self.Update Party HUD` (`Controller.PlayerState` _asbp_controller) _asbp_controller))

(event `self.K2_OnSwapPlayerControllers`
  (params (OldPC :type "PlayerController Object Reference") (NewPC :type "PlayerController Object Reference"))
  ;[1 1 1] Connection
)

(event `self.K2_PostLogin`
  (params (NewPlayer :type "PlayerController Object Reference"))
  (bind _uniquenetid (`AdvancedSessionsLibrary.GetUniqueNetID` NewPlayer))
  (bind _playerstate (`Controller.PlayerState` NewPlayer))
  (bind _party_members (`self.Party members`))
  ;[1 1 1] Connection
  (if (< (`KismetArrayLibrary.Array_Length` _party_members) 4)
    (`KismetArrayLibrary.Array_Add` _party_members _uniquenetid)
    (bind _asbp_controller (cast `/Game/BigMaze/Core/Characters/PlayerCharacter/BP_Controller` NewPlayer))
    (bind _returnvalue (`KismetArrayLibrary.Array_Add` (`self.Players`) _asbp_controller))
    (bind _returnvalue_2 (`AdvancedSteamFriendsLibrary.GetSteamPersonaName` _uniquenetid))
    (message `/Game/BigMaze/Core/Characters/PlayerCharacter/Interfaces/BPI_Player.P Set Player Info` _playerstate (make `/Game/BigMaze/Core/GameModes/Extraction/Structs/S_PlayerScore` (`KismetStringLibrary.Conv_StringToName` _returnvalue_2) _returnvalue 0 0 0 0.0 0.0 0.0 true null))
    (message `/Game/BigMaze/Core/Characters/PlayerCharacter/Interfaces/BPI_GM.GS Update Player Info` (`GameplayStatics.GetGameState`))
    (`self.Update Party HUD` _playerstate NewPlayer true)
    (for _array_element (`self.Players`)
      (`KismetSystemLibrary.PrintString` (`AdvancedSessionsLibrary.GetPlayerName` _array_element))
      (`/Game/BigMaze/Core/Characters/PlayerCharacter/BP_Controller.Gameplay Sequence` _array_element))
    (else
      (`AdvancedSessionsLibrary.KickPlayer` NewPlayer "Party Full"))))

(event `Finalize Death Score`
  (params (Controller :type "/Game/BigMaze/Core/Characters/PlayerCharacter/BP_Controller Object Reference") (Character :type "/Game/BigMaze/Core/Characters/PlayerCharacter/BP_Character Object Reference"))
  ;[1 1 1] Calculate Death Score
  (bind _score (`self.Calculate Death Score` Character))
  (set `/Game/BigMaze/Core/Characters/PlayerCharacter/BP_Controller.Death Score` _score Controller)
  (`self.Spawn Player` Controller))

(event `Update Party HUD`
  (params (`Player State` :type "PlayerState Object Reference") (`Player Controller` :type "PlayerController Object Reference") (Join :type Boolean))
  ;[1 1 1] Updates the HUD of all Party Members for Joining/Leaving Member
  (for _array_element (`self.Players`)
    (if Join
      (bind _returnvalue (`PlayerController.GetHUD` _array_element))
      (message `/Game/BigMaze/Core/Characters/PlayerCharacter/Interfaces/BPI_UI.UI Player Join` _returnvalue `Player State` `Player Controller`)
      (else
        (message `/Game/BigMaze/Core/Characters/PlayerCharacter/Interfaces/BPI_UI.UI Player Leave` _returnvalue `Player State` `Player Controller`)))))

(event `/Game/BigMaze/Core/Characters/PlayerCharacter/Interfaces/BPI_GM.GM Spawn Character`
  (params (Controller :type "/Game/BigMaze/Core/Characters/PlayerCharacter/BP_Controller Object Reference"))
  (`self.Spawn Player` Controller))

(event `/Game/BigMaze/Core/Characters/PlayerCharacter/Interfaces/BPI_GM.GM Player Death`
  (params (Controller :type "/Game/BigMaze/Core/Characters/PlayerCharacter/BP_Controller Object Reference") (Character :type "/Game/BigMaze/Core/Characters/PlayerCharacter/BP_Character Object Reference") (`Kill Credit` :type "/Game/BigMaze/Core/Characters/PlayerCharacter/BP_PlayerState Object Reference") (`Assist Credit` :type "Array of /Game/BigMaze/Core/Characters/PlayerCharacter/BP_PlayerState Object Reference (by ref)") (`Last AI Damager` :type "Actor Object Reference") (`Credit AI?` :type Boolean))
  ;[1 1 1] Player Death
  (`self.HandlePlayerDeath` Controller Character `Kill Credit` `Assist Credit` `Last AI Damager` `Credit AI?`))

(fn `Assist Credit Score Update`
  (params (`Kill Creditor` :type "Object Object Reference") (`Damager Array` :type "Array of /Game/BigMaze/Core/Characters/PlayerCharacter/BP_PlayerState Object Reference") (`Credit AI?` :type Boolean))
  (for _array_element `Damager Array`
    (if `Credit AI?`
      (bind _player_score (`/Game/BigMaze/Core/Characters/PlayerCharacter/BP_PlayerState.Player Score` _array_element))
      (bind (_name _id _kills _deaths _assists _score) (break `/Game/BigMaze/Core/GameModes/Extraction/Structs/S_PlayerScore` _player_score))
      (`/Engine/EditorBlueprintResources/StandardMacros.IncrementInt` _assists :!label _label
        (:`  `
          (`KismetArrayLibrary.Array_Set` (`/Game/BigMaze/Core/GameModes/Extraction/BP_Extraction_GameState.Leaderboard` (`self.Extraction Game State`)) _id _player_score)
          (bind _returnvalue (`|GetDataTableRow` (`self.Scoring Rules`) "assist")
            (:`then`
              (`|VariableSetRef` _score (+ _score (`.Score_5_1670A4A64D8923E134128FABE9F0AFA1` (break `/Game/BigMaze/Core/GameModes/Extraction/Structs/S_ScoreRule` _returnvalue))))))))
      (elif (not (== `Kill Creditor` _array_element))
        (goto _label))))
  (message `/Game/BigMaze/Core/Characters/PlayerCharacter/Interfaces/BPI_GM.GS Update Player Info` (`GameplayStatics.GetGameState`)))

(fn `Calculate Death Score`
  (params (Character :type "/Game/BigMaze/Core/Characters/PlayerCharacter/BP_Character Object Reference"))
  (returns (Score :type "Float (double-precision)"))
  (locals (`Player Death Order` :type Integer) (`Explosive Damage Taken` :type "Float (double-precision)") (`Postmortem Airtime` :type "Float (double-precision)") (`Damage Taken in LTI` :type "Float (double-precision)") (`Enemies in Close Prox` :type Integer) (`Damage Dealt in LTI` :type "Float (double-precision)") (`Postmortem Distance Travelled (m)` :type "Float (double-precision)") (`Death Score` :type "Float (double-precision)"))
  (bind _player_death_order (`local.Player Death Order`))
  (set `local.Player Death Order` (`/Game/BigMaze/Core/Characters/PlayerCharacter/BP_Character.Death Order` Character))
  (set `local.Damage Dealt in LTI` (`/Game/BigMaze/Core/Characters/PlayerCharacter/BP_Character.Damage Dealt in LTI` Character))
  (set `local.Enemies in Close Prox` (`/Game/BigMaze/Core/Characters/PlayerCharacter/BP_Character.Enemies in Close Proximity` Character))
  (set `local.Explosive Damage Taken` (`/Game/BigMaze/Core/Characters/PlayerCharacter/BP_Character.Explosive Damage Taken` Character))
  (set `local.Postmortem Airtime` (`/Game/BigMaze/Core/Characters/PlayerCharacter/BP_Character.PostMortem Airtime` Character))
  (set `local.Postmortem Distance Travelled (m)` (`/Game/BigMaze/Core/Characters/PlayerCharacter/BP_Character.Postmortem Distance Travelled (m)` Character))
  (bind _output_get (set `local.Death Score` (* (/ (+ (`local.Postmortem Airtime`) (/ (`local.Explosive Damage Taken`) 5.0) (/ (`local.Damage Taken in LTI`) 10.0) (`local.Enemies in Close Prox`) (/ (`local.Damage Dealt in LTI`) 10.0) (* (`local.Postmortem Distance Travelled (m)`) 2.0) (/ 10.0 (* 100.0 _player_death_order))) (`KismetMathLibrary.MultiplyMultiply_FloatFloat` (- (* _player_death_order 100) 100.0) 0.002)) 10.0)))
  (return _output_get))

(fn `Create Killfeed WIdget`
  (params (`Killed Player` :type "Object Object Reference") (`Kill Creditor` :type "/Game/BigMaze/Core/Characters/PlayerCharacter/BP_PlayerState Object Reference") (`Last AI Damager` :type "Actor Object Reference") (`Credit AI?` :type Boolean))
  (locals (Weapon :type "/Game/BigMaze/Core/ItemAssets/Common/Structs/ItemStruct Structure") (Score :type "/Game/BigMaze/Core/GameModes/Extraction/Structs/S_PlayerScore Structure"))
  (bind (_name _description _icon) (break `/Game/BigMaze/Core/ItemAssets/Common/Structs/ItemStruct` (`local.Weapon`)))
  (bind _returnvalue (`KismetTextLibrary.Conv_NameToText` (`.Name_19_3302F2994C57E384E4FB18A7E9F8A9CF` (break `/Game/BigMaze/Core/GameModes/Extraction/Structs/S_PlayerScore` (`local.Score`)))))
  (bind _ps (message `/Game/BigMaze/Core/Characters/PlayerCharacter/Interfaces/BPI_Player.P Retrieve Playerstate` `Killed Player`))
  (if (and `Credit AI?` (`KismetSystemLibrary.IsValid` `Last AI Damager`))
    (bind (_score _equipped_weapon) (message `/Game/BigMaze/Core/Characters/PlayerCharacter/Interfaces/BPI_Damageable.D Retrieve Score` `Last AI Damager`))
    (set `local.Score` _score)
    (set `local.Weapon` _equipped_weapon)
    (else
      (bind (_index _item) (message `/Game/BigMaze/Core/Characters/PlayerCharacter/Interfaces/BPI_InventoryComp.IC (Char) Get Equipped Item` (`Controller.K2_GetPawn` (`PlayerState.GetPlayerController` `Kill Creditor`))))
      (set `local.Score` (`/Game/BigMaze/Core/Characters/PlayerCharacter/BP_PlayerState.Player Score` `Kill Creditor`))
      (set `local.Weapon` _item)))
  (for _array_element (`GameStateBase.PlayerArray` (`GameplayStatics.GetGameState`))
    (bind _returnvalue_2 (`KismetTextLibrary.Conv_NameToText` (`.Name_19_3302F2994C57E384E4FB18A7E9F8A9CF` (break `/Game/BigMaze/Core/GameModes/Extraction/Structs/S_PlayerScore` (`/Game/BigMaze/Core/Characters/PlayerCharacter/BP_PlayerState.Player Score` _ps)))))
    (message `/Game/BigMaze/Core/Characters/PlayerCharacter/Interfaces/BPI_UI.UI Create Killfeed Widget` (`PlayerState.GetPlayerController` _array_element) _returnvalue _returnvalue_2 _icon)
    (`KismetSystemLibrary.PrintString` (`KismetStringLibrary.Concat_StrStr` (`KismetTextLibrary.Conv_TextToString` _returnvalue) " Killed " (`KismetTextLibrary.Conv_TextToString` _returnvalue_2) "Using " _name))))

(fn `Find Random Player Start`
  (returns (`Player Start Transform` :type "Transform Structure (by ref)"))
  (locals (`Tagged Array` :type "Array of PlayerStart Object Reference"))
  (bind _outactors (`GameplayStatics.GetAllActorsOfClassWithTag` "/Script/Engine.PlayerStart" "player"))
  (if (`self.Test Spawning`)
    (for _array_element _outactors
      (if (`self.ActorHasTag` _array_element "test")
        (`KismetArrayLibrary.Array_Add` (`local.Tagged Array`) _array_element)))
    (return (`self.GetTransform` (`KismetArrayLibrary.Array_Random` (`local.Tagged Array`))))
    (else
      (return (`self.GetTransform` (`KismetArrayLibrary.Array_Random` _outactors))))))

(fn `Find Random UIPawn Start`
  (returns (`Player Start Transform` :type "Transform Structure (by ref)"))
  (bind _outactors (`GameplayStatics.GetAllActorsOfClassWithTag` "/Script/Engine.PlayerStart" "uipawn"))
  (return (`self.GetTransform` (`|GetArrayItem` _outactors (`KismetMathLibrary.RandomIntegerInRange` 0 (`KismetArrayLibrary.Array_LastIndex` _outactors))))))

(fn `GI Get Friend Invites`
  (returns (Invites :type "Array of /Game/BigMaze/Core/Engine/S_FriendSession Structure"))
  (return))

(fn `GI Get Open LAN Sessions`
  (returns (Invites :type "Array of BlueprintSessionResult Structure"))
  (return))

(fn `GI Get Session Status`
  (returns (`Using LAN?` :type Boolean) (`Is Local Instance Host?` :type Boolean))
  (return false false))

(fn `GS Get Leaderboard`
  (returns (Leaderboard :type "Array of /Game/BigMaze/Core/GameModes/Extraction/Structs/S_PlayerScore Structure"))
  (return))

(fn `HandlePlayerDeath`
  (params (`Killed Player` :type "/Game/BigMaze/Core/Characters/PlayerCharacter/BP_Controller Object Reference") (`Killed Character` :type "/Game/BigMaze/Core/Characters/PlayerCharacter/BP_Character Object Reference") (`Kill Creditor` :type "/Game/BigMaze/Core/Characters/PlayerCharacter/BP_PlayerState Object Reference") (`Damager Array` :type "Array of /Game/BigMaze/Core/Characters/PlayerCharacter/BP_PlayerState Object Reference (by ref)") (`Last AI Damager` :type "Actor Object Reference") (`Credit AI?` :type Boolean))
  (bind _killed_character (`local.Killed Character`))
  (bind _killed_player (`local.Killed Player`))
  (bind _credit_ai_ (`local.Credit AI?`))
  (`|ExecutionSequence`
    (:`then_0`
      (`self.Player Death Score Update` (`local.Killed Player`)))
    (:`then_1`
      (`self.Player Kill Credit Score Update` (`local.Kill Creditor`) _credit_ai_))
    (:`then_2`
      (`self.Assist Credit Score Update` (`local.Kill Creditor`) (`local.Damager Array`) _credit_ai_))
    (:`then_3`
      (`self.DisableInput` _killed_character _killed_player)
      (`self.Finalize Death Score` _killed_player _killed_character)
      (message `/Game/BigMaze/Core/Characters/PlayerCharacter/Interfaces/BPI_GM.GS Update Player Info` (`GameplayStatics.GetGameState`)))
    (:`then_4`
      (`self.Create Killfeed WIdget` (`local.Killed Player`) (`local.Kill Creditor`) (`local.Last AI Damager`) (`local.Credit AI?`)))))

(fn `Player Death Score Update`
  (params (`Player Controller` :type "/Game/BigMaze/Core/Characters/PlayerCharacter/BP_Controller Object Reference"))
  (bind _ps (`/Game/BigMaze/Core/Characters/PlayerCharacter/BP_Controller.P Retrieve Playerstate` `Player Controller`))
  (bind (_name _id _kills _deaths _assists _score _deathscore _ping _alive _playerstate _respawntokens) (break `/Game/BigMaze/Core/GameModes/Extraction/Structs/S_PlayerScore` (`/Game/BigMaze/Core/Characters/PlayerCharacter/BP_PlayerState.Player Score` _ps)))
  (`/Engine/EditorBlueprintResources/StandardMacros.IncrementInt` _deaths
    (:`  `
      (bind _returnvalue (`|GetDataTableRow` (`self.Scoring Rules`) "death")
        (:`then`
          (`/Engine/EditorBlueprintResources/StandardMacros.DecrementInt` _respawntokens
            (:`  `
              (`|VariableSetRef` _score (+ _score (`.Score_5_1670A4A64D8923E134128FABE9F0AFA1` (break `/Game/BigMaze/Core/GameModes/Extraction/Structs/S_ScoreRule` _returnvalue))))
              (`|VariableSetRef` _alive))))))))

(fn `Player Kill Credit Score Update`
  (params (`Kill Creditor` :type "/Game/BigMaze/Core/Characters/PlayerCharacter/BP_PlayerState Object Reference") (`Credit AI?` :type Boolean))
  (bind _player_score (`/Game/BigMaze/Core/Characters/PlayerCharacter/BP_PlayerState.Player Score` `Kill Creditor`))
  (bind (_name _id _kills _deaths _assists _score) (break `/Game/BigMaze/Core/GameModes/Extraction/Structs/S_PlayerScore` _player_score))
  (if (not `Credit AI?`)
    (`/Engine/EditorBlueprintResources/StandardMacros.IsValid` `Kill Creditor`
      (:`Is Valid`
        (`/Engine/EditorBlueprintResources/StandardMacros.IncrementInt` _kills
          (:`  `
            (`KismetArrayLibrary.Array_Set` (`/Game/BigMaze/Core/GameModes/Extraction/BP_Extraction_GameState.Leaderboard` (`self.Extraction Game State`)) _id _player_score)
            (bind _returnvalue (`|GetDataTableRow` (`self.Scoring Rules`) "kill")
              (:`then`
                (`|VariableSetRef` _score (+ _score (`.Score_5_1670A4A64D8923E134128FABE9F0AFA1` (break `/Game/BigMaze/Core/GameModes/Extraction/Structs/S_ScoreRule` _returnvalue))))))))))))

(fn `Spawn Player`
  (params (`Player Controller` :type "/Game/BigMaze/Core/Characters/PlayerCharacter/BP_Controller Object Reference"))
  (locals (PS :type "/Game/BigMaze/Core/Characters/PlayerCharacter/BP_PlayerState Object Reference"))
  (bind _returnvalue (`Controller.K2_GetPawn` `Player Controller`))
  (bind _player_controller (`local.Player Controller`))
  (bind _player_controller_2 (`local.Player Controller`))
  (bind (_name _id _kills _deaths _assists _score _deathscore _ping _alive) (break `/Game/BigMaze/Core/GameModes/Extraction/Structs/S_PlayerScore` (`/Game/BigMaze/Core/Characters/PlayerCharacter/BP_PlayerState.Player Score` (`local.PS`))))
  (bind _asbp_player_state (cast `/Game/BigMaze/Core/Characters/PlayerCharacter/BP_PlayerState` (`Controller.PlayerState` `Player Controller`)))
  (set `local.PS` _asbp_player_state)
  (`/Engine/EditorBlueprintResources/StandardMacros.IsValid` _returnvalue
    (:`Is Valid`
      (`self.K2_DestroyActor` _returnvalue))
    (:`Is Not Valid`
      _))
  (if (> (`.RespawnTokens_38_DBA4073246A7CA56F9F66B8DECFD7F1D` (break `/Game/BigMaze/Core/GameModes/Extraction/Structs/S_PlayerScore` (`/Game/BigMaze/Core/Characters/PlayerCharacter/BP_PlayerState.Player Score` (`local.PS`)))) 0)
    (bind _returnvalue_2 (`|SpawnActorFromClass` "/Game/BigMaze/Core/Characters/PlayerCharacter/BP_Character.BP_Character_C" (`self.Find Random Player Start`) "Undefined" "MultiplyWithRoot" null null))
    (`Controller.Possess` _player_controller _returnvalue_2)
    (set `/Game/BigMaze/Core/Characters/PlayerCharacter/BP_Controller.Player Index` _id _player_controller)
    (`|VariableSetRef` _alive true)
    (else
      (for _array_element (`self.Players`)
        (bind _ps (message `/Game/BigMaze/Core/Characters/PlayerCharacter/Interfaces/BPI_Player.P Retrieve Playerstate` _array_element))
        (if (`.Alive_22_7AD1504A45F58D22EFBF9E99B3ECF561` (break `/Game/BigMaze/Core/GameModes/Extraction/Structs/S_PlayerScore` (`/Game/BigMaze/Core/Characters/PlayerCharacter/BP_PlayerState.Player Score` _ps)))
          (bind _return_hud (message `/Game/BigMaze/Core/Characters/PlayerCharacter/Interfaces/BPI_Player.P Spectator Add` _array_element))
          (message `/Game/BigMaze/Core/Characters/PlayerCharacter/Interfaces/BPI_Player.P Set HUD Override` (`/Game/BigMaze/Core/Characters/PlayerCharacter/BP_Controller.HUD` _player_controller_2) _return_hud)
          (`PlayerController.SetViewTargetWithBlend` _player_controller_2 _array_element 0.0 "VTBlend_Linear" 0.0 false)
          (break))))))

(fn `UserConstructionScript`)