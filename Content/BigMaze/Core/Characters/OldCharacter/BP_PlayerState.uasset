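; BP_PlayerState is a player state in BigMaze's OldCharacter folder, holding each player's score record and authority flags.
; PSetPlayerInfo rebuilds PlayerScore from incoming info with current ping, and PSetHasAuthority marks the first PlayerArray entry as server owner.
; SessionInvite checks the session for a join code, notifying the local HUD when found.
; Death, respawn, inventory, spectator and name functions are empty stubs.
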(event `self.ReceiveBeginPlay`)

(event `self.Player Death`)

(event `self.Player Respawn`
  (params (Controller :type "PlayerController Object Reference")))

(event `/Game/BigMaze/Core/Characters/OldCharacter/Interfaces/BPI_Player.P Set Player Info`
  (params (Info :type "/Game/BigMaze/Core/GameModes/Extraction/Structs/S_PlayerScore Structure"))
  (bind (_name _id _kills _deaths _assists _score _deathscore _ping _alive) (break `/Game/BigMaze/Core/GameModes/Extraction/Structs/S_PlayerScore` Info))
  (bind _output_get (set `self.Player Score` (make `/Game/BigMaze/Core/GameModes/Extraction/Structs/S_PlayerScore` _name _id _kills _deaths _assists _score _deathscore (`self.GetPingInMilliseconds`) _alive self))))

(event `/Game/BigMaze/Core/Characters/OldCharacter/Interfaces/BPI_Player.ReceiveSessionInvite`
  (params (`Session to Join` :type "/Game/BigMaze/Core/Engine/S_FriendSession Structure"))
  (bind _extrasettings (`AdvancedSessionsLibrary.GetExtraSettings` (`.Session_6_FF0BD9C24B7AAF1438B0C69692D0BB11` (break `/Game/BigMaze/Core/Engine/S_FriendSession` `Session to Join`))))
  (`AdvancedSessionsLibrary.GetSessionPropertyInt` _extrasettings "joincode"
    (:`Found`
      (message `/Game/BigMaze/Core/Characters/OldCharacter/Interfaces/BPI_UI.UI Invite Recieved` (`PlayerController.GetHUD` (`GameplayStatics.GetPlayerController` 0)) (struct))
      (`KismetSystemLibrary.PrintString` "Invite Received by Game"))
    (:`NotFound`
      (`KismetSystemLibrary.PrintString` "Invite Received, Join Code Unavailable" :!label _label))
    (:`WrongType`
      (goto _label))))

(event `/Game/BigMaze/Core/Characters/OldCharacter/Interfaces/BPI_Player.P Set Has Authority`
  (params (`Has Authority?` :type Boolean))
  (set `self.Has Authority` `Has Authority?`)
  (set `self.Is Server Owner` (== (`|GetArrayItem` (`GameStateBase.PlayerArray` (`GameplayStatics.GetGameState`))) self)))

(fn `OnRep_Has Authority`)

(fn `P Add Weapon to Inventory`
  (params (`Item Obj` :type "Object Object Reference"))
  (returns (Success :type Boolean))
  (return false))

(fn `P Get Equipped Weapon`
  (returns (`Weapon Index` :type Integer) (WeaponObjs :type "Map of Integer to Object Object Reference"))
  (return 0))

(fn `P Get Has Authority or is Server Owner`
  (returns (`Has Authority` :type Boolean) (`Is Server Owner` :type Boolean))
  (return (`self.Has Authority`) (`self.Is Server Owner`)))

(fn `P Get Player Info`
  (returns (Info :type "/Game/BigMaze/Core/GameModes/Extraction/Structs/S_PlayerScore Structure"))
  (return (`self.Player Score`)))

(fn `P Get Player Name`
  (returns (`Player Name` :type Name))
  (return "None"))

(fn `P Inventory Comps Active?`
  (returns (True :type Boolean))
  (return false))

(fn `P Retrieve Playerstate`
  (returns (PS :type "/Game/BigMaze/Core/Characters/OldCharacter/BP_PlayerState Object Reference"))
  (return null))

(fn `P Spectator Add`
  (returns (`Return HUD` :type "/Game/BigMaze/Core/UI/HUD/OnScreen/WBP_HUDMain Object Reference"))
  (return null))

(fn `UserConstructionScript`)