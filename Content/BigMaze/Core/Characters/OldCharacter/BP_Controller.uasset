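; Player controller for BigMaze that handles player startup and relays UI events to the HUD.
; Possession starts invite and message beacons; when ready, the local controller requests a spawn from the GameMode and fades in, with a looping timer to defer HUD creation until pawn inventory components are active.
; Input, health, item, killfeed, leaderboard, invite and interact-prompt events go to the HUD through interface messages.
; Some inventory queries forward to the pawn; most others are stubs.
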(event `self.ReceiveBeginPlay`
  ;[0.2891 1 0] BeginPlay
  (bind _returnvalue (`KismetSystemLibrary.K2_SetTimerDelegate` (delegate `TryAddMapping`) 0.1)))

(event `TryAddMapping`
  (bind _returnvalue (pcsubsystem `EnhancedInputLocalPlayerSubsystem` self))
  ;[0.2891 1 0] BeginPlay
  (`/Engine/EditorBlueprintResources/StandardMacros.IsValid` _returnvalue
    (:`Is Valid`
      (`EnhancedInputSubsystemInterface.AddMappingContext` _returnvalue "/Game/BigMaze/Core/Engine/Inputs/IMC_Default.IMC_Default" 0 (struct))
      (`KismetSystemLibrary.K2_ClearAndInvalidateTimerHandle` (stale `self.ReceiveBeginPlay` _returnvalue)))))

(event `/Game/BigMaze/Core/Characters/OldCharacter/Interfaces/BPI_Player.P Set Controller Ready`
  ;[0.2891 1 0] BeginPlay
  (if (`self.IsLocalPlayerController`)
    (`self.Gameplay Sequence`)))

(event `self.ReceivePossess`
  (params (PossessedPawn :type "Pawn Object Reference"))
  ;[0.2891 1 0] BeginPlay
  (`self.Begin Hosting Invite Beacon`)
  (`self.Begin Hosting Message Beacon`))

(event `EnhancedInput|/Game/BigMaze/Core/Engine/Inputs/Keys/IA_Pause`
  (params (ActionValue :type Boolean) (ElapsedSeconds :type "Float (double-precision)") (TriggeredSeconds :type "Float (double-precision)") (InputAction :type "InputAction Object Reference" :default "/Game/BigMaze/Core/Engine/Inputs/Keys/IA_Pause.IA_Pause"))
  ;[0.2891 1 0] BeginPlay
  (:`Started`
    (message `/Game/BigMaze/Core/Characters/OldCharacter/Interfaces/BPI_UI.UI Toggle Pause Menu` (`self.GetHUD`))))

(event `Gameplay Sequence`
  ;[0.2891 1 0] BeginPlay
  (`|ExecutionSequence`
    (:`then_0`
      (`self.CL Reset HUD`))
    (:`then_1`
      (`self.SR Spawn Player` self self))
    (:`then_2`
      (bind _returnvalue (`KismetSystemLibrary.K2_SetTimerDelegate` (`|CreateDelegate` :!event `Try Create HUD`) 0.1 true)))
    (:`then_3`
      (`WidgetBlueprintLibrary.SetInputMode_GameOnly` self)
      (`PlayerCameraManager.StartCameraFade` (`GameplayStatics.GetPlayerCameraManager` 0) 2.0 0.0 1.5 (struct :`A` 1.0) true false))))

(event `/Game/BigMaze/Core/Characters/OldCharacter/Interfaces/BPI_UI.UI Join Req Recieved`
  (params (`Join Request` :type "/Game/BigMaze/Core/Engine/S_FriendSession Structure"))
  (message `/Game/BigMaze/Core/Characters/OldCharacter/Interfaces/BPI_UI.UI Join Req Recieved` (`self.GetHUD`) `Join Request`))

(event `SR Spawn Player`
  (params (Controller :type "/Game/BigMaze/Core/Characters/OldCharacter/BP_Controller Object Reference"))
  ;[0.2891 1 0] BeginPlay
  (message `/Game/BigMaze/Core/Characters/OldCharacter/Interfaces/BPI_GM.GM Spawn Character` (`GameplayStatics.GetGameMode`) Controller))

(event `self.ReceiveUnPossess`
  (params (UnpossessedPawn :type "Pawn Object Reference"))
  ;[0.2891 1 0] BeginPlay
)

(event `Begin Hosting Invite Beacon`
  ;[1 0 0.9375] Host Invite and Message Beacons
  (if (not (`OnlineBeaconSubsystem.IsHostingBeacon` (subsystem `OnlineBeaconSubsystem`) "/Game/BigMaze/Core/Online/Beacons/BP_InviteBeacon.BP_InviteBeacon_C"))
    (`OnlineBeaconSubsystem.StartHostingBeacon` (subsystem `OnlineBeaconSubsystem`) "/Game/BigMaze/Core/Online/Beacons/BP_InviteBeacon.BP_InviteBeacon_C")))

(event `/Game/BigMaze/Core/Characters/OldCharacter/Interfaces/BPI_UI.UI Invite Recieved`
  (params (Invite :type "/Game/BigMaze/Core/Engine/S_FriendSession Structure"))
  (message `/Game/BigMaze/Core/Characters/OldCharacter/Interfaces/BPI_UI.UI Invite Recieved` (`self.GetHUD`) Invite))

(event `Try Create HUD`
  (bind _returnvalue (`self.GetHUD`))
  ;[0.2891 1 0] BeginPlay
  (bind _true (message `/Game/BigMaze/Core/Characters/OldCharacter/Interfaces/BPI_Player.P Inventory Comps Active?` (`self.K2_GetPawn`)))
  (if (and _true (`KismetSystemLibrary.IsValid` (`self.GetHUD`)))
    (`KismetSystemLibrary.K2_ClearAndInvalidateTimerHandle` (stale `Gameplay Sequence` _returnvalue))
    (message `/Game/BigMaze/Core/Characters/OldCharacter/Interfaces/BPI_UI.UI CreateHUD` _returnvalue)
    (bind (_index _item) (message `/Game/BigMaze/Core/Characters/OldCharacter/Interfaces/BPI_InventoryComp.IC (Char) Get Equipped Item` (`self.K2_GetPawn`)))
    (message `/Game/BigMaze/Core/Characters/OldCharacter/Interfaces/BPI_UI.UI Update Equipped Item` _returnvalue _item _index)
    (message `/Game/BigMaze/Core/Characters/OldCharacter/Interfaces/BPI_UI.UI CreatePersistentHUD` (`self.GetHUD`))
    (else
      (`KismetSystemLibrary.PrintString` "Comps Invalid" true true (struct :`G` 0.66 :`B` 1.0 :`A` 1.0) 0.1))))

(event `Begin Hosting Message Beacon`
  ;[1 0 0.9375] Host Invite and Message Beacons
  (if (not (`OnlineBeaconSubsystem.IsHostingBeacon` (subsystem `OnlineBeaconSubsystem`) "/Game/BigMaze/Core/Online/Beacons/BP_MessageBeacon.BP_MessageBeacon_C"))
    (`OnlineBeaconSubsystem.StartHostingBeacon` (subsystem `OnlineBeaconSubsystem`) "/Game/BigMaze/Core/Online/Beacons/BP_MessageBeacon.BP_MessageBeacon_C")))

(event `Key|P`
  (params (Key :type "Key Structure"))
  ;[0.2891 1 0] BeginPlay
  ;;[1 0 0] DEBUG
  (:`Pressed`
    (`self.SR Spawn Player` null)))

(event `CL Reset HUD`
  ;[0.2891 1 0] BeginPlay
  (`|ExecutionSequence`
    (:`then_0`
      (message `/Game/BigMaze/Core/Characters/OldCharacter/Interfaces/BPI_UI.UI DestroyHUD` (`self.GetHUD`)))))

(event `/Game/BigMaze/Core/Characters/OldCharacter/Interfaces/BPI_UI.UI Update Health and Shields`
  (params (Health :type "Float (double-precision)") (Shields :type "Float (double-precision)"))
  ;[1 0.1406 0] Health and Shields
  (`self.CL Set Health and Shields` Health Shields))

(event `CL Set Health and Shields`
  (params (NewHealth :type "Float (double-precision)") (NewShield :type "Float (double-precision)"))
  ;[1 0.1406 0] Health and Shields
  (message `/Game/BigMaze/Core/Characters/OldCharacter/Interfaces/BPI_UI.UI Update Health and Shields` (`self.GetHUD`) NewHealth NewShield))

(event `Try Set References`
  ;[0 1 0.1328] Depricated Set Game State Ref
)

(event `EnhancedInput|/Game/BigMaze/Core/Engine/Inputs/Keys/IA_Inventory`
  (params (ActionValue :type Boolean) (ElapsedSeconds :type "Float (double-precision)") (TriggeredSeconds :type "Float (double-precision)") (InputAction :type "InputAction Object Reference" :default "/Game/BigMaze/Core/Engine/Inputs/Keys/IA_Inventory.IA_Inventory"))
  ;[0.7344 0 1] Create Inventory Widget
  (:`Started`
    (if (`self.IsLocalPlayerController`)
      (message `/Game/BigMaze/Core/Characters/OldCharacter/Interfaces/BPI_UI.UI Toggle Inventory` (`self.GetHUD`)))))

(event `/Game/BigMaze/Core/Characters/OldCharacter/Interfaces/BPI_UI.UI Update Leaderboard`
  ;[0.03125 1 0] Leaderboard Updates
  (`self.CL Update Leaderboard`))

(event `EnhancedInput|/Game/BigMaze/Core/Engine/Inputs/Keys/IA_Leaderboard`
  (params (ActionValue :type Boolean) (ElapsedSeconds :type "Float (double-precision)") (TriggeredSeconds :type "Float (double-precision)") (InputAction :type "InputAction Object Reference" :default "/Game/BigMaze/Core/Engine/Inputs/Keys/IA_Leaderboard.IA_Leaderboard"))
  ;[0.3828 0 1] Create Leaderboard Widget
  (:`Started`
    (if (`self.IsLocalPlayerController`)
      (message `/Game/BigMaze/Core/Characters/OldCharacter/Interfaces/BPI_UI.UI Toggle Leaderboard` (`self.GetHUD`)))))

(event `CL Update Leaderboard`
  ;[0.03125 1 0] Leaderboard Updates
  (message `/Game/BigMaze/Core/Characters/OldCharacter/Interfaces/BPI_UI.UI Update Leaderboard` (`self.GetHUD`)))

(event `/Game/BigMaze/Core/Characters/OldCharacter/Interfaces/BPI_Interact.I Enter Interact Range`
  (params (Actor :type "Actor Object Reference"))
  (`self.Interact Widget`
    (:`then`)
    (:`else`
      (bind _returnvalue (`|CreateWidget` "/Game/BigMaze/Core/UI/HUD/OnScreen/WBP_InteractIcon.WBP_InteractIcon_C"))
      (bind _output_get (set `self.Interact Widget` _returnvalue))
      (message `/Game/BigMaze/Core/Characters/OldCharacter/Interfaces/BPI_UI.Add Interact Widget` (`self.GetHUD`) _output_get))))

(event `CL Create KillFeed Widget`
  (params (`Killer Text` :type Text) (`Killed text` :type Text) (`Weapon Ico` :type "Texture2D Object Reference"))
  ;[0.4766 1 0] Handle Killfeed Widgets
  (message `/Game/BigMaze/Core/Characters/OldCharacter/Interfaces/BPI_UI.UI Create Killfeed Widget` (`self.GetHUD`) `Killer Text` `Killed text` `Weapon Ico`))

(event `/Game/BigMaze/Core/Characters/OldCharacter/Interfaces/BPI_UI.UI Create Killfeed Widget`
  (params (`Killer Text` :type Text) (`Killed Text` :type Text) (`Killer Ico` :type "Texture2D Object Reference"))
  ;[0.4766 1 0] Handle Killfeed Widgets
  (`self.CL Create KillFeed Widget` `Killer Text` `Killed Text` `Killer Ico`))

(event `/Game/BigMaze/Core/Characters/OldCharacter/Interfaces/BPI_Interact.I Exit Interact Range`
  (params (Actor :type "Actor Object Reference"))
  (bind _interact_widget (`self.Interact Widget`)
    (:`then`
      (message `/Game/BigMaze/Core/Characters/OldCharacter/Interfaces/BPI_UI.Remove Interact Widget` (`self.GetHUD`) _interact_widget))
    (:`else`)))

(event `/Game/BigMaze/Core/Characters/OldCharacter/Interfaces/BPI_UI.UI Update Hotbar`
  (message `/Game/BigMaze/Core/Characters/OldCharacter/Interfaces/BPI_UI.UI Update Hotbar` (`self.GetHUD`)))

(event `/Game/BigMaze/Core/Characters/OldCharacter/Interfaces/BPI_UI.UI Update Equipped Item`
  (params (`New Item` :type "/Game/BigMaze/Core/ItemAssets/Common/Structs/S_ItemStruct Structure") (`New Index` :type Integer))
  (message `/Game/BigMaze/Core/Characters/OldCharacter/Interfaces/BPI_UI.UI Update Equipped Item` (`self.GetHUD`) `New Item` `New Index`))

(fn `IC (Char) Get Equipped Item`
  (returns (Index :type Integer) (Item :type "/Game/BigMaze/Core/ItemAssets/Common/Structs/S_ItemStruct Structure"))
  (return 0))

(fn `IC Drop Item`
  (params (Item :type "/Game/BigMaze/Core/ItemAssets/Common/Structs/S_ItemStruct Structure") (Index :type Integer))
  (returns (Success :type Boolean))
  (return false))

(fn `IC External Trade at Index`
  (params (`External Component` :type "/Game/BigMaze/Core/Characters/OldCharacter/Components/BP_InventoryComponent Object Reference") (`New Item` :type "/Game/BigMaze/Core/ItemAssets/Common/Structs/S_ItemStruct Structure") (`New Item Current Index` :type Integer) (`Old Item` :type "/Game/BigMaze/Core/ItemAssets/Common/Structs/S_ItemStruct Structure") (`Old Item Current Index` :type Integer) (`New External` :type Boolean) (`Old External` :type Boolean))
  (returns (Success :type Boolean))
  (return false))

(fn `IC Get Inventory Save Index`
  (returns (Index :type Integer))
  (return (`self.Profile Index`)))

(fn `IC Get Number of Inventory Components`
  (returns (`Has Component` :type Boolean) (`Out Number` :type Integer) (Components :type "Array of /Game/BigMaze/Core/Characters/OldCharacter/Components/BP_InventoryComponent Object Reference"))
  (bind (_has_component _out_number _components) (message `/Game/BigMaze/Core/Characters/OldCharacter/Interfaces/BPI_InventoryComp.IC Get Number of Inventory Components` (`self.K2_GetPawn`)))
  (return _has_component _out_number _components))

(fn `IC Insert Item`
  (params (`New Item` :type "/Game/BigMaze/Core/ItemAssets/Common/Structs/S_ItemStruct Structure") (`Destination Index` :type Integer))
  (returns (`Success?` :type Boolean))
  (return false))

(fn `IC Remove Item`
  (params (Index :type Integer))
  (returns (Success :type Boolean) (`Removed Item` :type "/Game/BigMaze/Core/ItemAssets/Common/Structs/S_ItemStruct Structure"))
  (return false))

(fn `IC Retrieve Component Reference`
  (params (Index :type Integer))
  (returns (Success :type Boolean) (Component :type "/Game/BigMaze/Core/Characters/OldCharacter/Components/BP_InventoryComponent Object Reference"))
  (bind _returnvalue (`self.K2_GetPawn`))
  (if (`KismetSystemLibrary.DoesImplementInterface` _returnvalue "/Game/BigMaze/Core/Characters/OldCharacter/Interfaces/BPI_InventoryComp.BPI_InventoryComp_C")
    (bind (_success _component) (message `/Game/BigMaze/Core/Characters/OldCharacter/Interfaces/BPI_InventoryComp.IC Retrieve Component Reference` _returnvalue Index))
    (return _success _component)
    (else
      (return false null))))

(fn `IC Split Stack`
  (params (Index :type Integer) (`Desired Out Amount` :type Integer))
  (returns (Success :type Boolean) (`Out Initial Item` :type "/Game/BigMaze/Core/ItemAssets/Common/Structs/S_ItemStruct Structure") (`Out Split Item` :type "/Game/BigMaze/Core/ItemAssets/Common/Structs/S_ItemStruct Structure"))
  (return false))

(fn `IC Stack Item`
  (params (`New Item` :type "/Game/BigMaze/Core/ItemAssets/Common/Structs/S_ItemStruct Structure") (`Old Item` :type "/Game/BigMaze/Core/ItemAssets/Common/Structs/S_ItemStruct Structure") (`Item Destination In` :type Integer))
  (returns (Success :type Boolean) (`Stacked item` :type "/Game/BigMaze/Core/ItemAssets/Common/Structs/S_ItemStruct Structure") (`Overflow Item` :type "/Game/BigMaze/Core/ItemAssets/Common/Structs/S_ItemStruct Structure") (`Rejected Item` :type "/Game/BigMaze/Core/ItemAssets/Common/Structs/S_ItemStruct Structure"))
  (return false))

(fn `IC Trade at Index`
  (params (`New Item` :type "/Game/BigMaze/Core/ItemAssets/Common/Structs/S_ItemStruct Structure") (`New Item Current Index` :type Integer) (`Old Item` :type "/Game/BigMaze/Core/ItemAssets/Common/Structs/S_ItemStruct Structure") (`Old Item Current Index` :type Integer))
  (returns (Success :type Boolean))
  (return false))

(fn `P Add Weapon to Inventory`
  (params (`Item Obj` :type "Object Object Reference"))
  (returns (Success :type Boolean))
  (return false))

(fn `P Get Equipped Weapon`
  (returns (`Weapon Index` :type Integer) (WeaponObjs :type "Map of Integer to Object Object Reference"))
  (return 0))

(fn `P Get Has Authority or is Server Owner`
  (returns (`Has Authority` :type Boolean) (`Is Server Owner` :type Boolean))
  (return false false))

(fn `P Get Player Info`
  (returns (Info :type "/Game/BigMaze/Core/GameModes/Extraction/Structs/S_PlayerScore Structure"))
  (return))

(fn `P Get Player Name`
  (returns (`Player Name` :type Name))
  (return "None"))

(fn `P Inventory Comps Active?`
  (returns (True :type Boolean))
  (return false))

(fn `P Retrieve Playerstate`
  (returns (PS :type "/Game/BigMaze/Core/Characters/OldCharacter/BP_PlayerState Object Reference"))
  (bind _asbp_player_state (cast `/Game/BigMaze/Core/Characters/OldCharacter/BP_PlayerState` (`self.PlayerState`)))
  (return _asbp_player_state))

(fn `P Spectator Add`
  (returns (`Return HUD` :type "/Game/BigMaze/Core/UI/HUD/OnScreen/WBP_HUDMain Object Reference"))
  (bind _override_hud (message `/Game/BigMaze/Core/Characters/OldCharacter/Interfaces/BPI_UI.UI Add Spectator (Spectator)` (`self.GetHUD`)))
  (return _override_hud))

(fn `UI Add Spectator (Spectator)`
  (returns (`Override HUD` :type "/Game/BigMaze/Core/UI/HUD/OnScreen/WBP_HUDMain Object Reference"))
  (return null))

(fn `UI Get HUD Reference`
  (returns (HUD :type "/Game/BigMaze/Core/Characters/OldCharacter/BP_HUD Object Reference") (`Active?` :type Boolean))
  (bind _asbp_hud (cast `/Game/BigMaze/Core/Characters/OldCharacter/BP_HUD` (`self.GetHUD`))
    (:`then`
      (return _asbp_hud true))
    (:`CastFailed`
      (return null false))))

(fn `UserConstructionScript`)