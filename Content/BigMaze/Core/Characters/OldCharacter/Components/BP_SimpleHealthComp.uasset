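; Simple health component from the old character folder that handles clamped health changes, optional regeneration and depletion.
; SRUpdateHealth applies additive changes and fires increase or decrease dispatchers, with damage restarting a retriggerable delay before a looping regen timer.
; The Health RepNotify feeds a BP_StatVM view model created at BeginPlay and fires HealthDepleted at zero, optionally carrying overflow damage subject to a full-health denial rule.
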(event `self.ReceiveBeginPlay`
  (bind _returnvalue (`|GenericCreateObject` "/Game/BigMaze/Core/UI/Common/BP_StatVM.BP_StatVM_C" (`self.Health`) (`self.MaxHealth`)))
  (set `self.Health VM` _returnvalue))

(event `SR Update Health`
  (params (Additive :type "Float (double-precision)"))
  (bind _health (`self.Health`))
  (set `self.Last Health Change` Additive)
  (set `self.Health On Last Update` (`self.Health`))
  (bind _output_get (set `self.Health` (`KismetMathLibrary.FClamp` (+ Additive (`self.Health`)) 0.0 (`self.MaxHealth`))))
  (`KismetSystemLibrary.PrintString` (`KismetStringLibrary.Conv_DoubleToString` _output_get))
  (if (>= _output_get (`self.Health On Last Update`))
    (`self.Health Increased` _health)
    (else
      (`self.Health Decreased` _health)
      (if (`self.Does Regenerate?`)
        (`KismetSystemLibrary.K2_ClearAndInvalidateTimerHandle` (`self.RegenTimer`))
        (`KismetSystemLibrary.RetriggerableDelay` (`self.Recharge Delay`))
        (bind _returnvalue (`KismetSystemLibrary.K2_SetTimerDelegate` (`|CreateDelegate` :!event `Regenerate`) (`self.Recharge Interval`) true))
        (set `self.RegenTimer` _returnvalue)))))

(event `Regenerate`
  (`self.SR Update Health` (`self.Regeneration Additive`))
  (if (== (`self.Health`) (`self.MaxHealth`))
    (`KismetSystemLibrary.K2_ClearAndInvalidateTimerHandle` (`self.RegenTimer`))))

(fn `OnRep_Health`
  (bind _health_vm (`self.Health VM`))
  (`/Game/BigMaze/Core/UI/Common/BP_StatVM.SetCurrentStat` _health_vm (`self.Health`))
  (`/Game/BigMaze/Core/UI/Common/BP_StatVM.SetMaxStat` _health_vm (`self.MaxHealth`))
  (if (`/Game/UlimateBlueprintPack/System/Blueprints/UBPP_FunctionLibrary.Smaller Than or Zero (Float)` (`self.Health`))
    (`self.Health Depleted` (`KismetMathLibrary.SelectFloat` 0.0 (`KismetMathLibrary.SelectFloat` (+ (`self.Health On Last Update`) (`self.Last Health Change`)) 0.0 (`self.Pass Overflow Damage When Depleted?`)) (or (not (`self.Only Deny Overflow on Full Health`)) (== (`self.Health On Last Update`) (`self.MaxHealth`)))))))