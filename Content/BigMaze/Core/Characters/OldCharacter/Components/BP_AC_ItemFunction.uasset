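; Actor component that handles the held item's use, release, reload and replication in BigMaze.
; Primary, secondary and tertiary uses match activation class, optionally start camera zoom, then check cooldown before class switches that are still empty; only primary release reverses zoom.
; Reload draws from the owner's "ammo" inventory by ammo ID, and item changes multicast from the server.
; A separate multi line trace picks its channel by penetration level.
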(event `LineTraceItem`
  (bind _actor_ref (`self.Actor Ref`))
  (bind (_origin _forward_vector) (message `/Game/BigMaze/Core/LegacyItemSystem/Common/BPI_ItemUse.Get Item Use Origin and Forward Vector` _actor_ref))
  (`KismetSystemLibrary.LineTraceMulti` _origin (+ _origin (* _forward_vector (`/Game/BigMaze/ItemSystem/Blueprints/BFL_Items.Get Range` (`self.Current item`)))) (select `int` (`/Game/BigMaze/ItemSystem/Blueprints/BFL_Items.Get Pen Level` (`self.Current item`)) :`0` "TraceTypeQuery3" :`1` "TraceTypeQuery4" :`2` "TraceTypeQuery5" :!type "ETraceTypeQuery Enum") false (`|MakeArray` _actor_ref) "ForDuration"))

(event `MC Set Current Item`
  (params (`New Item` :type "/Game/BigMaze/Core/LegacyItemSystem/Common/Structs/S_ItemStruct Structure") (Component :type "/Game/BigMaze/Core/Characters/OldCharacter/Components/BP_AC_ItemFunction Object Reference"))
  ;[1 1 1] Replicated Item Update
  (`/Engine/EditorBlueprintResources/ActorComponentMacros.Switch Has Authority`
    (:`Remote`
      (set `/Game/BigMaze/Core/Characters/OldCharacter/Components/BP_AC_ItemFunction.Current item` `New Item` Component :!label _label))))

(event `Reload Current Item`
  (bind _current_item (`self.Current item`))
  (bind (_stackable_ _stack _max_stack _has_ammunition_) (`/Game/BigMaze/ItemSystem/Blueprints/BFL_Items.Get Stack Data` (`self.Current item`)))
  (bind _max_stack_size (`/Game/BigMaze/ItemSystem/Blueprints/BFL_Items.Get Max Stack Size` _current_item))
  (bind _int (`self.String to AmmoID Int` (`.Value` (`/Game/BigMaze/ItemSystem/Blueprints/BFL_Items.Get Specific Attribute` _current_item "ammoid"))))
  ;[1 1 1] Calls Reload Function If the Item is Reloadable
  (bind (_success _component) (message `/Game/BigMaze/Core/Characters/OldCharacter/Interfaces/BPI_InventoryComp.IC Retrieve Component Reference` (`self.GetOwner`) 2))
  (if (and (< _stack _max_stack) _has_ammunition_ (== (`/Game/BigMaze/Core/Characters/OldCharacter/Components/BP_InventoryComponent.Inventory Name` _component) "ammo") _success)
    (bind _output_get (set `self.Ammo Component` _component))
    (bind _output (`|GetArrayItem` (`/Game/BigMaze/Core/Characters/OldCharacter/Components/BP_InventoryComponent.Inventory` _output_get) _int))
    (bind _amount_in_stack (`/Game/BigMaze/ItemSystem/Blueprints/BFL_Items.Get Stack Count` _output))
    (bind _returnvalue (`KismetMathLibrary.SelectInt` _max_stack_size (+ (`/Game/BigMaze/ItemSystem/Blueprints/BFL_Items.Get Stack Count` _current_item) _amount_in_stack) (< _max_stack_size _amount_in_stack)))
    (bind _out_item (`/Game/BigMaze/ItemSystem/Blueprints/BFL_Items.Update Item Stack Count` _output (- _amount_in_stack _returnvalue)))
    (`/Game/BigMaze/Core/Characters/OldCharacter/Components/BP_InventoryComponent.SR Insert Item` (`self.Ammo Component`) _out_item _int)
    (bind _out_item_2 (`/Game/BigMaze/ItemSystem/Blueprints/BFL_Items.Update Item Stack Count` (`self.Current item`) _returnvalue))
    (`self.Exec Item Update` _out_item_2 "NewEnumerator7")))

(event `Release Current Item`
  (params (Actor :type "Actor Object Reference") (Component :type "/Game/BigMaze/Core/Characters/OldCharacter/Components/BP_AC_ItemFunction Object Reference"))
  (bind (_use_ _activation_class) (`/Game/BigMaze/ItemSystem/Blueprints/BFL_Items.Get Primary Use` (`self.Current item`)))
  (if (`self.Is Item Primary in Use`)
    (switch `/Game/BigMaze/Core/LegacyItemSystem/Common/Enums/E_ActivationClass` _activation_class
      (:`NewEnumerator1`
        _)
      (:`NewEnumerator2`
        _))
    (switch `/Game/BigMaze/Core/LegacyItemSystem/Common/Enums/E_UseChart` _use_
      (:`NewEnumerator2`
        (`self.ReverseCameraZoom` (`/Game/BigMaze/ItemSystem/Blueprints/BFL_Items.Get Zoom` (`self.Current item`)))))))

(event `Set Current Item`
  (params (`New Item` :type "/Game/BigMaze/Core/LegacyItemSystem/Common/Structs/S_ItemStruct Structure") (Component :type "/Game/BigMaze/Core/Characters/OldCharacter/Components/BP_AC_ItemFunction Object Reference"))
  ;[1 1 1] Replicated Item Update
  (`/Engine/EditorBlueprintResources/ActorComponentMacros.Switch Has Authority`
    (:`Authority`
      (`|ExecutionSequence`
        (:`then_0`
          (`self.MC Set Current Item` `New Item` Component))
        (:`then_1`
          (goto _label))))))

(event `Release Secondary Item`
  (params (Actor :type "Actor Object Reference") (Component :type "/Game/BigMaze/Core/Characters/OldCharacter/Components/BP_AC_ItemFunction Object Reference")))

(event `Release Tertiary Item`
  (params (Actor :type "Actor Object Reference") (Component :type "/Game/BigMaze/Core/Characters/OldCharacter/Components/BP_AC_ItemFunction Object Reference")))

(event `Use Current Item`
  (params (`Actor Ref` :type "Actor Object Reference") (`Activation Class` :type "/Game/BigMaze/Core/LegacyItemSystem/Common/Enums/E_ActivationClass Enum" :default "NewEnumerator0"))
  (bind _current_item (`self.Current item`))
  (bind (_use_ _activation_class) (`/Game/BigMaze/ItemSystem/Blueprints/BFL_Items.Get Primary Use` (`self.Current item`)))
  (bind _output_get (set `self.Actor Ref` `Actor Ref`))
  (bind (_origin _forward_vector) (message `/Game/BigMaze/Core/LegacyItemSystem/Common/BPI_ItemUse.Get Item Use Origin and Forward Vector` _output_get))
  (if (`|EnumEquality` `Activation Class` _activation_class)
    (switch `/Game/BigMaze/Core/LegacyItemSystem/Common/Enums/E_UseChart` _use_
      (:`NewEnumerator1`
        _)
      (:`NewEnumerator2`
        (`self.StartCameraZoom` (`/Game/BigMaze/ItemSystem/Blueprints/BFL_Items.Get Zoom` _current_item) (`/Game/BigMaze/ItemSystem/Blueprints/BFL_Items.Get Handling` _current_item))))
    (set `self.Last Trace Origin` _origin)
    (set `self.Last Trace Foward Vector` _forward_vector)
    (if (not (`KismetSystemLibrary.K2_IsValidTimerHandle` (`self.Cooldown Timer`)))
      (switch `/Game/BigMaze/Core/LegacyItemSystem/Common/Enums/E_ItemClass` (`/Game/BigMaze/ItemSystem/Blueprints/BFL_Items.Get Class` (`self.Current item`))))))

(event `Secondary Use Current Item`
  (params (`Actor Ref` :type "Actor Object Reference") (`Activation Class` :type "/Game/BigMaze/Core/LegacyItemSystem/Common/Enums/E_ActivationClass Enum" :default "NewEnumerator0"))
  (bind _current_item (`self.Current item`))
  (bind (_use_ _activation_class) (`/Game/BigMaze/ItemSystem/Blueprints/BFL_Items.Get Secondary Use` (`self.Current item`)))
  (set `self.Actor Ref` `Actor Ref`)
  (if (`|EnumEquality` `Activation Class` _activation_class)
    (switch `/Game/BigMaze/Core/LegacyItemSystem/Common/Enums/E_UseChart` _use_
      (:`NewEnumerator1`
        _)
      (:`NewEnumerator2`
        (`self.StartCameraZoom` (`/Game/BigMaze/ItemSystem/Blueprints/BFL_Items.Get Zoom` _current_item) (`/Game/BigMaze/ItemSystem/Blueprints/BFL_Items.Get Handling` _current_item))))
    (if (not (`KismetSystemLibrary.K2_IsValidTimerHandle` (`self.Cooldown Timer`)))
      (switch `/Game/BigMaze/Core/LegacyItemSystem/Common/Enums/E_ItemClass` (`/Game/BigMaze/ItemSystem/Blueprints/BFL_Items.Get Class` (`self.Current item`))))))

(event `Tertiary Use Current Item`
  (params (`Actor Ref` :type "Actor Object Reference") (`Activation Class` :type "/Game/BigMaze/Core/LegacyItemSystem/Common/Enums/E_ActivationClass Enum" :default "NewEnumerator0"))
  (bind _current_item (`self.Current item`))
  (bind (_use_ _activation_class) (`/Game/BigMaze/ItemSystem/Blueprints/BFL_Items.Get Tertiary Use` (`self.Current item`)))
  (set `self.Actor Ref` `Actor Ref`)
  (if (`|EnumEquality` `Activation Class` _activation_class)
    (switch `/Game/BigMaze/Core/LegacyItemSystem/Common/Enums/E_UseChart` _use_
      (:`NewEnumerator1`
        _)
      (:`NewEnumerator2`
        (`self.StartCameraZoom` (`/Game/BigMaze/ItemSystem/Blueprints/BFL_Items.Get Zoom` _current_item) (`/Game/BigMaze/ItemSystem/Blueprints/BFL_Items.Get Handling` _current_item))))
    (if (not (`KismetSystemLibrary.K2_IsValidTimerHandle` (`self.Cooldown Timer`)))
      (switch `/Game/BigMaze/Core/LegacyItemSystem/Common/Enums/E_ItemClass` (`/Game/BigMaze/ItemSystem/Blueprints/BFL_Items.Get Class` (`self.Current item`))))))