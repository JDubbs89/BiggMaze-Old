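; Networked first-person player character for an extraction shooter, handling movement, ADS, combat and death through server and multicast events.
; Hotbar selection sets the replicated equipped item, updating HUD and both weapon meshes; Inventory and Ammo components complete storage.
; Hitscan traces read spread, range and damage from item attributes, with component tags setting hit-zone multipliers.
; Damage depletes shields before health and records attackers; OnRep_Health reports death and credit to the game mode.
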(event OnComponentActivated(Inventory)
  (params (Component :type Actor%20Component%20Object%20Reference) (bReset :type Boolean)))

(event OnComponentActivated(Hotbar)
  (params (Component :type Actor%20Component%20Object%20Reference) (bReset :type Boolean)))

(event Custom|SR_LineTrace
  ;[1 1 1] Line Trace
  (CallFunction|MCLineTrace))

(event Custom|MC_Jump
  (params (Start? :type Boolean) (AnimInstance :type Anim%20Instance%20Object%20Reference) (Jump%20Count :type Integer))
  ;[1 1 1] Jumping
  (if Start?
    _))

(event Custom|ADSEvent
  (params (Ads :type Boolean))
  (bind _returnvalue (Utilities|Time|GetWorldDeltaSeconds))
  (bind _sk_gun (Variables|Default|GetSK_Gun))
  (bind _sk_gun_2 (Variables|Default|GetSK_Gun))
  (bind _meshdefaultlocation (Variables|Weapons|GetMeshDefaultLocation))
  (bind _relativelocation (Variables|/Script/Engine.SceneComponent|GetRelativeLocation _sk_gun_2))
  ;[1 1 1] ADS
  (if Ads
    (CallFunction|SRADS true)
    (bind (_direction _timeline) (Timeline|AimDownTL Play)
      (:Update
        (Camera|SetFieldOfView (Variables|Default|GetCamera) _timeline)
        (switch Utilities|FlowControl|Switch|SwitchonETimelineDirection _direction
          (:Forward
            (Transformation|SetRelativeLocationAndRotation _sk_gun (Math|Interpolation|VInterptoConstant _relativelocation (+ _meshdefaultlocation "10.000000,-30.000000,5.000000") _returnvalue 5e+02) "0,-90.000000, 0" false true))
          (:Backward
            (Transformation|SetRelativeLocationAndRotation _sk_gun (Math|Interpolation|VInterptoConstant _relativelocation _meshdefaultlocation _returnvalue 5e+02) (Variables|Weapons|GetMeshDefaultRotation) false true)))))
    (else
      (CallFunction|SRADS false)
      (Timeline|AimDownTL Reverse))))

(event Custom|SR%20Update%20Item
  (params (Equipped%20Item :type Item%20Struct%20Structure))
  ;[1 1 1] Hotbar and Equipped Item
  (Variables|Weapons|SetEquipped%20Item Equipped%20Item))

(event Custom|SR_Rotate
  (params (NewParam :type Float%20%28double-precision%29))
  ;[1 1 1] Camera Rotation Replication
  (CallFunction|MCRotate NewParam))

(event Custom|MC_Rotate
  (params (NewParam :type Float%20%28double-precision%29))
  (bind _camera (Variables|Default|GetCamera))
  (bind _returnvalue (Transformation|GetWorldRotation _camera))
  ;[1 1 1] Camera Rotation Replication
  (Transformation|SetWorldRotation _camera (Math|Rotator|MakeRotator (.roll _returnvalue) NewParam (.yaw _returnvalue)) false false))

(event Custom|SR%20Update%20Index
  (params (Index :type Integer))
  ;[1 1 1] Hotbar and Equipped Item
  (Variables|Default|SetEquipped%20Index Index)
  (Variables|Weapons|SetEquipped%20Item (.Item (Utilities|FindEquippedWeapon))))

(event Custom|CL%20Update%20Equipped%20Weapon
  (bind _item (Utilities|FindEquippedWeapon))
  (bind _item_2 (Utilities|FindEquippedWeapon))
  (bind _self self)
  (bind _self_2 self)
  (bind _item_variable_table (Variables|Weapons|GetItem%20Variable%20Table))
  (bind (_name _description _icon _amountinstack _maxstacksize _itemclass) (Utilities|Struct|BreakItemStruct _item_2))
  ;[1 1 1] Updating Weapon Mesh
  (bind (_active_ _hud_ref) (Class|BPIHUD|GetHUDStatus(Message) (HUD|GetHUD (Game|GetPlayerController 0))))
  (if _active_
    (Class|BPIHUD|UpdateEquippedItem(Message) _hud_ref _item_2 (Variables|Default|GetEquipped%20Index))
    (Utilities|AsyncLoadAsset _item_variable_table
      (:Completed
        (bind _returnvalue (Utilities|GetDataTableRow (Utilities|ResolveSoftReference _item_variable_table) (Utilities|String|StringToName _name))
          (:then
            (Variables|Default|SetEquippedItemRow _returnvalue)
            (if (Utilities|Enum|Equal(Enum) _itemclass "NewEnumerator0")
              (CallFunction|SetBarrelSocket)
              (else
                (Networking|SwitchHasAuthority
                  (:Authority
                    (CallFunction|MCUpdateEquipedWeapon _self _self _item (Variables|Default|GetEquippedItemRow)))
                  (:Remote
                    (CallFunction|SRUpdateEquippedWeapon _self_2 _self_2 _item (Variables|Default|GetEquippedItemRow))))))))))
    (else
      (Utilities|Time|SetTimerbyEvent (EventDispatchers|CreateEvent :!event Custom|Update%20Component) 0.0))))

(event Custom|SR%20Update%20Equipped%20Weapon
  (params (Character :type BP%20Character%20Object%20Reference) (ItemStruct :type Item%20Struct%20Structure%20%28by%20ref%29) (S_WeaponVariableInfo :type S%20Weapon%20Variable%20Info%20Structure%20%28by%20ref%29))
  ;[1 1 1] Updating Weapon Mesh
  (CallFunction|MCUpdateEquipedWeapon Character Character ItemStruct S_WeaponVariableInfo))

(event Custom|MC%20Update%20Equiped%20Weapon
  (params (Character :type BP%20Character%20Object%20Reference) (ItemStruct :type Item%20Struct%20Structure%20%28by%20ref%29) (S_WeaponVariableInfo :type S%20Weapon%20Variable%20Info%20Structure%20%28by%20ref%29))
  (bind _sk_gun (Variables|BP_Character_C|GetSK_Gun Character))
  ;[1 1 1] Updating Weapon Mesh
  (Components|SkeletalMesh|SetSkeletalMeshAsset _sk_gun (.Skeletalmesh (Utilities|Struct|BreakItemStruct ItemStruct)))
  (Transformation|SetRelativeTransform _sk_gun (.RelativeTransform (Utilities|Struct|BreakS_WeaponVariableInfo S_WeaponVariableInfo)) false true))

(event Custom|SR
  (CallFunction|MC))

(event Custom|SR_HitBox
  (params (Hit :type Actor%20Component%20Object%20Reference))
  ;[1 1 1] Take Damage
  (Utilities|IsValid Hit
    (:Is%20Valid
      (if (Components|ComponentHasTag Hit "Head")
        (Variables|Health|SetDamageMultiplier 1.0)
        (Development|PrintString "Head shot" true true "(R=1.000000,G=0.000000,B=0.000000,A=1.000000)" 0.5)
        (elif (Components|ComponentHasTag Hit "Body")
          (Variables|Health|SetDamageMultiplier 0.4)
          (Development|PrintString "Body shot" true true "(R=1.000000,G=1.000000,B=0.000000,A=1.000000)" 0.5)
          (elif (Components|ComponentHasTag Hit "Legs")
            (Variables|Health|SetDamageMultiplier 0.2)
            (Development|PrintString "Leg shot" true true "(R=0.000000,G=1.000000,B=0.000000,A=1.000000)" 0.5)
            (else
              (Variables|Health|SetDamageMultiplier 1.0))))))))

(event Custom|BeginPlay
  ;[1 1 1] Begin Play
  (Variables|Health|SetHealth (Variables|Health|GetMax%20Health))
  (Variables|Health|SetShields (Variables|Health|GetMax%20Shields)))

(event Custom|MC
  (Animation|Montage|PlayMontage (Variables|Character|GetMesh) "/Game/BigMaze/CharacterModels/BuffPasta/FirstPerson/Anims/FPMan_CantSeeMe.FPMan_CantSeeMe"
    (:then
      (Animation|Montage|PlayMontage (Variables|Default|GetFPMesh) "/Game/BigMaze/CharacterModels/BuffPasta/FirstPerson/Anims/FPMan_CantSeeMe.FPMan_CantSeeMe"))))

(event Custom|SR%20Reload%20Weapon
  ;[1 1 1] Primary and Secondary Actions
  (Variables|Weapons|SetEquipped%20Item (.Item (Utilities|FindEquippedWeapon))))

(event Custom|Set%20Barrel%20Socket
  ;[1 1 1] Updating Weapon Mesh
)

(event Custom|aff
  (Variables|Weapons|SetEquipped%20Item (.Item (Utilities|FindEquippedWeapon))))

(event Custom|MC_LineTrace
  (bind _equipped_item (Variables|Weapons|GetEquipped%20Item))
  (bind _camera (Variables|Default|GetCamera))
  (bind _uniqueattributes (Utilities|Struct|BreakItemStruct _equipped_item))
  (bind _returnvalue (Transformation|GetWorldLocation _camera))
  (bind _value (Utilities|Map|Find _uniqueattributes "spread"))
  (bind _returnvalue_2 (Math|Conversions|ToFloat(Integer) _value))
  (bind _returnvalue_3 (* _returnvalue_2 -1.0))
  ;[1 1 1] Line Trace
  (Utilities|FlowControl|Sequence
    (:then_0
      (bind _outhit (Collision|LineTraceByChannel _returnvalue (+ (+ (Math|Vector|MakeVector (Math|Random|RandomFloatinRange _returnvalue_3 _returnvalue_2) (Math|Random|RandomFloatinRange _returnvalue_3 _returnvalue_2) (Math|Random|RandomFloatinRange _returnvalue_3 _returnvalue_2)) (+ _returnvalue (* (Math|Vector|GetForwardVector _camera) (Math|Conversions|ToFloat(Integer) (.Value (Utilities|Map|Find _uniqueattributes "range")))))) "") "TraceTypeQuery1" false 0 "None"))
      (Audio|PlaySoundatLocation "/Game/MilitaryWeapDark/Sound/Rifle/Wavs/RifleB_Fire01.RifleB_Fire01" _returnvalue "0, 0, 0" 0.8 1.0 0.0 "/Game/MilitaryWeapDark/Sound/Attenuation/WeaponShot_att.WeaponShot_att" 0 0 0) ; Play firing sound
      (if (.bBlockingHit (Collision|BreakHitResult _outhit))
        (Utilities|FlowControl|Delay (/ (Class|KismetMathLibrary|GetPointDistancetoSegment (.ImpactPoint (Collision|BreakHitResult _outhit)) (.TraceStart (Collision|BreakHitResult _outhit)) (.TraceStart (Collision|BreakHitResult _outhit))) 8e+04))
        (Utilities|FlowControl|Sequence
          (:then_1
            (CallFunction|SRHitBox (.HitComponent (Collision|BreakHitResult _outhit))))
          (:then_2
            (Game|Damage|ApplyDamage (.HitActor (Collision|BreakHitResult _outhit)) (Math|Conversions|ToFloat(Integer) (.Value (Utilities|Map|Find (.UniqueAttributes (Utilities|Struct|BreakItemStruct (Variables|Weapons|GetEquipped%20Item))) "damage"))) (Game|GetPlayerController (Variables|GetPlayerState)) 0 "/Script/Engine.DamageType"))
          (:then_3
            (Effects|SpawnEmitteratLocation "/Game/MilitaryWeapDark/FX/P_Impact_Metal_Small_01.P_Impact_Metal_Small_01" (.ImpactPoint (Collision|BreakHitResult _outhit)) "0, 0, 0" "0.700000,0.700000,0.700000")
            (Audio|SpawnSoundatLocation "/Game/BigMaze/Effects/Sound/Abstract_Pop_01.Abstract_Pop_01" (.ImpactPoint (Collision|BreakHitResult _outhit)) "0, 0, 0" 1.0 1.0 0.0 "/Game/MilitaryWeapDark/Sound/Attenuation/ProjectileImpact_att.ProjectileImpact_att" 0)))))))

(event Custom|MC_Land
  (params (AnimBp :type Anim%20Instance%20Object%20Reference))
  ;[1 1 1] Jumping
)

(event Custom|SR_Land
  (params (AnimBp :type Anim%20Instance%20Object%20Reference) (Char :type BP%20Character%20Object%20Reference))
  ;[1 1 1] Jumping
  (CallFunction|MCLand AnimBp)
  (Variables|BP_Character_C|SetJump%20Count Char 0))

(event Custom|SR%20Player%20death
  (params (Actor :type BP%20Character%20Object%20Reference) (Controller :type Player%20Controller%20Object%20Reference) (Kill%20Credit :type BP%20Player%20State%20Object%20Reference) (Assist%20Credit :type Array%20of%20BP%20Player%20State%20Object%20References) (Last%20AI%20Damager :type Actor%20Object%20Reference) (Credit%20AI? :type Boolean))
  ;[1 1 1] Death
  (bind _asbp_controller (Utilities|Casting|CastToBP_Controller Controller))
  (bind _asbp_extraction_game_mode (Utilities|Casting|CastToBP_Extraction_GameMode (Game|GetGameMode)))
  (Default|PlayerDeath _asbp_extraction_game_mode _asbp_controller Actor Kill%20Credit Assist%20Credit Last%20AI%20Damager Credit%20AI?))

(event Custom|SR_Jump
  (params (Start? :type Boolean) (AnimInstance :type Anim%20Instance%20Object%20Reference) (Jump%20Count :type Integer) (Player :type BP%20Character%20Object%20Reference))
  ;[1 1 1] Jumping
  (if Start?
    (bind _result (Math|Integer|IncrementInt Jump%20Count)
      (:%20%20
        (bind _output_get (Variables|BP_Character_C|SetJump%20Count Player _result)))))
  (CallFunction|MCJump Start? AnimInstance _output_get)
  (Variables|BP_Character_C|SetJumping Player Start?))

(event Custom|SR%20ADS
  (params (ADS :type Boolean))
  ;[1 1 1] ADS
  (CallFunction|MCADS ADS))

(event Custom|MC%20ADS
  (params (ADS :type Boolean))
  (bind _statustags (Variables|Default|GetStatusTags))
  ;[1 1 1] ADS
  (if ADS
    (GameplayTags|AddGameplayTag _statustags "(TagName=\"ActorStatusEffects.actions.ads\")" :!class /Script/GameplayTags.BlueprintGameplayTagLibrary)
    (else
      (GameplayTags|RemoveGameplayTag _statustags "(TagName=\"ActorStatusEffects.actions.ads\")" :!class /Script/GameplayTags.BlueprintGameplayTagLibrary))))

(event Custom|MC%20Player%20Death
  (params (Actor :type BP%20Character%20Object%20Reference))
  ;[1 1 1] Death
  (Actor|DestroyActor Actor))

(event Input|EnhancedActionEvents|EnhancedInputActionIA_Move
  (params (ActionValue :type Vector%202D%20Structure) (ElapsedSeconds :type Float%20%28double-precision%29) (TriggeredSeconds :type Float%20%28double-precision%29) (InputAction :type Input%20Action%20Object%20Reference :default "/Game/BigMaze/Core/Engine/Inputs/Keys/IA_Move.IA_Move"))
  (bind _returnvalue (Transformation|GetActorRotation))
  ;[1 1 1] Move Around
  (Pawn|Input|AddMovementInput (Math|Vector|GetForwardVector (Math|Rotator|MakeRotator 0.0 (.pitch _returnvalue) (.yaw _returnvalue))) (.y ActionValue) false)
  (Pawn|Input|AddMovementInput (Math|Vector|GetRightVector (Math|Rotator|MakeRotator (.roll _returnvalue) 0.0 (.yaw _returnvalue))) (.x ActionValue) false))

(event Input|EnhancedActionEvents|EnhancedInputActionIA_Crouch
  (params (ActionValue :type Boolean) (ElapsedSeconds :type Float%20%28double-precision%29) (TriggeredSeconds :type Float%20%28double-precision%29) (InputAction :type Input%20Action%20Object%20Reference :default "/Game/BigMaze/Core/Engine/Inputs/Keys/IA_Crouch.IA_Crouch"))
  ;[1 1 1] Crouch
  (:Started
    (Character|Crouch))
  (:Completed
    (Character|UnCrouch)))

(event Input|EnhancedActionEvents|EnhancedInputActionIA_Hotbar4
  (params (ActionValue :type Boolean) (ElapsedSeconds :type Float%20%28double-precision%29) (TriggeredSeconds :type Float%20%28double-precision%29) (InputAction :type Input%20Action%20Object%20Reference :default "/Game/BigMaze/Core/Engine/Inputs/Keys/IA_Hotbar4.IA_Hotbar4"))
  ;[1 1 1] Hotbar and Equipped Item
  (:Started
    (if (.Item%20Exists (Default|DoesItemExistatIndex? (Variables|Default|GetHotbar) 3))
      (CallFunction|SRUpdateIndex 3))))

(event Input|EnhancedActionEvents|EnhancedInputActionIA_Reload
  (params (ActionValue :type Boolean) (ElapsedSeconds :type Float%20%28double-precision%29) (TriggeredSeconds :type Float%20%28double-precision%29) (InputAction :type Input%20Action%20Object%20Reference :default "/Game/BigMaze/Core/Engine/Inputs/Keys/IA_Reload.IA_Reload"))
  ;[1 1 1] Primary and Secondary Actions
  (:Started
    (CallFunction|SRReloadWeapon)))

(event Input|EnhancedActionEvents|EnhancedInputActionIA_PrimaryAction
  (params (ActionValue :type Boolean) (ElapsedSeconds :type Float%20%28double-precision%29) (TriggeredSeconds :type Float%20%28double-precision%29) (InputAction :type Input%20Action%20Object%20Reference :default "/Game/BigMaze/Core/Engine/Inputs/Keys/IA_PrimaryAction.IA_PrimaryAction"))
  (bind _statustags (Variables|Default|GetStatusTags))
  (bind _statustags_2 (Variables|Default|GetStatusTags))
  ;[1 1 1] Primary and Secondary Actions
  (:Ongoing
    (if (GameplayTags|HasTag _statustags_2 "(TagName=\"ActorStatusEffects.actions.using_item\")" true)
      _
      (else
        (GameplayTags|AddGameplayTag _statustags_2 "(TagName=\"ActorStatusEffects.actions.using_item\")" :!class /Script/GameplayTags.BlueprintGameplayTagLibrary)))
    (CallFunction|SRUpdateItem (.Item (Utilities|FindEquippedWeapon))))
  (:Canceled
    (if (GameplayTags|HasTag _statustags "(TagName=\"ActorStatusEffects.actions.using_item\")" true) :!label _label
      (GameplayTags|RemoveGameplayTag _statustags "(TagName=\"ActorStatusEffects.actions.using_item\")" :!class /Script/GameplayTags.BlueprintGameplayTagLibrary)))
  (:Completed
    (goto _label)))

(event Input|EnhancedActionEvents|EnhancedInputActionIA_SecondaryAction
  (params (ActionValue :type Boolean) (ElapsedSeconds :type Float%20%28double-precision%29) (TriggeredSeconds :type Float%20%28double-precision%29) (InputAction :type Input%20Action%20Object%20Reference :default "/Game/BigMaze/Core/Engine/Inputs/Keys/IA_SecondaryAction.IA_SecondaryAction"))
  ;[1 1 1] Primary and Secondary Actions
  (:Started
    (CallFunction|SRUpdateItem (.Item (Utilities|FindEquippedWeapon)))))

(event Input|EnhancedActionEvents|EnhancedInputActionIA_Jump
  (params (ActionValue :type Boolean) (ElapsedSeconds :type Float%20%28double-precision%29) (TriggeredSeconds :type Float%20%28double-precision%29) (InputAction :type Input%20Action%20Object%20Reference :default "/Game/BigMaze/Core/Engine/Inputs/Keys/IA_Jump.IA_Jump"))
  (bind _self self)
  (bind _mesh (Variables|Character|GetMesh))
  (bind _jump_count (Variables|Movement|GetJump%20Count))
  (bind _returnvalue (Components|SkeletalMesh|GetAnimInstance _mesh))
  ;[1 1 1] Jumping
  (:Started
    (Character|Jump)
    (CallFunction|SRJump true _returnvalue _jump_count _self))
  (:Completed
    (Character|StopJumping)
    (CallFunction|SRJump false _returnvalue _jump_count _self)))

(event Input|EnhancedActionEvents|EnhancedInputActionIA_Look
  (params (ActionValue :type Vector%202D%20Structure) (ElapsedSeconds :type Float%20%28double-precision%29) (TriggeredSeconds :type Float%20%28double-precision%29) (InputAction :type Input%20Action%20Object%20Reference :default "/Game/BigMaze/Core/Engine/Inputs/Keys/IA_Look.IA_Look"))
  (bind _sensitivity (Variables|Movement|GetSensitivity))
  ;[1 1 1] Look Around
  (Pawn|Input|AddControllerYawInput (* (.x ActionValue) _sensitivity))
  (Pawn|Input|AddControllerPitchInput (* (.y ActionValue) _sensitivity))
  (CallFunction|SRRotate (.pitch (Transformation|GetWorldRotation (Variables|Default|GetCamera)))))

(event Input|EnhancedActionEvents|EnhancedInputActionIA_Scroll
  (params (ActionValue :type Float%20%28double-precision%29) (ElapsedSeconds :type Float%20%28double-precision%29) (TriggeredSeconds :type Float%20%28double-precision%29) (InputAction :type Input%20Action%20Object%20Reference :default "/Game/BigMaze/Core/Engine/Inputs/Keys/IA_Scroll.IA_Scroll"))
  (bind _returnvalue (* ActionValue -1.0))
  ;[1 1 1] Hotbar and Equipped Item
  (if (!= _returnvalue 0.0)
    (bind (_next_filled_index _success) (Default|FindNextValidIndex (Variables|Default|GetHotbar) (> _returnvalue 0.0) (Variables|Default|GetEquipped%20Index)))
    (if _success
      (CallFunction|SRUpdateIndex _next_filled_index))))

(event Input|EnhancedActionEvents|EnhancedInputActionIA_Hotbar1
  (params (ActionValue :type Boolean) (ElapsedSeconds :type Float%20%28double-precision%29) (TriggeredSeconds :type Float%20%28double-precision%29) (InputAction :type Input%20Action%20Object%20Reference :default "/Game/BigMaze/Core/Engine/Inputs/Keys/IA_Hotbar1.IA_Hotbar1"))
  ;[1 1 1] Hotbar and Equipped Item
  (:Started
    (if (.Item%20Exists (Default|DoesItemExistatIndex? (Variables|Default|GetHotbar)))
      (CallFunction|SRUpdateIndex))))

(event Input|EnhancedActionEvents|EnhancedInputActionIA_Hotbar2
  (params (ActionValue :type Boolean) (ElapsedSeconds :type Float%20%28double-precision%29) (TriggeredSeconds :type Float%20%28double-precision%29) (InputAction :type Input%20Action%20Object%20Reference :default "/Game/BigMaze/Core/Engine/Inputs/Keys/IA_Hotbar2.IA_Hotbar2"))
  ;[1 1 1] Hotbar and Equipped Item
  (:Started
    (if (.Item%20Exists (Default|DoesItemExistatIndex? (Variables|Default|GetHotbar) 1))
      (CallFunction|SRUpdateIndex 1))))

(event Input|EnhancedActionEvents|EnhancedInputActionIA_Hotbar3
  (params (ActionValue :type Boolean) (ElapsedSeconds :type Float%20%28double-precision%29) (TriggeredSeconds :type Float%20%28double-precision%29) (InputAction :type Input%20Action%20Object%20Reference :default "/Game/BigMaze/Core/Engine/Inputs/Keys/IA_Hotbar3.IA_Hotbar3"))
  ;[1 1 1] Hotbar and Equipped Item
  (:Started
    (if (.Item%20Exists (Default|DoesItemExistatIndex? (Variables|Default|GetHotbar) 2))
      (CallFunction|SRUpdateIndex 2))))

(event EventBeginPlay
  ;[1 1 1] Begin Play
  (Utilities|FlowControl|Sequence
    (:then_0
      (Audio|PlaySound2D "/Game/BigMaze/Effects/Sound/Abstract_Pop_04.Abstract_Pop_04" 1.0 1.0 0.0 0 0))
    (:then_1
      (bind _returnvalue (Utilities|Time|SetTimerbyEvent (EventDispatchers|CreateEvent :!event Custom|BeginPlay) 0.1))
      (Variables|Timers|SetBPTimer _returnvalue))
    (:then_2
      (CallFunction|SRInitInventory)
      (CallFunction|SRInitHotbar)
      (CallFunction|SRInitAmmo))))

(event EventTick
  (params (DeltaSeconds :type Float%20%28single-precision%29)))

(event EventOnLanded
  (params (Hit :type Hit%20Result%20Structure%20%28by%20ref%29))
  ;[1 1 1] Jumping
  (CallFunction|SRLand (Components|SkeletalMesh|GetAnimInstance (Variables|Character|GetMesh)) self))

(event EventDestroyed
  ;[1 1 1] Death
)

(event Game|Damage|EventAnyDamage
  (params (Damage :type Float%20%28single-precision%29) (DamageType :type Damage%20Type%20Object%20Reference) (InstigatedBy :type Controller%20Object%20Reference) (DamageCauser :type Actor%20Object%20Reference))
  (bind _damagemultiplier (Variables|Health|GetDamageMultiplier))
  (bind _returnvalue (* Damage _damagemultiplier))
  ;[1 1 1] Take Damage
  (if (Actor|ActorHasTag DamageCauser "ai")
    (Variables|Health|SetLast%20AI%20Damager DamageCauser)
    (Variables|Health|SetLast%20Damager%20AI? true)
    (else
      (Variables|Health|SetLast%20Damager%20AI? false)
      (bind _ps (Class|BPIPlayer|RetrievePlayerstate(Message) InstigatedBy))
      (bind _output_get (Variables|Health|SetLast%20Damager self _ps))
      (Utilities|Array|Add (Variables|Health|GetDamagers) _output_get)))
  (if (<= (Variables|Health|GetShields) 0.0)
    (Variables|Health|SetHealth (- (Variables|Health|GetHealth) _returnvalue))
    (else
      (Variables|Health|SetShields (- (Variables|Health|GetShields) _returnvalue)))))

(event Input|KeyboardEvents|DebugKeyG
  (params (Key :type Key%20Structure :default "None") (ActionValue :type Input%20Action%20Value%20Structure))
  ;[1 1 1] Line Trace
  (:Pressed
    (bind _asbp_player_state (Utilities|Casting|CastToBP_PlayerState (Variables|GetPlayerState)))))

(event Input|KeyboardEvents|Add
  (params (Key :type Key%20Structure :default "None"))
  (bind _self self)
  ;[1 1 1] Health Debug
  (:Pressed
    (Game|Damage|ApplyDamage _self 1e+01 0 _self "/Script/Engine.DamageType")))

(event Input|KeyboardEvents|Subtract
  (params (Key :type Key%20Structure :default "None"))
  (bind _self self)
  ;[1 1 1] Health Debug
  (:Pressed
    (Game|Damage|ApplyDamage _self -2e+01 0 _self "/Script/Engine.DamageType")))

(event Input|KeyboardEvents|Z
  (params (Key :type Key%20Structure :default "None"))
  (:Pressed
    (CallFunction|SR)))

(event Input|KeyboardEvents|V
  (params (Key :type Key%20Structure :default "None"))
  (:Pressed
    (CallFunction|Aff)))

(event Custom|SR%20Init%20Inventory
  (Components|Activation|Activate (Variables|Default|GetInventory) false))

(event Custom|SR%20Init%20Hotbar
  (Components|Activation|Activate (Variables|Default|GetHotbar) false)
  (Variables|Default|SetEquipped%20Index 0)
  (Variables|Weapons|SetEquipped%20Item (.Item (Utilities|FindEquippedWeapon))))

(event Custom|SR%20Init%20Ammo
  (bind _ammo (Variables|Default|GetAmmo))
  (bind _dt_items (Variables|/Game/BigMaze/Core/Characters/PlayerCharacter/Components/BP_InventoryComponent.BP_InventoryComponent_C|GetDT%20Items _ammo))
  ;[1 1 1] Initializes the Ammo Inventory
  (Components|Activation|Activate (Variables|Default|GetAmmo) false)
  (Utilities|AsyncLoadAsset _dt_items
    (:Completed
      (for (_ _array_index) (Variables|/Game/BigMaze/Core/Characters/PlayerCharacter/Components/BP_InventoryComponent.BP_InventoryComponent_C|GetInventory _ammo)
        (bind _returnvalue (Utilities|GetDataTableRow (Utilities|ResolveSoftReference _dt_items) (Utilities|Select :Index _array_index :Option%200 "Rifle-Ammo" :Option%201 "Pistol-Ammo" :Option%202 "Sniper-Ammo" :Option%203 "Shotgun-Ammo" :Option%204 "Rocket-Ammo" :Option%205 "Universal-Ammo"))
          (:then
            (Default|InsertItem (Variables|Default|GetAmmo) _returnvalue _array_index)))))))

(event Custom|Update%20Component
  (Variables|Default|SetEquipped%20Index 0)
  (Variables|Weapons|SetEquipped%20Item (.Item (Utilities|FindEquippedWeapon))))

(fn ConstructionScript
  (Transformation|AttachComponentToComponent (Variables|Default|GetSK_HeldWeapon) (Variables|Character|GetMesh) "hand_r" "SnapToTarget" "KeepWorld" "KeepWorld" true)
  (Transformation|AttachComponentToComponent (Variables|Default|GetSK_Gun) (Variables|Default|GetFPMesh) "hand_r" "SnapToTarget" "KeepWorld" "KeepWorld" true))

(fn OnRepHealth
  (bind _self self)
  (bind _health (Variables|Health|GetHealth))
  (bind _shields (Variables|Health|GetShields))
  (Class|BPIHUD|SetHealthandShields(Message) (Pawn|GetController) _health _shields)
  (Class|BPIHUD|SetHealthandShields(Message) (UserInterface|GetWidget (Variables|Default|GetWidget)) _health _shields)
  (if (<= _health 0.0)
    (CallFunction|SRPlayerDeath _self (Pawn|GetLocalViewingPlayerController _self) (Variables|Health|GetLast%20Damager) (Variables|Health|GetDamagers) (Variables|Health|GetLast%20AI%20Damager) (Variables|Health|GetLast%20Damager%20AI?))))

(fn OnRepShields
  (Class|BPIHUD|SetHealthandShields(Message) (UserInterface|GetWidget (Variables|Default|GetWidget)) (Variables|Health|GetHealth) (Variables|Health|GetShields))
  (Class|BPIHUD|SetHealthandShields(Message) (Pawn|GetController) (Variables|Health|GetHealth) (Variables|Health|GetShields)))

(fn FUpdateWeaponStance)

(fn OnRepCurrentlyHoldingWeapon)

(fn OnRepHoldingWeapon)

(fn OnRepWeapon)

(fn OnRepEquippedItem
  (if (Pawn|IsLocallyControlled)
    (CallFunction|CLUpdateEquippedWeapon)))

(fn OnRepDamageMultiplier)

(fn OnRepEquippedIndex)

(fn FFindEquippedWeapon
  (bind (_valid_ _item) (Utilities|FindEquippedWeapon))
  (return _valid_ _item))

(fn (Char)GetEquippedItem
  (return (Variables|Default|GetEquipped%20Index) (.Item (Utilities|FindEquippedWeapon))))

(fn AddWeapontoInventory
  (params (Item%20Obj :type Object%20Object%20Reference))
  (return false))

(fn BPIDropItem
  (params (Item :type Item%20Struct%20Structure) (Index :type Integer))
  (return false))

(fn BPIExternalTradeatIndex
  (params (External%20Component :type BP%20Inventory%20Component%20Object%20Reference) (New%20Item :type Item%20Struct%20Structure) (New%20Item%20Current%20Index :type Integer) (Old%20Item :type Item%20Struct%20Structure) (Old%20Item%20Current%20Index :type Integer) (New%20External :type Boolean) (Old%20External :type Boolean))
  (return false))

(fn BPIInsertItem
  (params (New%20Item :type Item%20Struct%20Structure) (Destination%20Index :type Integer))
  (return false))

(fn BPIRemoveItem
  (params (Index :type Integer))
  (return false ""))

(fn BPISplitStack
  (params (Index :type Integer) (Desired%20Out%20Amount :type Integer))
  (return false "" ""))

(fn BPIStackItem
  (params (New%20Item :type Item%20Struct%20Structure) (Old%20Item :type Item%20Struct%20Structure) (Item%20Destination%20In :type Integer))
  (return false "" "" ""))

(fn BPITradeatIndex
  (params (New%20Item :type Item%20Struct%20Structure) (New%20Item%20Current%20Index :type Integer) (Old%20Item :type Item%20Struct%20Structure) (Old%20Item%20Current%20Index :type Integer))
  (return false))

(fn GetEquippedWeapon
  (return 0 0))

(fn GetNumberOfInventoryComponents
  (return true 3 (Utilities|Array|MakeArray (Variables|Default|GetInventory) (Variables|Default|GetHotbar) (Variables|Default|GetAmmo))))

(fn GetPlayerInfo
  (return ""))

(fn GetPlayerName
  (return "None"))

(fn InventoryCompsActive?
  (return (Math|Boolean|ANDBoolean (Variables|/Game/BigMaze/Core/Characters/PlayerCharacter/Components/BP_InventoryComponent.BP_InventoryComponent_C|GetInitialized (Variables|Default|GetInventory)) (Variables|/Game/BigMaze/Core/Characters/PlayerCharacter/Components/BP_InventoryComponent.BP_InventoryComponent_C|GetInitialized (Variables|Default|GetHotbar)) (Variables|/Game/BigMaze/Core/Characters/PlayerCharacter/Components/BP_InventoryComponent.BP_InventoryComponent_C|GetInitialized (Variables|Default|GetAmmo)))))

(fn RetrieveComponentReference
  (params (Index :type Integer))
  (bind _output_get (LocalVariables|SetComp (Utilities|Select :Index Index :Option%200 (Variables|Default|GetInventory) :Option%201 (Variables|Default|GetHotbar) :Option%202 (Variables|Default|GetAmmo))))
  (return (Utilities|IsValid _output_get) _output_get))

(fn RetrievePlayerstate
  (return 0))

(fn RetrieveScore
  (return "" ""))

(fn SpectatorAdd
  (return 0))