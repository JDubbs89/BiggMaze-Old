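; Player character component for the held item, handling its replication, reloading and use.
; SetCurrentItem runs on authority, assigning the item and passing it to remote machines through MCSetCurrentItem.
; Reload looks up the owner's "ammo" inventory via interface, picks the slot from the item's ammoid attribute, rewrites both stack counts and broadcasts the update.
; Primary use is cooldown-gated with an empty class switch, while secondary and tertiary use are stubs.
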(event `MC Set Current Item`
  (params (`New Item` :type "/Game/BigMaze/Core/ItemAssets/Common/Structs/S_ItemStruct Structure") (Component :type "/Game/BigMaze/Core/Characters/PlayerCharacter/Components/BP_AC_ItemFunction Object Reference"))
  ;[1 1 1] Replicated Item Update
  (`/Engine/EditorBlueprintResources/ActorComponentMacros.Switch Has Authority`
    (:`Remote`
      (set `/Game/BigMaze/Core/Characters/PlayerCharacter/Components/BP_AC_ItemFunction.Current item` `New Item` Component :!label _label))))

(event `Reload Current Item`
  (bind _current_item (`self.Current item`))
  (bind (_stackable_ _stack _max_stack _has_ammunition_) (`/Game/BigMaze/ItemSystem/Blueprints/BFL_Items.Get Stack Data` (`self.Current item`)))
  (bind _max_stack_size (`/Game/BigMaze/ItemSystem/Blueprints/BFL_Items.Get Max Stack Size` _current_item))
  (bind _int (`self.String to AmmoID Int` (`.Value` (`/Game/BigMaze/ItemSystem/Blueprints/BFL_Items.Get Specific Attribute` _current_item "ammoid"))))
  ;[1 1 1] Calls Reload Function If the Item is Reloadable
  (bind (_success _component) (message `/Game/BigMaze/Core/Characters/PlayerCharacter/Interfaces/BPI_InventoryComp.IC Retrieve Component Reference` (`self.GetOwner`) 2))
  (if (and (< _stack _max_stack) _has_ammunition_ (== (`/Game/BigMaze/Core/Characters/PlayerCharacter/Components/BP_InventoryComponent.Inventory Name` _component) "ammo") _success)
    (bind _output_get (set `self.Ammo Component` _component))
    (bind _output (`|GetArrayItem` (`/Game/BigMaze/Core/Characters/PlayerCharacter/Components/BP_InventoryComponent.Inventory` _output_get) _int))
    (bind _amount_in_stack (`/Game/BigMaze/ItemSystem/Blueprints/BFL_Items.Get Stack Count` _output))
    (bind _returnvalue (`KismetMathLibrary.SelectInt` _max_stack_size (+ (`/Game/BigMaze/ItemSystem/Blueprints/BFL_Items.Get Stack Count` _current_item) _amount_in_stack) (< _max_stack_size _amount_in_stack)))
    (bind _out_item (`/Game/BigMaze/ItemSystem/Blueprints/BFL_Items.Update Item Stack Count` _output (- _amount_in_stack _returnvalue)))
    (`/Game/BigMaze/Core/Characters/PlayerCharacter/Components/BP_InventoryComponent.SR Insert Item` (`self.Ammo Component`) _out_item _int)
    (bind _out_item_2 (`/Game/BigMaze/ItemSystem/Blueprints/BFL_Items.Update Item Stack Count` (`self.Current item`) _returnvalue))
    (`self.Exec Item Update` _out_item_2 "NewEnumerator7")))

(event `Set Current Item`
  (params (`New Item` :type "/Game/BigMaze/Core/ItemAssets/Common/Structs/S_ItemStruct Structure") (Component :type "/Game/BigMaze/Core/Characters/PlayerCharacter/Components/BP_AC_ItemFunction Object Reference"))
  ;[1 1 1] Replicated Item Update
  (`/Engine/EditorBlueprintResources/ActorComponentMacros.Switch Has Authority`
    (:`Authority`
      (`|ExecutionSequence`
        (:`then_0`
          (`self.MC Set Current Item` `New Item` Component))
        (:`then_1`
          (goto _label))))))

(event `Tertiary Use Current Item`)

(event `Secondary Use Current Item`)

(event `Use Current Item`
  (params (`Use Origin` :type "Vector Structure") (`Use Destination` :type "Vector Structure"))
  (if (not (`KismetSystemLibrary.K2_IsValidTimerHandle` (`self.Cooldown Timer`)))
    (switch `/Game/BigMaze/Core/ItemAssets/Common/Enums/E_ItemClass` (`/Game/BigMaze/ItemSystem/Blueprints/BFL_Items.Get Class` (`self.Current item`)))))