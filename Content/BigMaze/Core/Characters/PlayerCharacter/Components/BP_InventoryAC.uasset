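; BP_InventoryAC is a player character inventory component that stores items in an index-keyed map, pre-filled with null placeholders on BeginPlay.
; Functions add, stack, replace, split and remove items, check per-slot class and name allow/disallow rules, and fire item change callbacks.
; SR events on authority call MC events for remotes and repeat the same logic locally.
; Leftover, removed or replaced items spawn as BP_ItemActor at the owner's location.
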(event `MC Remove Item`
  (params (Target :type "Self Object Reference") (Name :type String) (Index :type Integer) (Amount :type Integer))
  ;[0 0.8125 1] Replication for Removing Item
  (`/Engine/EditorBlueprintResources/ActorComponentMacros.Switch Has Authority`
    (:`Remote`
      (bind (_success _removed_item) (`self.Remove Item` Target Name Index Amount :!label _label))
      (if (not (`/Game/BigMaze/ItemSystem/Blueprints/BFL_Items.Is Null` _removed_item))
        (`self.Drop Item` _removed_item)))))

(event `MC Zero Fill Inventory`
  (params (Inventory :type "Map of Integer to /Game/BigMaze/Core/ItemAssets/Common/Structs/ItemStruct Structure (by ref)") (`Inventory Size` :type Integer) (`Player Index` :type Integer))
  ;[0.1016 1 0] Fills Inventory With Null Item Values (Placeholders)
  (`/Engine/EditorBlueprintResources/ActorComponentMacros.Switch Has Authority`
    (:`Remote`
      (for _index (range `Inventory Size`) :!label _label_2
        (`BlueprintMapLibrary.Map_Add` Inventory _index (make `/Game/BigMaze/Core/ItemAssets/Common/Structs/ItemStruct`))
        (`KismetSystemLibrary.PrintString` (`KismetStringLibrary.Concat_StrStr` "Player: " (`KismetStringLibrary.Conv_IntToString` `Player Index`) "Inventory Length: " (`KismetStringLibrary.Conv_IntToString` `Inventory Size`)))))))

(event `SR Remove Item`
  (params (Target :type "/Game/BigMaze/Core/Characters/PlayerCharacter/Components/BP_InventoryAC Object Reference") (Name :type String) (Index :type Integer) (Amount :type Integer :default -1))
  ;[0 0.8125 1] Replication for Removing Item
  (`/Engine/EditorBlueprintResources/ActorComponentMacros.Switch Has Authority`
    (:`Authority`
      (`|ExecutionSequence`
        (:`then_0`
          (`self.MC Remove Item` Target Name Index Amount))
        (:`then_1`
          (goto _label))))))

(event `SR Zero Fill Inventory`
  (params (PlayerController :type "PlayerController Object Reference"))
  ;[0.1016 1 0] Fills Inventory With Null Item Values (Placeholders)
  (`/Engine/EditorBlueprintResources/ActorComponentMacros.Switch Has Authority`
    (:`Authority`
      (`|ExecutionSequence`
        (:`then_0`
          (`self.MC Zero Fill Inventory` (`self.Items`) (`self.Inventory Size`) (`AdvancedSessionsLibrary.GetNetPlayerIndex` PlayerController)))
        (:`then_1`
          (goto _label_2))))))

(event `MC Replace Item At Index`
  (params (Target :type "Self Object Reference") (`New Item` :type "/Game/BigMaze/Core/ItemAssets/Common/Structs/ItemStruct Structure") (`Target Index` :type Integer))
  ;[1 0 0.8906] Replication for Replacing Item
  (`/Engine/EditorBlueprintResources/ActorComponentMacros.Switch Has Authority`
    (:`Remote`
      (bind (_success _replaced_item) (`self.Replace Item at Index` Target `New Item` `Target Index` :!label _label_3))
      (if (not (`/Game/BigMaze/ItemSystem/Blueprints/BFL_Items.Is Null` _replaced_item))
        (`self.Drop Item` _replaced_item)))))

(event `SR Replace Item At Index`
  (params (Target :type "/Game/BigMaze/Core/Characters/PlayerCharacter/Components/BP_InventoryAC Object Reference") (`New Item` :type "/Game/BigMaze/Core/ItemAssets/Common/Structs/ItemStruct Structure") (`Target Index` :type Integer))
  ;[1 0 0.8906] Replication for Replacing Item
  (`/Engine/EditorBlueprintResources/ActorComponentMacros.Switch Has Authority`
    (:`Authority`
      (`|ExecutionSequence`
        (:`then_0`
          (`self.MC Replace Item At Index` Target `New Item` `Target Index`))
        (:`then_1`
          (goto _label_3))))))

(event `self.ReceiveBeginPlay`
  (`self.SR Zero Fill Inventory` (`GameplayStatics.GetPlayerController` 0)))

(event `MC Add Item`
  (params (Target :type "Self Object Reference") (Item :type "/Game/BigMaze/Core/ItemAssets/Common/Structs/ItemStruct Structure"))
  ;[0.6641 1 0] Replication for Adding Item
  (`/Engine/EditorBlueprintResources/ActorComponentMacros.Switch Has Authority`
    (:`Remote`
      (bind (_success _new_stack _has_leftover_item _leftover_item) (`self.Add Item` Target Item :!label _label_4))
      (if _has_leftover_item
        (bind (_success_2 _new_stack_2 _has_leftover_item_2 _leftover_item_2) (`self.Add Item` Target _leftover_item))
        (if _has_leftover_item_2
          (`self.Drop Item` _leftover_item_2))))))

(event `SR Add Item`
  (params (Target :type "/Game/BigMaze/Core/Characters/PlayerCharacter/Components/BP_InventoryAC Object Reference") (Item :type "/Game/BigMaze/Core/ItemAssets/Common/Structs/ItemStruct Structure"))
  ;[0.6641 1 0] Replication for Adding Item
  (`/Engine/EditorBlueprintResources/ActorComponentMacros.Switch Has Authority`
    (:`Authority`
      (`|ExecutionSequence`
        (:`then_0`
          (`self.MC Add Item` Target Item))
        (:`then_1`
          (goto _label_4))))))

(event `Drop Item`
  (params (Item :type "/Game/BigMaze/Core/ItemAssets/Common/Structs/ItemStruct Structure"))
  ;[0.6641 1 0] Replication for Adding Item
  (`/Engine/EditorBlueprintResources/ActorComponentMacros.Switch Has Authority`
    (:`Authority`
      (`|SpawnActorFromClass` "/Game/BigMaze/Core/Pickups/BP_ItemActor.BP_ItemActor_C" (`KismetMathLibrary.MakeTransform` (`Actor.K2_GetActorLocation` (`self.GetOwner`))) "AdjustIfPossibleButAlwaysSpawn" "MultiplyWithRoot" null Item null))))

(fn `Add Item`
  (params (Item :type "/Game/BigMaze/Core/ItemAssets/Common/Structs/ItemStruct Structure"))
  (returns (Success :type Boolean) (`New Stack` :type "/Game/BigMaze/Core/ItemAssets/Common/Structs/ItemStruct Structure") (`Has Leftover Item` :type Boolean) (`Leftover Item` :type "/Game/BigMaze/Core/ItemAssets/Common/Structs/ItemStruct Structure"))
  (bind (_index _full) (`self.Get First Available Index`))
  (bind _items (`self.Items`))
  (bind _item (`local.Item`))
  (bind _values (`BlueprintMapLibrary.Map_Values` (`self.Items`)))
  (if (`KismetArrayLibrary.Array_Contains` _values Item)
    (bind _returnvalue (`KismetArrayLibrary.Array_Find` _values Item))
    (bind (_success _combined_item _has_leftover_item _leftover_item) (`/Game/BigMaze/ItemSystem/Blueprints/BFL_Items.Add to Item Stack` (`BlueprintMapLibrary.Map_Find` (`self.Items`) _returnvalue) (`local.Item`)))
    (bind _keys (`BlueprintMapLibrary.Map_Keys` _items))
    (bind _output (`|GetArrayItem` _keys _returnvalue))
    (`BlueprintMapLibrary.Map_Add` _items _output _combined_item)
    (`self.Item Added` _combined_item _output)
    (return _success _combined_item _has_leftover_item _leftover_item)
    (else
      (if (not _full)
        (if (`self.Can Item Fit in Slot?` (`local.Item`) _index)
          (`BlueprintMapLibrary.Map_Add` (`self.Items`) _index _item)
          (`self.Item Added` _item _index)
          (return true _item false)
          (else
            (`KismetSystemLibrary.PrintString` "Failed: Item Cannot Occupy Slot")))
        (else
          (`KismetSystemLibrary.PrintString` "Failed: Inventory Full")))
      (return false (struct) false (`local.Item`)))))

(fn `Can Item Fit in Slot?`
  (params (Item :type "/Game/BigMaze/Core/ItemAssets/Common/Structs/ItemStruct Structure") (Index :type Integer))
  (returns (Fits :type Boolean))
  (bind ((`Name_2_C8A30FD44209EC8654ED65827C16873B` _name) (`ItemClass_34_463E1F7D44177C7E4922A6BF67BA516E` _itemclass)) (break `/Game/BigMaze/Core/ItemAssets/Common/Structs/ItemStruct` Item))
  (bind (_value _returnvalue) (`BlueprintMapLibrary.Map_Find` (`self.Slot Preferences`) Index))
  (bind _returnvalue_2 (`KismetStringLibrary.Conv_StringToName` _name))
  (bind (_classesallowed _classesdisallowed _itemsallowed _itemsdisallowed) (break `/Game/BigMaze/ItemSystem/Blueprints/S_SlotPreferences` _value))
  (return (or (and (or (`KismetArrayLibrary.Array_Contains` _classesallowed _itemclass) (not (`KismetArrayLibrary.Array_Contains` _classesdisallowed _itemclass))) (or (`KismetArrayLibrary.Array_Contains` _itemsallowed _returnvalue_2) (not (`KismetArrayLibrary.Array_Contains` _itemsdisallowed _returnvalue_2)))) (not _returnvalue))))

(fn `Get First Available Index`
  (returns (Index :type Integer) (Full :type Boolean))
  (locals (foundindex :type Integer))
  (bind _foundindex (`local.foundindex`))
  (bind _values (`BlueprintMapLibrary.Map_Values` (`self.Items`)))
  (for (_array_element _array_index) _values
    (if (not (`/Game/BigMaze/ItemSystem/Blueprints/BFL_Items.Is Null` _array_element))
      (set `local.foundindex` _array_index)
      (break)))
  (return _foundindex (== _foundindex -1)))

(fn `Get Item (Index)`
  (params (Index :type Integer))
  (returns (Item :type "/Game/BigMaze/Core/ItemAssets/Common/Structs/ItemStruct Structure") (Found :type Boolean))
  (bind (_value _returnvalue) (`BlueprintMapLibrary.Map_Find` (`self.Items`) Index))
  (return _value _returnvalue))

(fn `Get Item (Name)`
  (params (Name :type String))
  (returns (Index :type Integer) (`Out Item` :type "/Game/BigMaze/Core/ItemAssets/Common/Structs/ItemStruct Structure") (`Null?` :type Boolean))
  (locals (`Found index` :type Integer) (`Found item` :type "/Game/BigMaze/Core/ItemAssets/Common/Structs/ItemStruct Structure"))
  (bind _found_item (`local.Found item`))
  (bind _values (`BlueprintMapLibrary.Map_Values` (`self.Items`)))
  (for (_array_element _array_index) _values
    (if (`KismetStringLibrary.EqualEqual_StrStr` (`/Game/BigMaze/ItemSystem/Blueprints/BFL_Items.Get Name` _array_element) (`local.Name`))
      (set `local.Found index` _array_index)
      (set `local.Found item` _array_element)
      (break)))
  (return (`local.Found index`) _found_item (`/Game/BigMaze/ItemSystem/Blueprints/BFL_Items.Is Null` _found_item)))

(fn `Get Length`
  (returns (`Non Null Items` :type Integer))
  (locals (Count :type Integer :default 0))
  (bind _values (`BlueprintMapLibrary.Map_Values` (`self.Items`)))
  (for _array_element _values
    (if (not (`/Game/BigMaze/ItemSystem/Blueprints/BFL_Items.Is Null` _array_element))
      (`/Engine/EditorBlueprintResources/StandardMacros.IncrementInt` (`local.Count`))))
  (return (`local.Count`)))

(fn `Is Slot Empty?`
  (params (Index :type Integer))
  (returns (Empty :type Boolean))
  (bind (_value _returnvalue) (`BlueprintMapLibrary.Map_Find` (`self.Items`) Index))
  (return (or (`/Game/BigMaze/ItemSystem/Blueprints/BFL_Items.Is Null` _value) _returnvalue)))

(fn `Remove Item`
  (params (Name :type String :default "null") (Index :type Integer) (Amount :type Integer :default -1))
  (returns (Success :type Boolean) (`Removed Item` :type "/Game/BigMaze/Core/ItemAssets/Common/Structs/ItemStruct Structure"))
  (locals (ItemToRemove :type "/Game/BigMaze/Core/ItemAssets/Common/Structs/ItemStruct Structure"))
  (bind _index (`local.Index`))
  (bind _index_2 (`local.Index`))
  (bind (_index_3 _out_item) (`self.Get Item (Name)` (`local.Name`)))
  (bind _value (`BlueprintMapLibrary.Map_Find` (`self.Items`) (`local.Index`)))
  (bind (_index_4 _out_item_2) (`self.Get Item (Name)` (`local.Name`)))
  (if (== Amount -1)
    (if (== Name "null")
      (if (`/Game/BigMaze/ItemSystem/Blueprints/BFL_Items.Is Null` (`BlueprintMapLibrary.Map_Find` (`self.Items`) (`local.Index`)))
        (return false (make `/Game/BigMaze/Core/ItemAssets/Common/Structs/ItemStruct`))
        (else
          (bind (_success _replaced_item) (`self.Replace Item at Index` (make `/Game/BigMaze/Core/ItemAssets/Common/Structs/ItemStruct`) _index_2))
          (if _success
            (`self.Item Removed` _replaced_item _index_2))
          (return _success _replaced_item)))
      (else
        (bind _output_get (set `local.ItemToRemove` _out_item_2))
        (`BlueprintMapLibrary.Map_Add` (`self.Items`) _index_4 (make `/Game/BigMaze/Core/ItemAssets/Common/Structs/ItemStruct`))
        (`self.Item Removed` _output_get _index_4)
        (return true _output_get)))
    (elif (== Name "null")
      (if (`/Game/BigMaze/ItemSystem/Blueprints/BFL_Items.Is Null` _value)
        (return false (make `/Game/BigMaze/Core/ItemAssets/Common/Structs/ItemStruct`))
        (else
          (bind (_old_stack _new_stack _success_2) (`/Game/BigMaze/ItemSystem/Blueprints/BFL_Items.Split Item Stack` _value (`local.Amount`)))
          (if _success_2
            (`BlueprintMapLibrary.Map_Add` (`self.Items`) _index _old_stack)
            (`self.Item Dropped` _new_stack _index (`/Game/BigMaze/ItemSystem/Blueprints/BFL_Items.Get Stack Count` _new_stack)))
          (return _success_2 _new_stack)))
      (else
        (bind _output_get_2 (set `local.ItemToRemove` _out_item))
        (bind (_old_stack_2 _new_stack_2 _success_3) (`/Game/BigMaze/ItemSystem/Blueprints/BFL_Items.Split Item Stack` _output_get_2 (`local.Amount`)))
        (if _success_3
          (`BlueprintMapLibrary.Map_Add` (`self.Items`) _index_3 _old_stack_2)
          (`self.Item Dropped` _new_stack_2 _index_3 (`/Game/BigMaze/ItemSystem/Blueprints/BFL_Items.Get Stack Count` _new_stack_2))
          (return true _new_stack_2)
          (else
            (return false)))))))

(fn `Replace Item at Index`
  (params (`New Item` :type "/Game/BigMaze/Core/ItemAssets/Common/Structs/ItemStruct Structure") (`Target Index` :type Integer))
  (returns (Success :type Boolean) (`Replaced Item` :type "/Game/BigMaze/Core/ItemAssets/Common/Structs/ItemStruct Structure"))
  (locals (`Item to Replace` :type "/Game/BigMaze/Core/ItemAssets/Common/Structs/ItemStruct Structure"))
  (bind (_item _found) (`self.Get Item (Index)` (`local.Target Index`)))
  (if (`self.Can Item Fit in Slot?` `New Item` `Target Index`)
    (set `local.Item to Replace` (select `bool` _found :`false` (make `/Game/BigMaze/Core/ItemAssets/Common/Structs/ItemStruct`) :`true` _item))
    (`BlueprintMapLibrary.Map_Add` (`self.Items`) (`local.Target Index`) (`local.New Item`))
    (`self.Item Added` (`local.New Item`) (`local.Target Index`))
    (return true (`local.Item to Replace`))
    (else
      (return false (make `/Game/BigMaze/Core/ItemAssets/Common/Structs/ItemStruct`)))))