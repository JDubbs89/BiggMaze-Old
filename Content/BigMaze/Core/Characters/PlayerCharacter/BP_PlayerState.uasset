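; BP_PlayerState is the player state for BigMaze, holding one player's score record as an SPlayerScore struct.
; PSetPlayerInfo rebuilds that record from incoming info, stamping in the current ping and a reference to itself, and PGetPlayerInfo returns it.
; The other P-prefixed functions for weapons, inventory, name and spectating are stubs returning defaults or nothing, and the death and respawn events are empty.
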(event `self.ReceiveBeginPlay`)

(event `self.Player Death`)

(event `self.Player Respawn`
  (params (Controller :type "PlayerController Object Reference")))

(event `/Game/BigMaze/Core/Characters/PlayerCharacter/Interfaces/BPI_Player.P Set Player Info`
  (params (Info :type "/Game/BigMaze/Core/GameModes/Extraction/Structs/S_PlayerScore Structure"))
  (bind (_name _id _kills _deaths _assists _score _deathscore _ping _alive) (break `/Game/BigMaze/Core/GameModes/Extraction/Structs/S_PlayerScore` Info))
  (bind _output_get (set `self.Player Score` (make `/Game/BigMaze/Core/GameModes/Extraction/Structs/S_PlayerScore` _name _id _kills _deaths _assists _score _deathscore (`self.GetPingInMilliseconds`) _alive self))))

(fn `P Add Weapon to Inventory`
  (params (`Item Obj` :type "Object Object Reference"))
  (returns (Success :type Boolean))
  (return false))

(fn `P Get Equipped Weapon`
  (returns (`Weapon Index` :type Integer) (WeaponObjs :type "Map of Integer to Object Object Reference"))
  (return 0))

(fn `P Get Player Info`
  (returns (Info :type "/Game/BigMaze/Core/GameModes/Extraction/Structs/S_PlayerScore Structure"))
  (return (`self.Player Score`)))

(fn `P Get Player Name`
  (returns (`Player Name` :type Name))
  (return "None"))

(fn `P Inventory Comps Active?`
  (returns (True :type Boolean))
  (return false))

(fn `P Retrieve Playerstate`
  (returns (PS :type "/Game/BigMaze/Core/Characters/PlayerCharacter/BP_PlayerState Object Reference"))
  (return null))

(fn `P Spectator Add`
  (returns (`Return HUD` :type "/Game/BigMaze/Core/UI/HUD/OnScreen/WBP_HUDMain Object Reference"))
  (return null))

(fn `UserConstructionScript`)