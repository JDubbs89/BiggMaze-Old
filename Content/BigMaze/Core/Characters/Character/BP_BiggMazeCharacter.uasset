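; Networked player character for BigMaze, handling Enhanced Input movement, look, jump, crouch, sprint and hotbar item switching.
; Sprint speed, jump state and camera pitch go through server RPCs, with pitch multicast to clients and jump/land multicasts left as empty hooks.
; Number keys or scroll (optionally looping) set EquippedIndex on the server.
; Its OnRep equips through HotbarComponent, whose ItemEquipped event sets EquippedItem, whose OnRep updates the view model.
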(event `SR Set Equipped Index`
  (params (Char :type "/Game/BigMaze/Core/Characters/Character/BP_BiggMazeCharacter Object Reference") (Index :type Integer))
  ;[1 0.5156 0] Change Equipped Hotbar Index
  (bind _output_get (set `/Game/BigMaze/Core/Characters/Character/BP_BiggMazeCharacter.Equipped Index` Index Char))
  (`KismetSystemLibrary.PrintString` (`KismetStringLibrary.Conv_IntToString` _output_get)))

(event `EnhancedInput|/Game/BigMaze/Core/Engine/Inputs/Keys/IA_Scroll`
  (params (ActionValue :type "Float (double-precision)") (ElapsedSeconds :type "Float (double-precision)") (TriggeredSeconds :type "Float (double-precision)") (InputAction :type "InputAction Object Reference" :default "/Game/BigMaze/Core/Engine/Inputs/Keys/IA_Scroll.IA_Scroll"))
  ;[1 0.5156 0] Change Equipped Hotbar Index
  (:`Started`
    (`self.Find Next Valid Index` (`/Game/UlimateBlueprintPack/System/Blueprints/UBPP_FunctionLibrary.Bigger Than Zero (Float)` ActionValue))))

(event `EnhancedInput|/Game/BigMaze/Core/Engine/Inputs/Keys/IA_Move`
  (params (ActionValue :type "Vector2D Structure") (ElapsedSeconds :type "Float (double-precision)") (TriggeredSeconds :type "Float (double-precision)") (InputAction :type "InputAction Object Reference" :default "/Game/BigMaze/Core/Engine/Inputs/Keys/IA_Move.IA_Move"))
  (bind (_returnvalue_roll _returnvalue_pitch _returnvalue_yaw) (`KismetMathLibrary.BreakRotator` (`self.K2_GetActorRotation`)))
  ;[0.5469 1 0] Move Around
  (:`Triggered`
    (`self.AddMovementInput` (* (`KismetMathLibrary.GetForwardVector` (`KismetMathLibrary.MakeRotator` 0.0 _returnvalue_pitch _returnvalue_yaw)) (`self.Forward Movement Multiplier`)) ActionValue_Y)
    (`self.AddMovementInput` (* (`KismetMathLibrary.GetRightVector` (`KismetMathLibrary.MakeRotator` _returnvalue_roll 0.0 _returnvalue_yaw)) (`self.Right Movement Multiplier`)) ActionValue_X)))

(event `EnhancedInput|/Game/BigMaze/Core/Engine/Inputs/Keys/IA_Hotbar1`
  (params (ActionValue :type Boolean) (ElapsedSeconds :type "Float (double-precision)") (TriggeredSeconds :type "Float (double-precision)") (InputAction :type "InputAction Object Reference" :default "/Game/BigMaze/Core/Engine/Inputs/Keys/IA_Hotbar1.IA_Hotbar1"))
  ;[1 0.5156 0] Change Equipped Hotbar Index
  (:`Started`
    (if (`self.Is Index Valid?` (`self.HotbarComponent`))
      (`self.SR Set Equipped Index` self))))

(event `SR_Jump`
  ;[0 1 0.01562] Jumping
  (set `self.Jumping` true :!label _label)
  (bind _result (`/Game/UlimateBlueprintPack/System/Blueprints/UBPP_MacroLibrary.Increment Int By` (`self.Jump Count`))
    (:`  `
      (`self.MC_Jump` _result))))

(event `EnhancedInput|/Game/BigMaze/Core/Engine/Inputs/Keys/IA_Jump`
  (params (ActionValue :type Boolean) (ElapsedSeconds :type "Float (double-precision)") (TriggeredSeconds :type "Float (double-precision)") (InputAction :type "InputAction Object Reference" :default "/Game/BigMaze/Core/Engine/Inputs/Keys/IA_Jump.IA_Jump"))
  ;[0 1 0.01562] Jumping
  (:`Started`
    (`self.Jump`)
    (`/Engine/EditorBlueprintResources/ActorMacros.Switch Has Authority`
      (:`Authority`
        (goto _label))
      (:`Remote`
        (`self.SR_Jump`))))
  (:`Completed`
    (`self.StopJumping`)
    (`/Engine/EditorBlueprintResources/ActorMacros.Switch Has Authority`
      (:`Authority`
        (set `self.Jumping` false :!label _label_2)
        (`self.MC_StopJump`))
      (:`Remote`
        (`self.SR_StopJump`)))))

(event `MC_Jump`
  (params (JumpCount :type "Integer (by ref)"))
  ;[0 1 0.01562] Jumping
)

(event `self.HotbarComponent.Item Equipped`
  (params (Item :type "ItemFunctionalityBase Object Reference") (Index :type Integer) (Data :type "Item Structure"))
  (bind _asa_item_function (cast `/Game/BigMaze/Core/ItemSystem2/Actors/ItemFunctions/A_ItemFunction` Item))
  (`self.Set Equipped Item` _asa_item_function Data))

(event `MC_StopJump`
  ;[0 1 0.01562] Jumping
)

(event `SR_StopJump`
  ;[0 1 0.01562] Jumping
  (goto _label_2))

(event `EnhancedInput|/Game/BigMaze/Core/Engine/Inputs/Keys/IA_Hotbar2`
  (params (ActionValue :type Boolean) (ElapsedSeconds :type "Float (double-precision)") (TriggeredSeconds :type "Float (double-precision)") (InputAction :type "InputAction Object Reference" :default "/Game/BigMaze/Core/Engine/Inputs/Keys/IA_Hotbar2.IA_Hotbar2"))
  ;[1 0.5156 0] Change Equipped Hotbar Index
  (:`Started`
    (if (`self.Is Index Valid?` (`self.HotbarComponent`) 1)
      (`self.SR Set Equipped Index` self 1))))

(event `Set Equipped Item`
  (params (`Equipped Item` :type "/Game/BigMaze/Core/ItemSystem2/Actors/ItemFunctions/A_ItemFunction Object Reference") (Data :type "Item Structure (by ref)"))
  (bind _output_get (set `self.Equipped Item` `Equipped Item`))
  (`ItemFunctionalityBase.OnSwapItem` _output_get Data true))

(event `MC_Land`
  ;[0 1 0.01562] Jumping
)

(event `SR_Land`
  ;[0 1 0.01562] Jumping
  (set `self.Jumping` false)
  (set `self.Jump Count` 0)
  (`self.MC_Land`))

(event `EnhancedInput|/Game/BigMaze/Core/Engine/Inputs/Keys/IA_Crouch`
  (params (ActionValue :type Boolean) (ElapsedSeconds :type "Float (double-precision)") (TriggeredSeconds :type "Float (double-precision)") (InputAction :type "InputAction Object Reference" :default "/Game/BigMaze/Core/Engine/Inputs/Keys/IA_Crouch.IA_Crouch"))
  ;[1 0.4219 0] Crouch
  (:`Started`
    (`self.Crouch`))
  (:`Completed`
    (`self.UnCrouch`)))

(event `self.OnLanded`
  (params (Hit :type "HitResult Structure (by ref)"))
  ;[0 1 0.01562] Jumping
  (`self.SR_Land`))

(event `EnhancedInput|/Game/BigMaze/Core/Engine/Inputs/Keys/IA_Hotbar3`
  (params (ActionValue :type Boolean) (ElapsedSeconds :type "Float (double-precision)") (TriggeredSeconds :type "Float (double-precision)") (InputAction :type "InputAction Object Reference" :default "/Game/BigMaze/Core/Engine/Inputs/Keys/IA_Hotbar3.IA_Hotbar3"))
  ;[1 0.5156 0] Change Equipped Hotbar Index
  (:`Started`
    (if (`self.Is Index Valid?` (`self.HotbarComponent`) 2)
      (`self.SR Set Equipped Index` self 2))))

(event `EnhancedInput|/Game/BigMaze/Core/Engine/Inputs/Keys/IA_Sprint`
  (params (ActionValue :type Boolean) (ElapsedSeconds :type "Float (double-precision)") (TriggeredSeconds :type "Float (double-precision)") (InputAction :type "InputAction Object Reference" :default "/Game/BigMaze/Core/Engine/Inputs/Keys/IA_Sprint.IA_Sprint"))
  (bind _charactermovement (`self.CharacterMovement`))
  ;[0.8984 0 1] Sprint
  (:`Started`
    (`self.SR_Sprint`)
    (set `CharacterMovementComponent.MaxWalkSpeed` (`self.Sprint Speed`) _charactermovement))
  (:`Completed`
    (`self.SR_StopSprint`)
    (set `CharacterMovementComponent.MaxWalkSpeed` (`self.Walk Speed`) _charactermovement)))

(event `SR_Sprint`
  ;[0.8984 0 1] Sprint
  (set `CharacterMovementComponent.MaxWalkSpeed` (`self.Sprint Speed`) (`self.CharacterMovement`)))

(event `SR_StopSprint`
  ;[0.8984 0 1] Sprint
  (set `CharacterMovementComponent.MaxWalkSpeed` (`self.Walk Speed`) (`self.CharacterMovement`)))

(event `EnhancedInput|/Game/BigMaze/Core/Engine/Inputs/Keys/IA_Look`
  (params (ActionValue :type "Vector2D Structure") (ElapsedSeconds :type "Float (double-precision)") (TriggeredSeconds :type "Float (double-precision)") (InputAction :type "InputAction Object Reference" :default "/Game/BigMaze/Core/Engine/Inputs/Keys/IA_Look.IA_Look"))
  (bind (_returnvalue_roll _returnvalue_pitch) (`KismetMathLibrary.BreakRotator` (`SceneComponent.K2_GetComponentRotation` (`self.Camera`))))
  ;[0 1 0.5781] Look
  (:`Triggered`
    (`self.AddControllerYawInput` (* ActionValue_X (`self.Sensitivity X`)))
    (`self.AddControllerPitchInput` (* ActionValue_Y (`self.Sensitivity Y`)))
    (`self.SR_Rotate` _returnvalue_pitch)))

(event `SR_Rotate`
  (params (`New Pitch` :type "Float (double-precision)"))
  ;[1 0.6094 0] Camera Rotation Replication
  (`self.MC_Rotate` `New Pitch`))

(event `MC_Rotate`
  (params (`New Pitch` :type "Float (double-precision)"))
  (bind _camera (`self.Camera`))
  (bind (_returnvalue_roll _returnvalue_pitch _returnvalue_yaw) (`KismetMathLibrary.BreakRotator` (`SceneComponent.K2_GetComponentRotation` _camera)))
  ;[1 0.6094 0] Camera Rotation Replication
  (`SceneComponent.K2_SetWorldRotation` _camera (`KismetMathLibrary.MakeRotator` _returnvalue_roll `New Pitch` _returnvalue_yaw) false false))

(fn `Find Next Valid Index`
  (params (`Next?` :type Boolean))
  (bind (_index _valid_ _last_) (`self.Get Next or Prev Index` `Next?`))
  (bind _next_ (`local.Next?`))
  (bind _items (`/Game/BigMaze/Core/ItemSystem2/Components/AC_InventoryComponent.Items` (`self.HotbarComponent`)))
  (if _valid_
    (`self.SR Set Equipped Index` self _index)
    (elif _last_
      (if (`self.Scroll Loops?`)
        (if (`.Valid?` (`/Game/BigMaze/Core/ItemSystem2/Libraries/BFL_ItemSystem.Is Item Valid` (select `bool` (`local.Next?`) :`false` (`.Reference Output` (`/Game/UlimateBlueprintPack/System/Blueprints/UBPP_MacroLibrary.Last Item` _items)) :`true` (`|GetArrayItem` _items))))
          (`self.SR Set Equipped Index` self (`KismetMathLibrary.SelectInt` 0 (`KismetArrayLibrary.Array_LastIndex` _items) _next_))))
      (else
        (`self.Find Next Valid Index` _next_)))))

(fn `OnRep_Equipped Index`
  (`/Game/BigMaze/Core/ItemSystem2/Components/AC_InventoryComponent.Equip Item` (`self.HotbarComponent`) (`self.Equipped Index`)))

(fn `OnRep_Equipped Item`
  (bind _hotbarcomponent (`self.HotbarComponent`))
  (bind _view_model (`/Game/BigMaze/Core/ItemSystem2/Components/AC_PlayerInventoryComponent.View Model` _hotbarcomponent)
    (:`then`
      (`/Game/BigMaze/Core/UI/ViewModels/BP_InventoryViewModel.Set Equipped Item` _view_model (`|GetArrayItem` (`/Game/BigMaze/Core/ItemSystem2/Components/AC_InventoryComponent.Items` _hotbarcomponent) (`self.Equipped Index`))))
    (:`else`)))

(fn `UserConstructionScript`)