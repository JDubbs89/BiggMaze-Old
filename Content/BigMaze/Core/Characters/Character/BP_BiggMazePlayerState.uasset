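; Player state for BigMaze that ties the player's Gameplay Ability System health attributes to an MVVM character view model.
; On BeginPlay it fills or creates the view model with current, max and regen health, then applies the GE_PlayerStats effect.
; Unconnected logic, which never runs, would update the view model and apply GE_Regenerate when a health comparison passes and the regenerating tag is absent.
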(event `self.ReceiveBeginPlay`
  (bind (_currenthealth _bsuccessfullyfoundattribute _maxhealth _bsuccessfullyfoundattribute2 _regenhealth) (`self.Get Attribute Values`))
  (bind _attributeviewmodel (`self.AttributeViewModel`)
    (:`then`
      (set `/Game/BigMaze/Core/GAS/ViewModel/BP_BMCharacterVM.CurrentHealth` _currenthealth _attributeviewmodel)
      (set `/Game/BigMaze/Core/GAS/ViewModel/BP_BMCharacterVM.MaxHealth` _maxhealth _attributeviewmodel)
      (set `/Game/BigMaze/Core/GAS/ViewModel/BP_BMCharacterVM.RegenHealth` _regenhealth _attributeviewmodel))
    (:`else`
      (bind _returnvalue (`|GenericCreateObject` "/Game/BigMaze/Core/GAS/ViewModel/BP_BMCharacterVM.BP_BMCharacterVM_C" _currenthealth _maxhealth _regenhealth))
      (set `self.AttributeViewModel` _returnvalue)))
  (`AbilitySystemComponent.BP_ApplyGameplayEffectToSelf` :`self` (`self.AbilitySystemComponent`) :`GameplayEffectClass` "/Game/BigMaze/Core/GAS/GameplayEffects/GE_PlayerStats.GE_PlayerStats_C" :`Level` 1.0))

(fn `UserConstructionScript`)