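; HUD class for BiggMaze that draws a configurable crosshair and hosts the core HUD widget.
; DrawHUD renders a center dot and four lines, using helper math relative to screen center.
; EventInitHUD sets game-only input, shows the crosshair and creates WB_CoreHUD once the controlled character's health view model is available.
; A retry macro polls for that view model with Delay and DoN; SetHealthUIEnabled is an empty stub.
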(event `self.ReceiveDrawHUD`
  (params (SizeX :type Integer) (SizeY :type Integer))
  (bind _returnvalue (`KismetMathLibrary.Conv_IntToDouble` SizeY))
  (bind _returnvalue_2 (`KismetMathLibrary.Conv_IntToDouble` SizeX))
  (bind _h_thickness (`self.H Thickness`))
  (bind _v_thickness (`self.V Thickness`))
  (bind _cc_color (`self.CC Color`))
  (bind (_x1 _y1) (`self.Get CC Center` _returnvalue_2 _returnvalue))
  (bind (_a _a2 _b _b2 _y) (`self.Get Hor Lines` _returnvalue_2 _returnvalue))
  (bind (_a_2 _a2_2 _b_2 _b2_2 _x) (`self.Get Vert Lines` _returnvalue_2 _returnvalue))
  (if (`self.Crosshair Visible`)
    (`self.DrawLine` _x1 _y1 _x1 _y1 (`self.CC Color`) (`self.Center Dot Thickness`))
    (`self.DrawLine` _a _y _b _y _cc_color _h_thickness)
    (`self.DrawLine` _a2 _y _b2 _y _cc_color _h_thickness)
    (`self.DrawLine` _x _a_2 _x _b_2 _cc_color _v_thickness)
    (`self.DrawLine` _x _a2_2 _x _b2_2 _cc_color _v_thickness)))

(event `/Game/BigMaze/Core/Characters/Character/Interfaces/BI_HUD.Init HUD (To HUD)`
  (`WidgetBlueprintLibrary.SetInputMode_GameOnly` (`self.GetOwningPlayerController`))
  (set `self.Crosshair Visible` true)
  (`/Engine/EditorBlueprintResources/StandardMacros.IsValid` (`self.CoreHUD Widget`)
    (:`Is Valid`
      _)
    (:`Is Not Valid`
      (bind _view_model (`self.Get Health View Model` 10 0.1)
        (:`Success`
          (bind _returnvalue (`|CreateWidget` "/Game/BigMaze/Core/UI/BiggMazeHUD/Widgets/WB_CoreHUD.WB_CoreHUD_C" null _view_model))
          (set `self.CoreHUD Widget` _returnvalue)))))
  (if (not (`Widget.IsInViewport` (`self.CoreHUD Widget`)))
    (`UserWidget.AddToViewport` (`self.CoreHUD Widget`) 0)))

(event `/Game/BigMaze/Core/Characters/Character/Interfaces/BI_HUD.Set Health UI Enabled`
  (params (Enable :type Boolean))
  (if Enable
    _))

(fn `UserConstructionScript`)