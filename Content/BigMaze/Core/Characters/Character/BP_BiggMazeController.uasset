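; Player controller for BiggMaze that sets up input, the controlled character reference and the HUD.
; InitPlayerController adds the default Enhanced Input mapping context, then uses GetBiggMazeCharacter to retry retrieval until success or timeout.
; On success it caches the character and initializes the HUD message connection; both outcomes print a log.
; An older timer-polling route through TrySetPawnRef and TryInitializeCoreHUD remains, but its timer setup is disconnected.
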(event `Try Initialize Core HUD`
  ;[1 0 0.4453] Tries to initialize HUD widgets based on qualifying factors
  (if (not (`KismetSystemLibrary.K2_IsTimerActiveHandle` (`self.Pawn Ref Timer`)))
    (message `/Game/BigMaze/Core/Characters/Character/Interfaces/BI_HUD.Init HUD (To HUD)` (`self.GetHUD`))
    (`KismetSystemLibrary.K2_ClearAndInvalidateTimerHandle` (`self.Hud Init Timer`))))

(event `Try Set Pawn Ref`
  (bind _returnvalue (`self.K2_GetPawn`))
  ;[0 1 0.6953] Tries to cast to the controlled pawn and cache a casted reference as a variable.
  (`/Engine/EditorBlueprintResources/StandardMacros.IsValid` _returnvalue
    (:`Is Valid`
      (bind _asbp_bigg_maze_character (cast `/Game/BigMaze/Core/Characters/Character/BP_BiggMazeCharacter` _returnvalue))
      (set `self.Controlled Character` _asbp_bigg_maze_character)
      (`KismetSystemLibrary.K2_ClearAndInvalidateTimerHandle` (`self.Pawn Ref Timer`)))))

(event `Init Player Controller`
  (`|ExecutionSequence`
    (:`then_0`
      (`EnhancedInputSubsystemInterface.AddMappingContext` (subsystem `EnhancedInputLocalPlayerSubsystem`) "/Game/BigMaze/Core/Engine/Inputs/IMC_Default.IMC_Default" 0 (struct)))
    (:`then_1`
      (bind _asbp_bigg_maze_character (`/Game/BigMaze/Core/Characters/Character/BML_PlayerController.Get BiggMaze Character` 10)
        (:`Success`
          (set `self.Controlled Character` _asbp_bigg_maze_character)
          (message `/Game/BigMaze/Core/Characters/Character/Interfaces/BI_HUD.Init HUD (To HUD)` (`self.GetHUD`))
          (`KismetSystemLibrary.PrintString` "[BP_BiggMazeController - BeginPlay]: \nCharacter Reference retrieved." true true (struct :`R` 0.057249 :`G` 1.0 :`A` 1.0)))
        (:`Failed`
          (`KismetSystemLibrary.PrintString` "[BP_BiggMazeController - BeginPlay]: \nFailed to retrieve Character Reference." true true (struct :`R` 1.0 :`G` 0.027472 :`A` 1.0)))))))

(fn `UserConstructionScript`)