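; World item pickup that transfers its Item into the inventory of an actor overlapping its box.
; Construction can fill the Item from a data table row plus attribute modifiers, then applies its physics-simulated skeletal mesh through server/multicast-named events.
; Pickups with a valid previous owner are blocked for 0.75 seconds after BeginPlay.
; Overlap searches the actor's inventory components through interfaces, destroying the pickup on successful insertion or resetting its DoOnce after a delay.
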(event `SR Update Meshes`
  (`self.MC Update Meshes`))

(event `MC Update Meshes`
  (bind _skeletalmesh (`self.SkeletalMesh`))
  (bind (_name _description _icon _amountinstack _maxstacksize _itemclass _itemvalue _backdropcolor _skeletalmesh_2) (break `/Game/BigMaze/Core/ItemAssets/Common/Structs/ItemStruct` (`self.Item`)))
  (if (`KismetSystemLibrary.IsValid` _skeletalmesh_2)
    (`SkeletalMeshComponent.SetSkeletalMeshAsset` _skeletalmesh _skeletalmesh_2)
    (`PrimitiveComponent.SetSimulatePhysics` _skeletalmesh true)))

(event `self.ReceiveBeginPlay`
  (`KismetSystemLibrary.K2_SetTimerDelegate` (delegate `Reset`) 0.75)
  (`|LoadAsset` (`self.DT`)
    (:`Completed`
      (set `self.DT Loaded` true))))

(event `Reset`
  (set `self.Can Pickup` true))

(event `SR DEstroy Actor`
  (`self.K2_DestroyActor`))

(event `PickUp`
  (params (Target :type "Object Object Reference"))
  (bind _previous_owner (`self.Previous Owner`))
  (`/Engine/EditorBlueprintResources/StandardMacros.DoOnce` false :!label _label
    (:`Completed`
      (if (not (and (or (== Target _previous_owner) (`KismetSystemLibrary.IsValid` _previous_owner)) (not (`self.Can Pickup`))))
        (bind (_has_component _out_number) (message `/Game/BigMaze/Core/Characters/PlayerCharacter/Interfaces/BPI_InventoryComp.IC Get Number of Inventory Components` Target))
        (if _has_component
          (for _index (range _out_number)
            (bind (_success _component) (message `/Game/BigMaze/Core/Characters/PlayerCharacter/Interfaces/BPI_InventoryComp.IC Retrieve Component Reference` Target _index))
            (if _success
              (bind (_success_2 _index_2) (`/Game/BigMaze/Core/Characters/PlayerCharacter/Components/BP_InventoryComponent.Find Last Item Index` _component))
              (if (and (`KismetSystemLibrary.DoesImplementInterface` _component "/Game/BigMaze/Core/Characters/PlayerCharacter/Interfaces/BPI_InventoryComp.BPI_InventoryComp_C") _success_2)
                (bind _success_ (`/Game/BigMaze/Core/Characters/PlayerCharacter/Components/BP_InventoryComponent.Insert Item` _component (`self.Item`) _index_2))
                (if _success_
                  (set `self.Pickup Success` true)
                  (break)))))
          (if (`self.Pickup Success`)
            (`self.SR DEstroy Actor`)
            (else
              (`KismetSystemLibrary.Delay` 1.0)
              (goto _label :!via `Reset`))))))))

(event `self.Box.OnComponentBeginOverlap`
  (params (OverlappedComponent :type "PrimitiveComponent Object Reference") (OtherActor :type "Actor Object Reference") (OtherComp :type "PrimitiveComponent Object Reference") (OtherBodyIndex :type Integer) (bFromSweep :type Boolean) (SweepResult :type "HitResult Structure (by ref)"))
  (`self.PickUp` OtherActor))

(fn `UserConstructionScript`
  (if (and (`self.Use Data Table`) (`self.DT Loaded`))
    (bind _returnvalue (`|GetDataTableRow` (`|ConvertAsset` (`self.DT`)) (`self.Row Name`))
      (:`then`
        (bind _output_get (set `self.Item` _returnvalue))
        (bind _values (`BlueprintMapLibrary.Map_Values` (`self.Attribute Modifiers`)))
        (bind _keys (`BlueprintMapLibrary.Map_Keys` (`self.Attribute Modifiers`)))
        (for (_array_element _array_index) _values
          (`BlueprintMapLibrary.Map_Add` (`.UniqueAttributes_28_D97642464C73B875ED3C1FB98B20E72B` (break `/Game/BigMaze/Core/ItemAssets/Common/Structs/ItemStruct` _output_get)) (`|GetArrayItem` _keys _array_index) _array_element)))))
  (`/Engine/EditorBlueprintResources/ActorMacros.Switch Has Authority`
    (:`Authority`
      (`self.MC Update Meshes`))
    (:`Remote`
      (`self.SR Update Meshes`))))