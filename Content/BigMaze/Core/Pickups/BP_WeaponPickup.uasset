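; Pickup actor that presents the item held in Obj and offers it to any overlapping actor that can take it.
; On BeginPlay it switches on item type: weapons set a skeletal mesh and show their current magazine count as text, while ammunition, upgrades and attachments set a static mesh.
; Sphere overlap passes Obj through an inventory interface message, destroying the pickup on success and printing a debug string on failure.
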(event `self.ReceiveBeginPlay`
  (switch `/Game/BigMaze/Core/Items/Common/Enums/E_ItemClass` (`/Game/BigMaze/Core/Pickups/BP_WeaponPickup.Item Type` (`.Obj` (`self.Obj`)))
    (:`NewEnumerator0`
      (`SkinnedMeshComponent.SetSkinnedAssetAndUpdate` (`self.SkeletalMesh`) (`self.Get Skeletal Mesh` (`.Obj` (`self.Obj`))) true :!label _label)
      (`TextRenderComponent.K2_SetText` (`self.TextRender`) (`KismetTextLibrary.Conv_IntToText` (`.CurrentMagazine_45_37D0BAA74DD420A4B99704A8059BDC9C` (break `/Game/BigMaze/Core/Items/Common/Structs/S_WeaponInfo` (`self.Get Weapon Info` (`.Obj` (`self.Obj`))))))))
    (:`NewEnumerator1`
      (goto _label))
    (:`NewEnumerator5`
      (goto _label))
    (:`NewEnumerator3`
      (`StaticMeshComponent.SetStaticMesh` (`self.StaticMesh`) (`self.Get Static Mesh` (`.Obj` (`self.Obj`))) :!label _label_2))
    (:`NewEnumerator2`
      (goto _label_2))
    (:`NewEnumerator4`
      (goto _label_2))))

(event `self.Sphere.OnComponentBeginOverlap`
  (params (OverlappedComponent :type "PrimitiveComponent Object Reference") (OtherActor :type "Actor Object Reference") (OtherComp :type "PrimitiveComponent Object Reference") (OtherBodyIndex :type Integer) (bFromSweep :type Boolean) (SweepResult :type "HitResult Structure (by ref)"))
  (if (`KismetSystemLibrary.DoesImplementInterface` OtherActor)
    (bind _success (message `/Game/BigMaze/Core/Pickups/BP_WeaponPickup.Add Weapon to Inventory` OtherActor (`.Obj` (`self.Obj`))))
    (if _success
      (`self.K2_DestroyActor`)
      (else
        (`KismetSystemLibrary.PrintString` "Hello")))))

(fn `UserConstructionScript`)