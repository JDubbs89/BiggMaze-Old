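; BP_ItemActor is a world pickup that shows its Item's skeletal mesh and moves that item into an overlapping player's inventory.
; BeginPlay and OnRep_Item refresh the mesh through server and multicast events.
; On overlap, SRPickup inserts most items into inventory component 1, falling back to 0 when no index is found, while one class (apparently ammo) requires a name match in component 2.
; Successful insertion destroys the actor and updates the hotbar.
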(event `Update Mesh Server`
  (`self.Update Mesh Multicast`))

(event `Update Mesh Multicast`
  (bind (_item_name _item_description _item_icon _item_amountinstack _item_maxstacksize _item_itemclass _item_itemvalue _item_backdropcolor _item_skeletalmesh) (break `/Game/BigMaze/Core/ItemAssets/Common/Structs/ItemStruct` (`self.Item`)))
  (`SkeletalMeshComponent.SetSkeletalMeshAsset` (`self.SkeletalMesh`) _item_skeletalmesh))

(event `self.ReceiveBeginPlay`
  (`self.Update Mesh Server`))

(event `SR Pickup`
  (params (Actor :type "Actor Object Reference"))
  (bind _item (`self.Item`))
  (bind _asbp_character (cast `/Game/BigMaze/Core/Characters/PlayerCharacter/BP_Character` Actor)
    (:`then`
      (set `self.BP Character Ref` _asbp_character)
      (if (`|EnumInequality` (`/Game/BigMaze/ItemSystem/Blueprints/BFL_Items.Get Class` (`self.Item`)) "NewEnumerator3")
        (bind (_success _component) (message `/Game/BigMaze/Core/Characters/PlayerCharacter/Interfaces/BPI_InventoryComp.IC Retrieve Component Reference` Actor 1))
        (if _success
          (bind (_success_2 _index) (`/Game/BigMaze/Core/Characters/PlayerCharacter/Components/BP_InventoryComponent.Find Last Item Index` _component))
          (if _success_2
            (bind _success_ (`/Game/BigMaze/Core/Characters/PlayerCharacter/Components/BP_InventoryComponent.Insert Item` _component (`self.Item`) _index))
            (if _success_
              (`self.K2_DestroyActor`)
              (message `/Game/BigMaze/Core/Characters/PlayerCharacter/Interfaces/BPI_UI.UI Update Hotbar` (`self.BP Character Ref`))
              (`KismetSystemLibrary.PrintString` (`KismetStringLibrary.Concat_StrStr` "Item: " (`/Game/BigMaze/ItemSystem/Blueprints/BFL_Items.Get Name` _item) " Stack: " (`KismetStringLibrary.Conv_IntToString` (`/Game/BigMaze/ItemSystem/Blueprints/BFL_Items.Get Stack Count` _item))) :!label _label))
            (else
              (bind (_success_3 _component_2) (message `/Game/BigMaze/Core/Characters/PlayerCharacter/Interfaces/BPI_InventoryComp.IC Retrieve Component Reference` Actor 0 :!label _label_2))
              (if _success_3
                (bind (_success_4 _index_2) (`/Game/BigMaze/Core/Characters/PlayerCharacter/Components/BP_InventoryComponent.Find Last Item Index` _component_2))
                (if _success_4
                  (bind _success__2 (`/Game/BigMaze/Core/Characters/PlayerCharacter/Components/BP_InventoryComponent.Insert Item` _component_2 (`self.Item`) _index_2))
                  (if _success__2
                    (`self.K2_DestroyActor`)
                    (message `/Game/BigMaze/Core/Characters/PlayerCharacter/Interfaces/BPI_UI.UI Update Hotbar` (`self.BP Character Ref`))
                    (goto _label))))))
          (else
            (goto _label_2)))
        (else
          (bind (_success_5 _component_3) (message `/Game/BigMaze/Core/Characters/PlayerCharacter/Interfaces/BPI_InventoryComp.IC Retrieve Component Reference` Actor 2))
          (if _success_5
            (for (_array_element _array_index) (`/Game/BigMaze/Core/Characters/PlayerCharacter/Components/BP_InventoryComponent.Inventory` _component_3)
              (if (== (`/Game/BigMaze/ItemSystem/Blueprints/BFL_Items.Get Name` _array_element) (`/Game/BigMaze/ItemSystem/Blueprints/BFL_Items.Get Name` (`self.Item`)))
                (set `self.Found Matching Ammo` true)
                (break)
                (else
                  (set `self.Found Matching Ammo` false))))
            (if (`self.Found Matching Ammo`)
              (bind _success__3 (`/Game/BigMaze/Core/Characters/PlayerCharacter/Components/BP_InventoryComponent.Insert Item` _component_3 (`self.Item`) _array_index))
              (if _success__3
                (`self.K2_DestroyActor`)
                (message `/Game/BigMaze/Core/Characters/PlayerCharacter/Interfaces/BPI_UI.UI Update Hotbar` (`self.BP Character Ref`))
                (goto _label)))))))
    (:`CastFailed`
      (`KismetSystemLibrary.PrintString` "FFF"))))

(event `self.Pickup Collision.OnComponentBeginOverlap`
  (params (OverlappedComponent :type "PrimitiveComponent Object Reference") (OtherActor :type "Actor Object Reference") (OtherComp :type "PrimitiveComponent Object Reference") (OtherBodyIndex :type Integer) (bFromSweep :type Boolean) (SweepResult :type "HitResult Structure (by ref)"))
  (if (`KismetSystemLibrary.DoesImplementInterface` OtherActor "/Game/BigMaze/Core/Characters/PlayerCharacter/Interfaces/BPI_Player.BPI_Player_C")
    (`self.SR Pickup` OtherActor)))

(fn `OnRep_Item`
  (`/Engine/EditorBlueprintResources/ActorMacros.Switch Has Authority`
    (:`Authority`
      (`self.Update Mesh Multicast`))
    (:`Remote`
      (`self.Update Mesh Server`))))

(fn `UserConstructionScript`)