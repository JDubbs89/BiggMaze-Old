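; Minimap detector helper actor that attaches to a parent actor, carrying a sphere trigger and an optional in-world icon widget.
; Initialise snaps it to the parent and either configures the icon's image, tint, scale, animation and height, or destroys the widget component.
; Tick turns the icon against the camera's forward vector and destroys the actor once its parent is invalid.
; SetActive toggles the trigger's query collision and the icon's visibility.
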(event `self.ReceiveTick`
  (params (DeltaSeconds :type "Float (single-precision)"))
  ;[1 1 1] Set the in-world widget to face the camera.
  (`SceneComponent.K2_SetWorldRotation` (`self.Widget_InWorldIcon`) (`KismetMathLibrary.Conv_VectorToRotator` (* (`self.GetActorForwardVector` (`GameplayStatics.GetPlayerCameraManager` 0)) -1.0)) false false)
  (`/Engine/EditorBlueprintResources/StandardMacros.IsValid` (`self.ParentActor`)
    (:`Is Not Valid`
      (`self.K2_DestroyActor`))))

(fn `GetInWorldWidget`
  (returns (Widget :type "Object Object Reference"))
  ;[1 1 1] Return the in-world widget
  (bind _aswidget_in_world_icon (cast `` (`WidgetComponent.GetUserWidgetObject` (`self.Widget_InWorldIcon`))))
  (return _aswidget_in_world_icon))

(fn `Initialise`
  (params (ParentActor :type "Actor Object Reference") (ShowIconInWorld :type Boolean) (InWorldIcon :type "Texture2D Object Reference") (InWorldIconZOffset :type "Float (double-precision)") (Tint :type "LinearColor Structure") (Scale :type "Float (double-precision)") (AnimationType :type "/Game/BigMaze/Core/UI/HUD/Minimap/ENUM_MinimapIconAnimationType Enum" :default "NewEnumerator3"))
  ;[1 1 1] Initialise the in-world widget, and attach it to the supplied parent actor.
  ; If the actor does not need an in-world widget, destroy the component.
  (bind _output_get (set `self.ParentActor` ParentActor))
  (`self.K2_AttachToActor` _output_get "None" "SnapToTarget" "SnapToTarget" "SnapToTarget")
  (if ShowIconInWorld
    (`self.SetActorTickEnabled` true)
    (`self.SetZOffset` InWorldIconZOffset)
    (bind _aswidget_in_world_icon (cast `` (`WidgetComponent.GetUserWidgetObject` (`self.Widget_InWorldIcon`))))
    (`self.SetImage` _aswidget_in_world_icon InWorldIcon)
    (`self.SetTint` _aswidget_in_world_icon Tint)
    (`self.SetScale` _aswidget_in_world_icon Scale)
    (`self.SetAnimationType` _aswidget_in_world_icon AnimationType)
    (else
      (`ActorComponent.K2_DestroyComponent` (`self.Widget_InWorldIcon`)))))

(fn `SetActive`
  (params (IsActive :type Boolean))
  (bind _sphere_trigger (`self.Sphere_Trigger`))
  (bind _widget_inworldicon (`self.Widget_InWorldIcon`))
  ;[1 1 1] Enable or disable the minimap attachment
  (if IsActive
    (`PrimitiveComponent.SetCollisionEnabled` _sphere_trigger "QueryOnly")
    (`SceneComponent.SetHiddenInGame` _widget_inworldicon false false)
    (else
      (`PrimitiveComponent.SetCollisionEnabled` _sphere_trigger "NoCollision")
      (`SceneComponent.SetHiddenInGame` _widget_inworldicon true true))))

(fn `SetZOffset`
  (params (ZOffset :type "Float (double-precision)"))
  ;[1 1 1] Set the Z offset of the in-world widget.
  (`SceneComponent.K2_SetRelativeLocation` (`self.Widget_InWorldIcon`) (`KismetMathLibrary.MakeVector` 0.0 0.0 ZOffset) false true))

(fn `UserConstructionScript`)