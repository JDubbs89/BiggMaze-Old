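; Blueprint function library for the item system, operating on the item struct for stacking, comparison, field editing and value-based rarity color.
; Weapon and use data (range, fire rate, magazine counts, activation modes) is parsed from the item's string attribute map, partly as colon-delimited fields.
; Combat helpers run randomized line traces, apply damage scaled by crit/armor component tags, distance and penetration, and send heals through BPI_Damageable.
; CanPerformAction gates item actions using exclusivity flags and gameplay tags.
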(fn `Add Item Stat`
  (params (`In Item` :type "/Game/BigMaze/Core/ItemAssets/Common/Structs/S_ItemStruct Structure") (`New Stat` :type "/Game/BigMaze/Core/ItemAssets/Common/Structs/S_Stat Structure"))
  (returns (`Out Item` :type "/Game/BigMaze/Core/ItemAssets/Common/Structs/S_ItemStruct Structure"))
  (locals (Stats :type "Array of /Game/BigMaze/Core/ItemAssets/Common/Structs/S_Stat Structure") (Item :type "/Game/BigMaze/Core/ItemAssets/Common/Structs/S_ItemStruct Structure"))
  (bind _output_get (set `local.Item` `In Item`))
  (bind _output_get_2 (set `local.Stats` (`.StatstoShow_32_75E0D92F4152130CE96400B0EC0CDFC5` (break `/Game/BigMaze/Core/ItemAssets/Common/Structs/S_ItemStruct` _output_get))))
  (`KismetArrayLibrary.Array_Add` _output_get_2 `New Stat`)
  (bind _structout (setmembers `/Game/BigMaze/Core/ItemAssets/Common/Structs/S_ItemStruct` :`StructRef` (`local.Item`) :`Stats to Show` _output_get_2))
  (return _structout))

(fn `Add Item Unique Attr`
  (params (`In Item` :type "/Game/BigMaze/Core/ItemAssets/Common/Structs/S_ItemStruct Structure") (`Unique Attr. Key` :type String) (`Unilque Attr. Value` :type String))
  (returns (`Out Item` :type "/Game/BigMaze/Core/ItemAssets/Common/Structs/S_ItemStruct Structure"))
  (locals (Atts :type "Map of String to String") (Item :type "/Game/BigMaze/Core/ItemAssets/Common/Structs/S_ItemStruct Structure"))
  (bind _output_get (set `local.Item` `In Item`))
  (bind _output_get_2 (set `local.Atts` (`.UniqueAttributes_28_D97642464C73B875ED3C1FB98B20E72B` (break `/Game/BigMaze/Core/ItemAssets/Common/Structs/S_ItemStruct` _output_get))))
  (`BlueprintMapLibrary.Map_Add` _output_get_2 `Unique Attr. Key` `Unilque Attr. Value`)
  (bind _structout (setmembers `/Game/BigMaze/Core/ItemAssets/Common/Structs/S_ItemStruct` :`StructRef` (`local.Item`) :`Unique Attributes` _output_get_2))
  (return _structout))

(fn `Add to Item Stack`
  (params (`Original Item` :type "/Game/BigMaze/Core/ItemAssets/Common/Structs/S_ItemStruct Structure") (`Item to Add` :type "/Game/BigMaze/Core/ItemAssets/Common/Structs/S_ItemStruct Structure"))
  (returns (Success :type Boolean) (`Combined Item` :type "/Game/BigMaze/Core/ItemAssets/Common/Structs/S_ItemStruct Structure") (`Has Leftover Item` :type Boolean) (`Leftover Item` :type "/Game/BigMaze/Core/ItemAssets/Common/Structs/S_ItemStruct Structure"))
  (locals (`Combined Stack Size` :type Integer) (`Og Item` :type "/Game/BigMaze/Core/ItemAssets/Common/Structs/S_ItemStruct Structure") (`New Item` :type "/Game/BigMaze/Core/ItemAssets/Common/Structs/S_ItemStruct Structure"))
  (bind ((`AmountinStack_19_98AFE5A043AE6D66199856AECC6A8541` _amountinstack) (`MaxStackSize_20_9553F7374D2178988D91708A575A7F07` _maxstacksize)) (break `/Game/BigMaze/Core/ItemAssets/Common/Structs/S_ItemStruct` (`local.Original Item`)))
  (bind _returnvalue (+ _amountinstack (`.AmountinStack_19_98AFE5A043AE6D66199856AECC6A8541` (break `/Game/BigMaze/Core/ItemAssets/Common/Structs/S_ItemStruct` (`local.Item to Add`)))))
  (set `local.Og Item` `Original Item`)
  (set `local.New Item` `Item to Add`)
  (if (`self.Compare Items` (`local.Og Item`) (`local.New Item`))
    (if (> _returnvalue _maxstacksize)
      (bind _output_get (set `local.Combined Stack Size` (`KismetMathLibrary.Clamp` _returnvalue 1 _maxstacksize)))
      (bind _structout (setmembers `/Game/BigMaze/Core/ItemAssets/Common/Structs/S_ItemStruct` :`StructRef` (`local.Og Item`) :`Amount in Stack` _output_get))
      (bind _structout_2 (setmembers `/Game/BigMaze/Core/ItemAssets/Common/Structs/S_ItemStruct` :`StructRef` (`local.Og Item`) :`Amount in Stack` (- _returnvalue _maxstacksize)))
      (return true _structout true _structout_2)
      (else
        (set `local.Combined Stack Size` _returnvalue)
        (bind _structout_3 (setmembers `/Game/BigMaze/Core/ItemAssets/Common/Structs/S_ItemStruct` :`StructRef` (`local.Og Item`)))
        (return true _structout_3 false)))
    (else
      (return false (struct) false))))

(fn `Can Perform Action`
  (params (Item :type "/Game/BigMaze/Core/ItemAssets/Common/Structs/S_ItemStruct Structure") (Tags :type "GameplayTagContainer Structure") (Action :type Integer))
  (returns (`Can Perform` :type Boolean))
  (bind _returnvalue (`BlueprintGameplayTagLibrary.HasTag` Tags (struct :`TagName` "itemstatus.tertiaryinuse")))
  (bind _returnvalue_2 (`BlueprintGameplayTagLibrary.HasTag` Tags (struct :`TagName` "itemstatus.primaryinuse")))
  (bind _returnvalue_3 (`BlueprintGameplayTagLibrary.HasTag` Tags (struct :`TagName` "itemstatus.secondaryinuse")))
  (bind _item (`local.Item`))
  (bind _tags (`local.Tags`))
  (return (select `int` (`local.Action`) :`0` (and (or (`KismetMathLibrary.BooleanNAND` _returnvalue_3 _returnvalue) (not (`self.Get Primary Exclusivity` _item))) (not (`BlueprintGameplayTagLibrary.HasTag` _tags (struct :`TagName` "itemstatus.primarycooldown")))) :`1` (and (or (`KismetMathLibrary.BooleanNAND` _returnvalue_2 _returnvalue) (not (`self.Get Secondary Exclusivity` _item))) (not (`BlueprintGameplayTagLibrary.HasTag` _tags (struct :`TagName` "itemstatus.secondarycooldown")))) :`2` (and (or (`KismetMathLibrary.BooleanNAND` _returnvalue_2 _returnvalue_3) (not (`self.Get Tertiary Exclusivity` _item))) (not (`BlueprintGameplayTagLibrary.HasTag` _tags (struct :`TagName` "itemstatus.tertiarycooldown")))))))

(fn `Compare Items`
  (params (`Item 1` :type "/Game/BigMaze/Core/ItemAssets/Common/Structs/S_ItemStruct Structure") (`Item 2` :type "/Game/BigMaze/Core/ItemAssets/Common/Structs/S_ItemStruct Structure"))
  (returns (`Are Items Same?` :type Boolean))
  (bind ((`Name_2_C8A30FD44209EC8654ED65827C16873B` _name) (`MaxStackSize_20_9553F7374D2178988D91708A575A7F07` _maxstacksize) (`ItemClass_34_463E1F7D44177C7E4922A6BF67BA516E` _itemclass) (`ItemValue_21_333E79CC4EAF9C5B38DE2AA4CB3C63C2` _itemvalue) (`UniqueAttributes_28_D97642464C73B875ED3C1FB98B20E72B` _uniqueattributes)) (break `/Game/BigMaze/Core/ItemAssets/Common/Structs/S_ItemStruct` (`local.Item 1`)))
  (bind ((`Name_2_C8A30FD44209EC8654ED65827C16873B` _name_2) (`MaxStackSize_20_9553F7374D2178988D91708A575A7F07` _maxstacksize_2) (`ItemClass_34_463E1F7D44177C7E4922A6BF67BA516E` _itemclass_2) (`ItemValue_21_333E79CC4EAF9C5B38DE2AA4CB3C63C2` _itemvalue_2) (`UniqueAttributes_28_D97642464C73B875ED3C1FB98B20E72B` _uniqueattributes_2)) (break `/Game/BigMaze/Core/ItemAssets/Common/Structs/S_ItemStruct` (`local.Item 2`)))
  (bind _values (`BlueprintMapLibrary.Map_Values` _uniqueattributes))
  (bind _values_2 (`BlueprintMapLibrary.Map_Values` _uniqueattributes_2))
  (return (and (== _name _name_2) (`KismetArrayLibrary.Array_Identical` _values_2 _values) (== _maxstacksize _maxstacksize_2) (== _itemvalue _itemvalue_2) (`|EnumEquality` _itemclass _itemclass_2))))

(fn `Damage Target`
  (params (Targets :type "Array of Actor Object Reference") (`Hit Components` :type "Array of ActorComponent Object Reference") (`Hit Distances` :type "Array of Float (double-precision)") (`Penetration Levels` :type "Array of Integer") (`Base Damage` :type "Float (double-precision)") (`Falloff Multiplier` :type "Float (double-precision)") (`Penetration Multiplier` :type "Float (double-precision)") (`Critical Hit Multiplier` :type "Float (double-precision)") (`Armor Damage Multiplier` :type "Float (double-precision)") (Instigator :type "Actor Object Reference") (`Instigator Controller` :type "Controller Object Reference"))
  (returns (`Damage Dealt` :type "Array of Float (double-precision)"))
  (locals (Damage :type "Float (double-precision)") (`Damages Dealt` :type "Array of Float (double-precision)"))
  (for (_array_element _array_index) Targets
    (bind _output_get (set `local.Damage` `Base Damage`))
    (bind _output (`|GetArrayItem` `Hit Components` _array_index))
    (bind _output_get_2 (set `local.Damage` (/ (* _output_get (`KismetMathLibrary.SelectFloat` `Critical Hit Multiplier` 1.0 (`ActorComponent.ComponentHasTag` _output "crit")) (`KismetMathLibrary.SelectFloat` `Armor Damage Multiplier` 1.0 (`ActorComponent.ComponentHasTag` _output "armor"))) (* (`|GetArrayItem` `Hit Distances` _array_index) (`local.Falloff Multiplier`) 0.01) (* (`local.Penetration Multiplier`) (select `int` (`|GetArrayItem` (`local.Penetration Levels`) _array_index) :`0` 3.0 :`1` 2.0 :`2` 1.0)))))
    (bind _returnvalue (`GameplayStatics.ApplyDamage` _array_element _output_get_2 (`local.Instigator Controller`) (`local.Instigator`) "/Game/BigMaze/Core/DamageTypes/Standard.Standard_C"))
    (`KismetArrayLibrary.Array_AddUnique` (`local.Damages Dealt`) _returnvalue))
  (return (`local.Damages Dealt`)))

(fn `Get Action ID`
  (params (Item :type "/Game/BigMaze/Core/ItemAssets/Common/Structs/S_ItemStruct Structure") (`Action Index` :type Integer))
  (returns (ID :type Integer))
  (return (`KismetStringLibrary.Conv_StringToInt` (`|GetArrayItem` (`KismetStringLibrary.ParseIntoArray` (`.Value` (`self.Get Specific Attribute` Item "actionid")) ":") `Action Index`))))

(fn `Get All Attributes`
  (params (Item :type "/Game/BigMaze/Core/ItemAssets/Common/Structs/S_ItemStruct Structure"))
  (returns (Map :type "Map of String to String"))
  (return (`.UniqueAttributes_28_D97642464C73B875ED3C1FB98B20E72B` (break `/Game/BigMaze/Core/ItemAssets/Common/Structs/S_ItemStruct` Item))))

(fn `Get Attributes`
  (params (Item :type "/Game/BigMaze/Core/ItemAssets/Common/Structs/S_ItemStruct Structure") (`Specific Attribute` :type String :default "none"))
  (returns (Map :type "Map of String to String") (Key :type String) (Value :type String) (Found :type Boolean))
  (bind ((`UniqueAttributes_28_D97642464C73B875ED3C1FB98B20E72B` _uniqueattributes)) (break `/Game/BigMaze/Core/ItemAssets/Common/Structs/S_ItemStruct` Item))
  (bind _returnvalue (== `Specific Attribute` "none"))
  (bind _specific_attribute (`local.Specific Attribute`))
  (bind (_value _returnvalue_2) (`BlueprintMapLibrary.Map_Find` _uniqueattributes _specific_attribute))
  (return _uniqueattributes (`KismetMathLibrary.SelectString` "none" _specific_attribute _returnvalue) (`KismetMathLibrary.SelectString` "none" _value _returnvalue) _returnvalue_2))

(fn `Get Backdrop Color`
  (params (Item :type "/Game/BigMaze/Core/ItemAssets/Common/Structs/S_ItemStruct Structure"))
  (returns (`Backdrop Color` :type "LinearColor Structure"))
  (return (`.BackdropColor_23_5D0B5FD9442455B2CC006A9464FB09DA` (break `/Game/BigMaze/Core/ItemAssets/Common/Structs/S_ItemStruct` Item))))

(fn `Get Class`
  (params (Item :type "/Game/BigMaze/Core/ItemAssets/Common/Structs/S_ItemStruct Structure"))
  (returns (`Item Class` :type "/Game/BigMaze/Core/ItemAssets/Common/Enums/E_ItemClass Enum"))
  (return (`.ItemClass_34_463E1F7D44177C7E4922A6BF67BA516E` (break `/Game/BigMaze/Core/ItemAssets/Common/Structs/S_ItemStruct` Item))))

(fn `Get Description`
  (params (Item :type "/Game/BigMaze/Core/ItemAssets/Common/Structs/S_ItemStruct Structure"))
  (returns (Description :type String))
  (return (`.Description_4_2229C7C6409CD1A8B034DEB6DCFBD8CD` (break `/Game/BigMaze/Core/ItemAssets/Common/Structs/S_ItemStruct` Item))))

(fn `Get Fall Off`
  (params (Item :type "/Game/BigMaze/Core/ItemAssets/Common/Structs/S_ItemStruct Structure"))
  (returns (NewParam :type "Float (double-precision)"))
  (bind (_out_key _value _found) (`self.Get Specific Attribute` Item "falloff"))
  (return (`KismetMathLibrary.SelectFloat` (`KismetStringLibrary.Conv_StringToDouble` _value) 0.0 _found)))

(fn `Get Full Auto`
  (params (Item :type "/Game/BigMaze/Core/ItemAssets/Common/Structs/S_ItemStruct Structure"))
  (returns (`Full Auto?` :type Boolean))
  (return (== (`.Value` (`self.Get Specific Attribute` Item "fullauto")) "True")))

(fn `Get Handling`
  (params (Item :type "/Game/BigMaze/Core/ItemAssets/Common/Structs/S_ItemStruct Structure"))
  (returns (Handling :type "Float (double-precision)"))
  (bind (_out_key _value _found) (`self.Get Specific Attribute` Item "handling"))
  (return (`KismetMathLibrary.SelectFloat` (`KismetStringLibrary.Conv_StringToDouble` _value) 1.0 _found)))

(fn `Get Icon`
  (params (Item :type "/Game/BigMaze/Core/ItemAssets/Common/Structs/S_ItemStruct Structure"))
  (returns (Icon :type "Texture2D Object Reference"))
  (return (`.Icon_33_977995DD4228B545E070B7A445F58AFB` (break `/Game/BigMaze/Core/ItemAssets/Common/Structs/S_ItemStruct` Item))))

(fn `Get Max Stack Size`
  (params (Item :type "/Game/BigMaze/Core/ItemAssets/Common/Structs/S_ItemStruct Structure"))
  (returns (`Max Stack Size` :type Integer))
  (return (`.MaxStackSize_20_9553F7374D2178988D91708A575A7F07` (break `/Game/BigMaze/Core/ItemAssets/Common/Structs/S_ItemStruct` Item))))

(fn `Get Name`
  (params (Item :type "/Game/BigMaze/Core/ItemAssets/Common/Structs/S_ItemStruct Structure"))
  (returns (Name :type String))
  (return (`.Name_2_C8A30FD44209EC8654ED65827C16873B` (break `/Game/BigMaze/Core/ItemAssets/Common/Structs/S_ItemStruct` Item))))

(fn `Get Pen Level`
  (params (Item :type "/Game/BigMaze/Core/ItemAssets/Common/Structs/S_ItemStruct Structure"))
  (returns (Range :type Integer))
  (return (`KismetStringLibrary.Conv_StringToInt` (`.Value` (`self.Get Specific Attribute` Item "pen")))))

(fn `Get Primary Activation Data`
  (params (Item :type "/Game/BigMaze/Core/ItemAssets/Common/Structs/S_ItemStruct Structure"))
  (returns (Press :type Boolean) (Release :type Boolean) (Hold :type Boolean))
  (bind _returnvalue (`KismetStringLibrary.ParseIntoArray` (`.Value` (`self.Get Specific Attribute` Item "primaryusetype")) ":"))
  (return (`KismetMathLibrary.Conv_IntToBool` (`KismetStringLibrary.Conv_StringToInt` (`|GetArrayItem` _returnvalue))) (`KismetMathLibrary.Conv_IntToBool` (`KismetStringLibrary.Conv_StringToInt` (`|GetArrayItem` _returnvalue 1))) (`KismetMathLibrary.Conv_IntToBool` (`KismetStringLibrary.Conv_StringToInt` (`|GetArrayItem` _returnvalue 2)))))

(fn `Get Primary Exclusivity`
  (params (Item :type "/Game/BigMaze/Core/ItemAssets/Common/Structs/S_ItemStruct Structure"))
  (returns (`Exclusive?` :type Boolean))
  (return (`KismetMathLibrary.Conv_IntToBool` (`KismetStringLibrary.Conv_StringToInt` (`|GetArrayItem` (`KismetStringLibrary.ParseIntoArray` (`.Value` (`self.Get Specific Attribute` Item "primaryusetype")) ":") 3)))))

(fn `Get Primary Use`
  (params (Item :type "/Game/BigMaze/Core/ItemAssets/Common/Structs/S_ItemStruct Structure"))
  (returns (`Use?` :type "/Game/BigMaze/Core/ItemAssets/Common/Enums/E_UseChart Enum") (`Activation Class` :type "/Game/BigMaze/Core/ItemAssets/Common/Enums/E_ActivationClass Enum"))
  (bind (_out_key _value _found) (`self.Get Specific Attribute` Item "primaryusehold"))
  (bind (_out_key_2 _value_2 _found_2) (`self.Get Specific Attribute` Item "primaryuse"))
  (return (select `bool` _found_2 :`false` "NewEnumerator0" :`true` (select `int` (`KismetStringLibrary.Conv_StringToInt` _value_2) :`0` "NewEnumerator0" :`1` "NewEnumerator1" :`2` "NewEnumerator2" :!type "/Game/BigMaze/Core/ItemAssets/Common/Enums/E_UseChart Enum")) (select `bool` _found :`false` "NewEnumerator0" :`true` (select `int` (`KismetStringLibrary.Conv_StringToInt` _value) :`0` "NewEnumerator0" :`1` "NewEnumerator1" :`2` "NewEnumerator2" :!type "/Game/BigMaze/Core/ItemAssets/Common/Enums/E_ActivationClass Enum"))))

(fn `Get Range`
  (params (Item :type "/Game/BigMaze/Core/ItemAssets/Common/Structs/S_ItemStruct Structure"))
  (returns (Range :type "Float (double-precision)"))
  (bind (_out_key _value _found) (`self.Get Specific Attribute` Item "range"))
  (return (`KismetMathLibrary.SelectFloat` (`KismetStringLibrary.Conv_StringToDouble` _value) 0.0 _found)))

(fn `Get Rarity Color`
  (params (Item :type "/Game/BigMaze/Core/ItemAssets/Common/Structs/S_ItemStruct Structure"))
  (returns (Color :type "LinearColor Structure"))
  (bind _item_value (`self.Get Value` Item))
  (return (`KismetMathLibrary.SelectColor` (struct :`R` 1.0 :`G` 0.15 :`B` 0.15 :`A` 1.0) (`KismetMathLibrary.SelectColor` (struct :`R` 0.92 :`G` 1.0 :`B` 0.12 :`A` 1.0) (`KismetMathLibrary.SelectColor` (struct :`R` 0.4 :`G` 0.08 :`B` 0.4 :`A` 1.0) (`KismetMathLibrary.SelectColor` (struct :`R` 0.2 :`G` 0.6 :`B` 1.0 :`A` 1.0) (`KismetMathLibrary.SelectColor` (struct :`R` 0.15 :`G` 1.0 :`B` 0.125 :`A` 1.0) (struct :`R` 0.4 :`G` 0.4 :`B` 0.4 :`A` 1.0) (> _item_value 150)) (> _item_value 300)) (> _item_value 600)) (> _item_value 1200)) (> _item_value 1800))))

(fn `Get Rate of Fire`
  (params (Item :type "/Game/BigMaze/Core/ItemAssets/Common/Structs/S_ItemStruct Structure"))
  (returns (`Fire Rate` :type "Float (double-precision)"))
  (bind (_out_key _value _found) (`self.Get Specific Attribute` Item "firerate"))
  (return (/ (`KismetMathLibrary.SelectFloat` (`KismetStringLibrary.Conv_StringToDouble` _value) 0.0 _found) 60.0)))

(fn `Get Secondary Activation Data`
  (params (Item :type "/Game/BigMaze/Core/ItemAssets/Common/Structs/S_ItemStruct Structure"))
  (returns (Press :type Boolean) (Release :type Boolean) (Hold :type Boolean))
  (bind _returnvalue (`KismetStringLibrary.ParseIntoArray` (`.Value` (`self.Get Specific Attribute` Item "secondaryusetype")) ":"))
  (return (`KismetMathLibrary.Conv_IntToBool` (`KismetStringLibrary.Conv_StringToInt` (`|GetArrayItem` _returnvalue))) (`KismetMathLibrary.Conv_IntToBool` (`KismetStringLibrary.Conv_StringToInt` (`|GetArrayItem` _returnvalue 1))) (`KismetMathLibrary.Conv_IntToBool` (`KismetStringLibrary.Conv_StringToInt` (`|GetArrayItem` _returnvalue 2)))))

(fn `Get Secondary Exclusivity`
  (params (Item :type "/Game/BigMaze/Core/ItemAssets/Common/Structs/S_ItemStruct Structure"))
  (returns (`Exclusive?` :type Boolean))
  (return (`KismetMathLibrary.Conv_IntToBool` (`KismetStringLibrary.Conv_StringToInt` (`|GetArrayItem` (`KismetStringLibrary.ParseIntoArray` (`.Value` (`self.Get Specific Attribute` Item "secondaryusetype")) ":") 3)))))

(fn `Get Secondary Use`
  (params (Item :type "/Game/BigMaze/Core/ItemAssets/Common/Structs/S_ItemStruct Structure"))
  (returns (`Use?` :type "/Game/BigMaze/Core/ItemAssets/Common/Enums/E_UseChart Enum") (`Activation Class` :type "/Game/BigMaze/Core/ItemAssets/Common/Enums/E_ActivationClass Enum"))
  (bind (_out_key _value _found) (`self.Get Specific Attribute` Item "secondaryusehold"))
  (bind (_out_key_2 _value_2 _found_2) (`self.Get Specific Attribute` Item "secondaryuse"))
  (return (select `bool` _found_2 :`false` "NewEnumerator0" :`true` (select `int` (`KismetStringLibrary.Conv_StringToInt` _value_2) :`0` "NewEnumerator0" :`1` "NewEnumerator1" :`2` "NewEnumerator2" :!type "/Game/BigMaze/Core/ItemAssets/Common/Enums/E_UseChart Enum")) (select `bool` _found :`false` "NewEnumerator0" :`true` (select `int` (`KismetStringLibrary.Conv_StringToInt` _value) :`0` "NewEnumerator0" :`1` "NewEnumerator1" :`2` "NewEnumerator2" :!type "/Game/BigMaze/Core/ItemAssets/Common/Enums/E_ActivationClass Enum"))))

(fn `Get Skeletal Mesh`
  (params (Item :type "/Game/BigMaze/Core/ItemAssets/Common/Structs/S_ItemStruct Structure"))
  (returns (`Skeletal mesh` :type "SkeletalMesh Object Reference"))
  (return (`.Skeletalmesh_22_9F66B36A4E99CF43E6FDFB85D416D8A0` (break `/Game/BigMaze/Core/ItemAssets/Common/Structs/S_ItemStruct` Item))))

(fn `Get Specific Attribute`
  (params (Item :type "/Game/BigMaze/Core/ItemAssets/Common/Structs/S_ItemStruct Structure") (`Attr Key` :type String :default "none"))
  (returns (`Out Key` :type String) (Value :type String) (Found :type Boolean))
  (bind (_value _returnvalue) (`BlueprintMapLibrary.Map_Find` (`.UniqueAttributes_28_D97642464C73B875ED3C1FB98B20E72B` (break `/Game/BigMaze/Core/ItemAssets/Common/Structs/S_ItemStruct` Item)) (`local.Attr Key`)))
  (return `Attr Key` _value (and (not (== `Attr Key` "none")) _returnvalue)))

(fn `Get Stack Count`
  (params (Item :type "/Game/BigMaze/Core/ItemAssets/Common/Structs/S_ItemStruct Structure"))
  (returns (`Amount in Stack` :type Integer))
  (return (`.AmountinStack_19_98AFE5A043AE6D66199856AECC6A8541` (break `/Game/BigMaze/Core/ItemAssets/Common/Structs/S_ItemStruct` Item))))

(fn `Get Stack Data`
  (params (Item :type "/Game/BigMaze/Core/ItemAssets/Common/Structs/S_ItemStruct Structure"))
  (returns (`Stackable?` :type Boolean) (Stack :type Integer) (`Max Stack` :type Integer) (`Has Ammunition?` :type Boolean))
  (bind _max_stack_size (`self.Get Max Stack Size` Item))
  (bind (_map _key _value _found) (`self.Get Attributes` Item "magsize"))
  (bind (_map_2 _key_2 _value_2 _found_2) (`self.Get Attributes` Item "magct"))
  (bind _returnvalue (and _found_2 _found))
  (return (> _max_stack_size 1) (`KismetMathLibrary.SelectInt` (`KismetStringLibrary.Conv_StringToInt` _value_2) (`self.Get Stack Count` Item) _returnvalue) (`KismetMathLibrary.SelectInt` (`KismetStringLibrary.Conv_StringToInt` _key) _max_stack_size _returnvalue) _returnvalue))

(fn `Get Stats`
  (params (Item :type "/Game/BigMaze/Core/ItemAssets/Common/Structs/S_ItemStruct Structure") (`Specific Stat Name` :type String :default "none"))
  (returns (Stats :type "Array of /Game/BigMaze/Core/ItemAssets/Common/Structs/S_Stat Structure") (`Specific Stat` :type "/Game/BigMaze/Core/ItemAssets/Common/Structs/S_Stat Structure"))
  (locals (Stat :type "/Game/BigMaze/Core/ItemAssets/Common/Structs/S_Stat Structure"))
  (bind ((`StatstoShow_32_75E0D92F4152130CE96400B0EC0CDFC5` _statstoshow)) (break `/Game/BigMaze/Core/ItemAssets/Common/Structs/S_ItemStruct` Item))
  (bind _returnvalue (== `Specific Stat Name` "none"))
  (if (not _returnvalue)
    (for _array_element _statstoshow
      (if (== (`.StatName_7_EBF1B7F5484456D782F15BBA30E0A45F` (break `/Game/BigMaze/Core/ItemAssets/Common/Structs/S_Stat` _array_element)) (`local.Specific Stat Name`))
        (set `local.Stat` _array_element)
        (break))))
  (return _statstoshow (select `bool` _returnvalue :`false` (`local.Stat`))))

(fn `Get Tertiary Activation Data`
  (params (Item :type "/Game/BigMaze/Core/ItemAssets/Common/Structs/S_ItemStruct Structure"))
  (returns (Press :type Boolean) (Release :type Boolean) (Hold :type Boolean))
  (bind _returnvalue (`KismetStringLibrary.ParseIntoArray` (`.Value` (`self.Get Specific Attribute` Item "tertiaryusetype")) ":"))
  (return (`KismetMathLibrary.Conv_IntToBool` (`KismetStringLibrary.Conv_StringToInt` (`|GetArrayItem` _returnvalue))) (`KismetMathLibrary.Conv_IntToBool` (`KismetStringLibrary.Conv_StringToInt` (`|GetArrayItem` _returnvalue 1))) (`KismetMathLibrary.Conv_IntToBool` (`KismetStringLibrary.Conv_StringToInt` (`|GetArrayItem` _returnvalue 2)))))

(fn `Get Tertiary Exclusivity`
  (params (Item :type "/Game/BigMaze/Core/ItemAssets/Common/Structs/S_ItemStruct Structure"))
  (returns (`Exclusive?` :type Boolean))
  (return (`KismetMathLibrary.Conv_IntToBool` (`KismetStringLibrary.Conv_StringToInt` (`|GetArrayItem` (`KismetStringLibrary.ParseIntoArray` (`.Value` (`self.Get Specific Attribute` Item "tertiaryusetype")) ":") 3)))))

(fn `Get Tertiary Use`
  (params (Item :type "/Game/BigMaze/Core/ItemAssets/Common/Structs/S_ItemStruct Structure"))
  (returns (`Use?` :type "/Game/BigMaze/Core/ItemAssets/Common/Enums/E_UseChart Enum") (`Activation Class` :type "/Game/BigMaze/Core/ItemAssets/Common/Enums/E_ActivationClass Enum"))
  (bind (_out_key _value _found) (`self.Get Specific Attribute` Item "tertiaryusehold"))
  (bind (_out_key_2 _value_2 _found_2) (`self.Get Specific Attribute` Item "tertiaryuse"))
  (return (select `bool` _found_2 :`false` "NewEnumerator0" :`true` (select `int` (`KismetStringLibrary.Conv_StringToInt` _value_2) :`0` "NewEnumerator0" :`1` "NewEnumerator1" :`2` "NewEnumerator2" :!type "/Game/BigMaze/Core/ItemAssets/Common/Enums/E_UseChart Enum")) (select `bool` _found :`false` "NewEnumerator0" :`true` (select `int` (`KismetStringLibrary.Conv_StringToInt` _value) :`0` "NewEnumerator0" :`1` "NewEnumerator1" :`2` "NewEnumerator2" :!type "/Game/BigMaze/Core/ItemAssets/Common/Enums/E_ActivationClass Enum"))))

(fn `Get Value`
  (params (Item :type "/Game/BigMaze/Core/ItemAssets/Common/Structs/S_ItemStruct Structure"))
  (returns (`Item Value` :type Integer))
  (return (`.ItemValue_21_333E79CC4EAF9C5B38DE2AA4CB3C63C2` (break `/Game/BigMaze/Core/ItemAssets/Common/Structs/S_ItemStruct` Item))))

(fn `Get Zoom`
  (params (Item :type "/Game/BigMaze/Core/ItemAssets/Common/Structs/S_ItemStruct Structure"))
  (returns (Zoom :type "Float (double-precision)"))
  (bind (_out_key _value _found) (`self.Get Specific Attribute` Item "zoom"))
  (return (`KismetMathLibrary.SelectFloat` (`KismetStringLibrary.Conv_StringToDouble` _value) 1.0 _found)))

(fn `Heal Target`
  (params (Targets :type "Array of Actor Object Reference") (Amount :type "Array of Float (double-precision)") (`Component Index` :type "Array of Integer"))
  (returns (`Heal Amount` :type "Array of Float (double-precision)"))
  (for (_array_element _array_index) Targets
    (if (`KismetSystemLibrary.DoesImplementInterface` _array_element "/Game/BigMaze/Core/Characters/PlayerCharacter/Interfaces/BPI_Damageable.BPI_Damageable_C")
      (message `/Game/BigMaze/Core/Characters/PlayerCharacter/Interfaces/BPI_Damageable.D RecieveHeal` _array_element (`|GetArrayItem` Amount _array_index) (`|GetArrayItem` `Component Index` _array_index))))
  (return Amount))

(fn `Is Null`
  (params (Item :type "/Game/BigMaze/Core/ItemAssets/Common/Structs/S_ItemStruct Structure"))
  (returns (`Null?` :type Boolean))
  (return (or (`KismetStringLibrary.EqualEqual_StrStr` (`self.Get Name` Item) "null") (<= (`self.Get Max Stack Size` Item) 0))))

(fn `Multi Trace for Targets`
  (params (Instigator :type "Actor Object Reference") (`Trace Count` :type Integer :default 1) (`Trace Variance Multiplier` :type "Float (double-precision)") (Origin :type "Vector Structure") (`Forward Vector` :type "Vector Structure") (Distance :type "Float (double-precision)") (`Excluded Targets` :type "Array of Actor Object Reference") (`Ignore Self?` :type Boolean) (Channel :type "ETraceTypeQuery Enum" :default "TraceTypeQuery1") (`Enable Debug` :type Boolean))
  (returns (OutHits :type "Array of HitResult Structure") (ReturnValue :type Boolean))
  (locals (Hits :type "Array of HitResult Structure") (`Hit?` :type Boolean :default false))
  (bind _returnvalue (+ Origin (* `Forward Vector` Distance)))
  (for _ (range `Trace Count`)
    (if `Ignore Self?`
      (`KismetArrayLibrary.Array_AddUnique` `Excluded Targets` Instigator))
    (bind (_outhits _returnvalue_2) (`KismetSystemLibrary.LineTraceMulti` Instigator Origin (+ (`/Game/UlimateBlueprintPack/System/Blueprints/UBPP_FunctionLibrary.Random Point On Circle` _returnvalue `Trace Variance Multiplier`) _returnvalue) Channel false `Excluded Targets` (select `bool` `Enable Debug` :`true` "ForDuration" :!type "EDrawDebugTrace Enum") `Ignore Self?`))
    (`KismetArrayLibrary.Array_Append` (`local.Hits`) _outhits)
    (if _returnvalue_2
      (set `local.Hit?` true)))
  (return (`local.Hits`) (`local.Hit?`)))

(fn `Remove Item From Stack`
  (params (Stack :type "/Game/BigMaze/Core/ItemAssets/Common/Structs/S_ItemStruct Structure") (Amount :type Integer))
  (returns (Success :type Boolean) (`Old Stack` :type "/Game/BigMaze/Core/ItemAssets/Common/Structs/S_ItemStruct Structure") (`Removed Item` :type "/Game/BigMaze/Core/ItemAssets/Common/Structs/S_ItemStruct Structure"))
  (locals (Item :type "/Game/BigMaze/Core/ItemAssets/Common/Structs/S_ItemStruct Structure"))
  (bind _stack (`local.Stack`))
  (bind _amount_in_stack (`self.Get Stack Count` (`local.Stack`)))
  (bind _returnvalue (`KismetMathLibrary.Clamp` (- _amount_in_stack (`local.Amount`)) 1 _amount_in_stack))
  (if (> (`self.Get Stack Count` (`local.Stack`)) 1)
    (bind _output_get (set `local.Item` Stack))
    (bind _out_item (`self.Update Item Stack Count` _output_get _returnvalue))
    (bind _out_item_2 (`self.Update Item Stack Count` (`local.Item`) (- (`self.Get Stack Count` _stack) _returnvalue)))
    (return true _out_item _out_item_2)
    (else
      (return false _stack))))

(fn `Remove Item Stat`
  (params (`In Item` :type "/Game/BigMaze/Core/ItemAssets/Common/Structs/S_ItemStruct Structure") (`Stat Name` :type String))
  (returns (`Out Item` :type "/Game/BigMaze/Core/ItemAssets/Common/Structs/S_ItemStruct Structure"))
  (locals (Stats :type "Array of /Game/BigMaze/Core/ItemAssets/Common/Structs/S_Stat Structure") (Item :type "/Game/BigMaze/Core/ItemAssets/Common/Structs/S_ItemStruct Structure"))
  (bind _output_get (set `local.Item` `In Item`))
  (bind _output_get_2 (set `local.Stats` (`.StatstoShow_32_75E0D92F4152130CE96400B0EC0CDFC5` (break `/Game/BigMaze/Core/ItemAssets/Common/Structs/S_ItemStruct` _output_get))))
  (for (_array_element _array_index) _output_get_2
    (if (== (`.StatName_7_EBF1B7F5484456D782F15BBA30E0A45F` (break `/Game/BigMaze/Core/ItemAssets/Common/Structs/S_Stat` _array_element)) (`local.Stat Name`))
      (`KismetArrayLibrary.Array_Remove` (`local.Stats`) _array_index)
      (break)))
  (bind _structout (setmembers `/Game/BigMaze/Core/ItemAssets/Common/Structs/S_ItemStruct` :`StructRef` (`local.Item`) :`Stats to Show` (`local.Stats`)))
  (return _structout))

(fn `Remove Item Unique Attr`
  (params (`In Item` :type "/Game/BigMaze/Core/ItemAssets/Common/Structs/S_ItemStruct Structure") (`Unique Attr. Key` :type String))
  (returns (`Out Item` :type "/Game/BigMaze/Core/ItemAssets/Common/Structs/S_ItemStruct Structure"))
  (locals (Atts :type "Map of String to String") (Item :type "/Game/BigMaze/Core/ItemAssets/Common/Structs/S_ItemStruct Structure"))
  (bind _output_get (set `local.Item` `In Item`))
  (bind _output_get_2 (set `local.Atts` (`.UniqueAttributes_28_D97642464C73B875ED3C1FB98B20E72B` (break `/Game/BigMaze/Core/ItemAssets/Common/Structs/S_ItemStruct` _output_get))))
  (`BlueprintMapLibrary.Map_Remove` _output_get_2 `Unique Attr. Key`)
  (bind _structout (setmembers `/Game/BigMaze/Core/ItemAssets/Common/Structs/S_ItemStruct` :`StructRef` (`local.Item`) :`Unique Attributes` _output_get_2))
  (return _structout))

(fn `Single Trace for Targets`
  (params (Instigator :type "Actor Object Reference") (`Trace Count` :type Integer :default 1) (`Trace Variance Radius` :type "Float (double-precision)") (Origin :type "Vector Structure") (`Forward Vector` :type "Vector Structure") (Distance :type "Float (double-precision)") (`Excluded Targets` :type "Array of Actor Object Reference") (`Ignore Self?` :type Boolean) (Channel :type "ETraceTypeQuery Enum" :default "TraceTypeQuery1") (`Enable Debug` :type Boolean))
  (returns (`Hit Results` :type "Array of HitResult Structure") (`Hit Target?` :type Boolean))
  (locals (Hits :type "Array of HitResult Structure") (`Hit?` :type Boolean))
  (bind _returnvalue (+ Origin (* `Forward Vector` Distance)))
  (for _ (range `Trace Count`)
    (if `Ignore Self?`
      (`KismetArrayLibrary.Array_AddUnique` `Excluded Targets` Instigator))
    (bind (_outhit _returnvalue_2) (`KismetSystemLibrary.LineTraceSingle` Instigator Origin (+ _returnvalue (`/Game/UlimateBlueprintPack/System/Blueprints/UBPP_FunctionLibrary.Random Point On Circle` _returnvalue `Trace Variance Radius` Instigator)) Channel false `Excluded Targets` (select `bool` `Enable Debug` :`true` "ForDuration" :!type "EDrawDebugTrace Enum") `Ignore Self?`))
    (`KismetArrayLibrary.Array_AddUnique` (`local.Hits`) _outhit)
    (if _returnvalue_2
      (set `local.Hit?` true)))
  (return (`local.Hits`) (`local.Hit?`)))

(fn `Split Item Stack`
  (params (Item :type "/Game/BigMaze/Core/ItemAssets/Common/Structs/S_ItemStruct Structure") (`New Stack Count` :type Integer))
  (returns (`Old Stack` :type "/Game/BigMaze/Core/ItemAssets/Common/Structs/S_ItemStruct Structure") (`New Stack` :type "/Game/BigMaze/Core/ItemAssets/Common/Structs/S_ItemStruct Structure") (Success :type Boolean))
  (locals (`Old Stack Value` :type Integer :default 0) (`In Item` :type "/Game/BigMaze/Core/ItemAssets/Common/Structs/S_ItemStruct Structure") (`Old Item` :type "/Game/BigMaze/Core/ItemAssets/Common/Structs/S_ItemStruct Structure"))
  (bind _old_item (`local.Old Item`))
  (bind ((`AmountinStack_19_98AFE5A043AE6D66199856AECC6A8541` _amountinstack)) (break `/Game/BigMaze/Core/ItemAssets/Common/Structs/S_ItemStruct` _old_item))
  (bind _output_get (set `local.Old Item` Item))
  (set `local.In Item` _output_get)
  (if (> (`.MaxStackSize_20_9553F7374D2178988D91708A575A7F07` (break `/Game/BigMaze/Core/ItemAssets/Common/Structs/S_ItemStruct` _old_item)) 1)
    (set `local.Old Stack Value` (`KismetMathLibrary.Clamp` (- _amountinstack (`local.New Stack Count`)) 1 (- _amountinstack 1)))
    (bind _structout (setmembers `/Game/BigMaze/Core/ItemAssets/Common/Structs/S_ItemStruct` :`StructRef` (`local.In Item`) :`Amount in Stack` (- (`.AmountinStack_19_98AFE5A043AE6D66199856AECC6A8541` (break `/Game/BigMaze/Core/ItemAssets/Common/Structs/S_ItemStruct` (`local.In Item`))) (`local.Old Stack Value`))))
    (bind _structout_2 (setmembers `/Game/BigMaze/Core/ItemAssets/Common/Structs/S_ItemStruct` :`StructRef` (`local.Old Item`) :`Amount in Stack` (`local.Old Stack Value`)))
    (return _structout_2 _structout true)
    (else
      (return (`local.Old Item`) (struct) false))))

(fn `Update Item Backdrop Color`
  (params (`In Item` :type "/Game/BigMaze/Core/ItemAssets/Common/Structs/S_ItemStruct Structure") (`New Color` :type "LinearColor Structure"))
  (returns (`Out Item` :type "/Game/BigMaze/Core/ItemAssets/Common/Structs/S_ItemStruct Structure"))
  (locals (Item :type "/Game/BigMaze/Core/ItemAssets/Common/Structs/S_ItemStruct Structure"))
  (bind _output_get (set `local.Item` `In Item`))
  (bind _structout (setmembers `/Game/BigMaze/Core/ItemAssets/Common/Structs/S_ItemStruct` :`StructRef` _output_get :`Backdrop Color` `New Color`))
  (return _structout))

(fn `Update Item Class`
  (params (`In Item` :type "/Game/BigMaze/Core/ItemAssets/Common/Structs/S_ItemStruct Structure") (`New Class` :type "/Game/BigMaze/Core/ItemAssets/Common/Enums/E_ItemClass Enum" :default "NewEnumerator0"))
  (returns (`Out Item` :type "/Game/BigMaze/Core/ItemAssets/Common/Structs/S_ItemStruct Structure"))
  (locals (Item :type "/Game/BigMaze/Core/ItemAssets/Common/Structs/S_ItemStruct Structure"))
  (bind _output_get (set `local.Item` `In Item`))
  (bind _structout (setmembers `/Game/BigMaze/Core/ItemAssets/Common/Structs/S_ItemStruct` :`StructRef` _output_get :`Item Class` `New Class`))
  (return _structout))

(fn `Update Item Description`
  (params (`In Item` :type "/Game/BigMaze/Core/ItemAssets/Common/Structs/S_ItemStruct Structure") (`New Desc` :type String))
  (returns (`Out Item` :type "/Game/BigMaze/Core/ItemAssets/Common/Structs/S_ItemStruct Structure"))
  (locals (Item :type "/Game/BigMaze/Core/ItemAssets/Common/Structs/S_ItemStruct Structure"))
  (bind _output_get (set `local.Item` `In Item`))
  (bind _structout (setmembers `/Game/BigMaze/Core/ItemAssets/Common/Structs/S_ItemStruct` :`StructRef` _output_get :`Description` `New Desc`))
  (return _structout))

(fn `Update Item Icon`
  (params (`In Item` :type "/Game/BigMaze/Core/ItemAssets/Common/Structs/S_ItemStruct Structure") (`New Icon` :type "Texture2D Object Reference"))
  (returns (`Out Item` :type "/Game/BigMaze/Core/ItemAssets/Common/Structs/S_ItemStruct Structure"))
  (locals (Item :type "/Game/BigMaze/Core/ItemAssets/Common/Structs/S_ItemStruct Structure"))
  (bind _output_get (set `local.Item` `In Item`))
  (bind _structout (setmembers `/Game/BigMaze/Core/ItemAssets/Common/Structs/S_ItemStruct` :`StructRef` _output_get :`Icon` `New Icon`))
  (return _structout))

(fn `Update Item Max Stack Size`
  (params (`In Item` :type "/Game/BigMaze/Core/ItemAssets/Common/Structs/S_ItemStruct Structure") (`New Max Stack Size` :type Integer))
  (returns (`Out Item` :type "/Game/BigMaze/Core/ItemAssets/Common/Structs/S_ItemStruct Structure"))
  (locals (Item :type "/Game/BigMaze/Core/ItemAssets/Common/Structs/S_ItemStruct Structure"))
  (bind _output_get (set `local.Item` (struct)))
  (bind _structout (setmembers `/Game/BigMaze/Core/ItemAssets/Common/Structs/S_ItemStruct` :`StructRef` _output_get :`Max Stack Size` `New Max Stack Size`))
  (return _structout))

(fn `Update Item Name`
  (params (`In Item` :type "/Game/BigMaze/Core/ItemAssets/Common/Structs/S_ItemStruct Structure") (`New Name` :type String))
  (returns (`Out Item` :type "/Game/BigMaze/Core/ItemAssets/Common/Structs/S_ItemStruct Structure"))
  (locals (Item :type "/Game/BigMaze/Core/ItemAssets/Common/Structs/S_ItemStruct Structure"))
  (bind _output_get (set `local.Item` `In Item`))
  (bind _structout (setmembers `/Game/BigMaze/Core/ItemAssets/Common/Structs/S_ItemStruct` :`StructRef` _output_get :`Name` `New Name`))
  (return _structout))

(fn `Update Item Skeletal Mesh`
  (params (`In Item` :type "/Game/BigMaze/Core/ItemAssets/Common/Structs/S_ItemStruct Structure") (`New Skeletal Mesh` :type "SkeletalMesh Object Reference"))
  (returns (`Out Item` :type "/Game/BigMaze/Core/ItemAssets/Common/Structs/S_ItemStruct Structure"))
  (locals (Item :type "/Game/BigMaze/Core/ItemAssets/Common/Structs/S_ItemStruct Structure"))
  (bind _output_get (set `local.Item` `In Item`))
  (bind _structout (setmembers `/Game/BigMaze/Core/ItemAssets/Common/Structs/S_ItemStruct` :`StructRef` _output_get :`Skeletal mesh` `New Skeletal Mesh`))
  (return _structout))

(fn `Update Item Stack Count`
  (params (`In Item` :type "/Game/BigMaze/Core/ItemAssets/Common/Structs/S_ItemStruct Structure") (`New Stack Ct` :type Integer))
  (returns (`Out Item` :type "/Game/BigMaze/Core/ItemAssets/Common/Structs/S_ItemStruct Structure"))
  (locals (Item :type "/Game/BigMaze/Core/ItemAssets/Common/Structs/S_ItemStruct Structure"))
  (bind _output_get (set `local.Item` `In Item`))
  (bind _structout (setmembers `/Game/BigMaze/Core/ItemAssets/Common/Structs/S_ItemStruct` :`StructRef` _output_get :`Amount in Stack` `New Stack Ct`))
  (return _structout))

(fn `Update Item Stats`
  (params (`In Item` :type "/Game/BigMaze/Core/ItemAssets/Common/Structs/S_ItemStruct Structure") (`New Stats` :type "Array of /Game/BigMaze/Core/ItemAssets/Common/Structs/S_Stat Structure"))
  (returns (`Out Item` :type "/Game/BigMaze/Core/ItemAssets/Common/Structs/S_ItemStruct Structure"))
  (locals (Item :type "/Game/BigMaze/Core/ItemAssets/Common/Structs/S_ItemStruct Structure"))
  (bind _output_get (set `local.Item` `In Item`))
  (bind _structout (setmembers `/Game/BigMaze/Core/ItemAssets/Common/Structs/S_ItemStruct` :`StructRef` _output_get :`Stats to Show` `New Stats`))
  (return _structout))

(fn `Update Item Unique Attr`
  (params (`In Item` :type "/Game/BigMaze/Core/ItemAssets/Common/Structs/S_ItemStruct Structure") (`New Unique Attrs` :type "Map of String to String"))
  (returns (`Out Item` :type "/Game/BigMaze/Core/ItemAssets/Common/Structs/S_ItemStruct Structure"))
  (locals (Item :type "/Game/BigMaze/Core/ItemAssets/Common/Structs/S_ItemStruct Structure"))
  (bind _output_get (set `local.Item` `In Item`))
  (bind _structout (setmembers `/Game/BigMaze/Core/ItemAssets/Common/Structs/S_ItemStruct` :`StructRef` _output_get :`Unique Attributes` `New Unique Attrs`))
  (return _structout))

(fn `Update Item Value`
  (params (`In Item` :type "/Game/BigMaze/Core/ItemAssets/Common/Structs/S_ItemStruct Structure") (`New Value` :type Integer))
  (returns (`Out Item` :type "/Game/BigMaze/Core/ItemAssets/Common/Structs/S_ItemStruct Structure"))
  (locals (Item :type "/Game/BigMaze/Core/ItemAssets/Common/Structs/S_ItemStruct Structure"))
  (bind _output_get (set `local.Item` `In Item`))
  (bind _structout (setmembers `/Game/BigMaze/Core/ItemAssets/Common/Structs/S_ItemStruct` :`StructRef` _output_get :`Item Value` `New Value`))
  (return _structout))